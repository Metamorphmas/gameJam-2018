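; Damage volume for a body part of the crab boss, attached as a child actor of Boss_Crab.
; Damage it takes is forwarded to the parent boss through TakePartDmg, along with flags identifying the leg, claw or center part.
; When DealDmg is set, the box also deals fixed damage to the player character on overlap.
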(event `/Game/Blueprints/CanTakeDamage.TakeDamage`
  (params (Damage :type "Float (single-precision)") (DamageType :type "/Game/Blueprints/Enums/DamageType Enum" :default "NewEnumerator5"))
  (bind _asboss_crab (cast `/Game/Blueprints/Enemies/Boss_Crab` (`self.GetParentActor`)))
  (`/Game/Blueprints/Enemies/Boss_Crab.TakePartDmg` _asboss_crab (`self.LeftLeg`) (`self.RightLeg`) (`self.LeftClaw`) (`self.RightClaw`) (`self.Center`) Damage))

(event `self.Box.OnComponentBeginOverlap`
  (params (OverlappedComponent :type "PrimitiveComponent Object Reference") (OtherActor :type "Actor Object Reference") (OtherComp :type "PrimitiveComponent Object Reference") (OtherBodyIndex :type Integer) (bFromSweep :type Boolean) (SweepResult :type "HitResult Structure (by ref)"))
  (bind _asplayer_character_final (cast `/Game/Blueprints/PlayerCharacter_Final` OtherActor))
  (if (`self.DealDmg`)
    (`/Game/Blueprints/PlayerCharacter_Final.TakeDamage` _asplayer_character_final 10.0 "NewEnumerator0")))

(fn `UserConstructionScript`)