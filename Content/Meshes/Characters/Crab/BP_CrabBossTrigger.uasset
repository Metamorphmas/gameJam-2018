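; BP_CrabBossTrigger is a trigger volume that starts the crab boss fight when the player walks into it.
; A Box overlap by PlayerCharacter_Final prints a debug message, then uses a Triggered flag so the fight starts only once.
; It calls StartFight on the CrabBoss reference, falling back to the first Boss_Crab found in the level when that reference is invalid.
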(event `self.Box.OnComponentBeginOverlap`
  (params (OverlappedComponent :type "PrimitiveComponent Object Reference") (OtherActor :type "Actor Object Reference") (OtherComp :type "PrimitiveComponent Object Reference") (OtherBodyIndex :type Integer) (bFromSweep :type Boolean) (SweepResult :type "HitResult Structure (by ref)"))
  (bind _crabboss (`self.CrabBoss`))
  (cast `/Game/Blueprints/PlayerCharacter_Final` OtherActor)
  (`KismetSystemLibrary.PrintString` "TRIGGERED")
  (if (not (`self.Triggered`))
    (set `self.Triggered` true)
    (if (`KismetSystemLibrary.IsValid` _crabboss)
      (`/Game/Blueprints/Enemies/Boss_Crab.StartFight` _crabboss)
      (else
        (bind _outactors (`GameplayStatics.GetAllActorsOfClass` "/Game/Blueprints/Enemies/Boss_Crab.Boss_Crab_C"))
        (`/Game/Blueprints/Enemies/Boss_Crab.StartFight` (`|GetArrayItem` _outactors))))))

(fn `UserConstructionScript`)