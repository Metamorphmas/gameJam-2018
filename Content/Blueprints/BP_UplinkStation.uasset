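; Uplink station that acts as a single-active checkpoint, storing the player's mech loadout and respawning them near it.
; Overlapping the outer box shows the Uplink widget and registers the station on the player.
; MakeActive saves state, turns screen and light green, and deactivates other stations.
; SpawnPlayer possesses a new mech with saved legs, chassis and fragments, but fixed arms and health; part-health restore is disconnected.
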(event `self.ReceiveBeginPlay`
  (bind _widget (`self.Widget`))
  (bind _asuplink (cast `/Game/UI/Uplink` (`WidgetComponent.GetUserWidgetObject` _widget)))
  (`/Game/UI/Uplink.MakeInactive` _asuplink)
  (`SceneComponent.SetHiddenInGame` _widget true false)
  (bind _returnvalue (`KismetMaterialLibrary.CreateDynamicMaterialInstance` "/Game/Materials/UplinkScreen.UplinkScreen"))
  (bind _output_get (set `self.Mat` _returnvalue))
  (`PrimitiveComponent.SetMaterial` (`self.StaticMesh`) 0 _output_get))

(event `self.OuterBox.OnComponentBeginOverlap`
  (params (OverlappedComponent :type "PrimitiveComponent Object Reference") (OtherActor :type "Actor Object Reference") (OtherComp :type "PrimitiveComponent Object Reference") (OtherBodyIndex :type Integer) (bFromSweep :type Boolean) (SweepResult :type "HitResult Structure (by ref)"))
  (bind _asplayer_character_final (cast `/Game/Blueprints/PlayerCharacter_Final` OtherActor))
  (`SceneComponent.SetHiddenInGame` (`self.Widget`) false false)
  (set `/Game/Blueprints/PlayerCharacter_Final.Uplink` self _asplayer_character_final)
  (`AudioComponent.Play` (`self.WAV_Chirp1`) 0.0))

(event `self.OuterBox.OnComponentEndOverlap`
  (params (OverlappedComponent :type "PrimitiveComponent Object Reference") (OtherActor :type "Actor Object Reference") (OtherComp :type "PrimitiveComponent Object Reference") (OtherBodyIndex :type Integer))
  (bind _asplayer_character_final (cast `/Game/Blueprints/PlayerCharacter_Final` OtherActor))
  (`SceneComponent.SetHiddenInGame` (`self.Widget`) true false)
  (set `/Game/Blueprints/PlayerCharacter_Final.Uplink` null _asplayer_character_final))

(fn `MakeActive`
  (params (LArm :type "/Game/Blueprints/Enums/ArmType Enum" :default "NewEnumerator0") (RArm :type "/Game/Blueprints/Enums/ArmType Enum" :default "NewEnumerator0") (Chassis :type "/Game/Blueprints/Enums/ChassisType Enum" :default "NewEnumerator0") (Legs :type "/Game/Blueprints/Enums/LegType Enum" :default "NewEnumerator0") (Health :type "Float (double-precision)") (FragmentNum :type Integer) (LArmHealth :type "Float (double-precision)") (RArmHealth :type "Float (double-precision)") (LegHealth :type "Float (double-precision)"))
  (bind _mat (`self.Mat`))
  (set `self.Active` true)
  (set `self.LeftArm` LArm)
  (set `self.RightArm` RArm)
  (set `self.Chassis` Chassis)
  (set `self.Legs` Legs)
  (set `self.Health` Health)
  (bind _output_get (set `self.FragmentNum` FragmentNum))
  (set `self.LArmHealth` LArmHealth)
  (set `self.RArmHealth` RArmHealth)
  (set `self.LegHealth` LegHealth)
  (bind _asuplink (cast `/Game/UI/Uplink` (`WidgetComponent.GetUserWidgetObject` (`self.Widget`))))
  (`/Game/UI/Uplink.MakeActive` _asuplink _output_get)
  (`AudioComponent.Play` (`self.WAV_Click2`) 0.0)
  (`MaterialInstanceDynamic.SetScalarParameterValue` _mat "Mask" 0.0)
  (`MaterialInstanceDynamic.SetVectorParameterValue` _mat "ScreenColor" (struct :`R` 0.219608 :`G` 1.0 :`A` 1.0))
  (`LightComponent.SetLightColor` (`self.PointLight`) (struct :`R` 0.219608 :`G` 1.0 :`A` 1.0) true)
  (bind _outactors (`GameplayStatics.GetAllActorsOfClass` "BP_UplinkStation_C"))
  (for _array_element _outactors
    (if (`/Game/Blueprints/BP_UplinkStation.Active` _array_element)
      (if (!= _array_element self)
        (`self.MakeInactive` _array_element)))))

(fn `MakeInactive`
  (bind _mat (`self.Mat`))
  (bind _asuplink (cast `/Game/UI/Uplink` (`WidgetComponent.GetUserWidgetObject` (`self.Widget`))))
  (`/Game/UI/Uplink.MakeInactive` _asuplink)
  (`MaterialInstanceDynamic.SetScalarParameterValue` _mat "Mask" 1.0)
  (`MaterialInstanceDynamic.SetVectorParameterValue` _mat "ScreenColor" (struct :`R` 1.0 :`G` 1.0 :`B` 1.0 :`A` 1.0))
  (`LightComponent.SetLightColor` (`self.PointLight`) (struct :`R` 1.0 :`G` 1.0 :`B` 1.0 :`A` 1.0) true)
  (set `self.Active` false))

(fn `SpawnPlayer`
  (bind _returnvalue (`self.GetTransform`))
  (bind _returnvalue_2 (`|SpawnActorFromClass` "/Game/Blueprints/PlayerCharacter_Final.PlayerCharacter_Final_C" (`KismetMathLibrary.MakeTransform` (`KismetMathLibrary.MakeVector` (+ (.x (.location _returnvalue)) -300.0) (.y (.location _returnvalue)) (+ (.z (.location _returnvalue)) 500.0))) "Undefined" "OverrideRootScale" null null))
  (`/Game/Blueprints/PlayerCharacter_Final.SetVars` _returnvalue_2 (`self.Legs`) (`self.Chassis`) "NewEnumerator1" "NewEnumerator10" 1.0 (`self.FragmentNum`))
  (`/Game/Blueprints/PlayerCharacter_Final.SetupRobot` _returnvalue_2)
  (`Controller.Possess` (`GameplayStatics.GetPlayerController` 0) _returnvalue_2)
  (bind _outactors (`GameplayStatics.GetAllActorsOfClass` "/Game/Blueprints/BP_FadeHandler.BP_FadeHandler_C"))
  (`/Game/Blueprints/BP_FadeHandler.FadeIn` (`|GetArrayItem` _outactors)))

(fn `UserConstructionScript`
  (bind _hidden (`self.Hidden`))
  (`SceneComponent.SetHiddenInGame` (`self.StaticMesh`) _hidden false)
  (if _hidden
    (`PrimitiveComponent.SetCollisionEnabled` (`self.Box`) "NoCollision")
    (`PrimitiveComponent.SetCollisionEnabled` (`self.OuterBox`) "NoCollision")
    (`PrimitiveComponent.SetCollisionEnabled` (`self.StaticMesh`) "NoCollision")
    (`SceneComponent.SetHiddenInGame` (`self.PointLight`) true false)))