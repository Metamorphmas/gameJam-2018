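; BP_PlasmaOrb is an optionally guided plasma projectile that explodes on impact.
; A fast timer moves it forward without sweeping, accelerating to a capped speed, while the Guided flag sets homing on ProjectileMovement.
; Only the first sphere hit counts: if the short arming delay has passed, it damages CanTakeDamage actors, spawns an explosion, disables collision and particles, then destroys itself after a delay.
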(event `Prime`
  (set `self.Primed` true))

(event `self.ReceiveBeginPlay`
  (set `ProjectileMovementComponent.bIsHomingProjectile` (`self.Guided`) (`self.ProjectileMovement`))
  (`KismetSystemLibrary.K2_SetTimerDelegate` (delegate `Prime`) 0.2 true)
  (`KismetSystemLibrary.K2_SetTimerDelegate` (delegate `Update`) 0.02 true))

(event `Update`
  (if (not (`self.Hit`))
    (`self.K2_SetActorLocation` (+ (`self.K2_GetActorLocation`) (* (`self.GetActorForwardVector`) (`self.Speed`))))
    (set `self.Speed` (`KismetMathLibrary.FClamp` (+ (`self.Speed`) 1.0) 0.0 50.0))))

(event `self.Sphere.OnComponentHit`
  (params (HitComponent :type "PrimitiveComponent Object Reference") (OtherActor :type "Actor Object Reference") (OtherComp :type "PrimitiveComponent Object Reference") (NormalImpulse :type "Vector Structure") (Hit :type "HitResult Structure (by ref)"))
  (bind _sphere (`self.Sphere`))
  (`/Engine/EditorBlueprintResources/StandardMacros.DoOnce` false
    (:`Completed`
      (if (`self.Primed`)
        (if (`KismetSystemLibrary.DoesImplementInterface` OtherActor "/Game/Blueprints/CanTakeDamage.CanTakeDamage_C")
          (message `/Game/Blueprints/CanTakeDamage.TakeDamage` OtherActor (`self.Damage`)))
        (`PrimitiveComponent.SetCollisionEnabled` _sphere "NoCollision")
        (`GameplayStatics.SpawnEmitterAtLocation` "/Game/ParticleEffects/P_PlasmaExplosion.P_PlasmaExplosion" (`SceneComponent.K2_GetComponentLocation` _sphere))
        (`ActorComponent.SetActive` (`self.ParticleSystem`) false false)
        (set `self.Hit` true)
        (`KismetSystemLibrary.K2_SetTimerDelegate` (delegate `DestroySelf`) 5.0)))))

(event `DestroySelf`
  (`self.K2_DestroyActor`))

(fn `UserConstructionScript`)