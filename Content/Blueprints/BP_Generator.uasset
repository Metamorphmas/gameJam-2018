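; BP_Generator is a destructible generator that sets its linked Gate's Powered flag to true when destroyed.
; CallwhenDestroyed runs once, spawning a scaled explosion, playing destruction sounds and activating broken-fire and spark particles.
; It applies one shared dynamic material instance to all linked cables, and a Flicker timeline animates its Brightness parameter.
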(event `self.ReceiveBeginPlay`
  (`self.Init`))

(event `self.CallWhenDestroyed`
  (bind _returnvalue (`self.K2_GetActorLocation`))
  (bind _expsize (`self.ExpSize`))
  (if (not (`self.Destroyed`))
    (set `self.Destroyed` true)
    (set `/Game/Blueprints/BP_Gate.Powered` true (`self.Gate`))
    (`GameplayStatics.SpawnEmitterAtLocation` "/Game/ParticleEffects/P_Explosion.P_Explosion" (`SceneComponent.K2_GetComponentLocation` (`self.DefaultSceneRoot`)) (struct) (`KismetMathLibrary.MakeVector` _expsize _expsize _expsize))
    (`GameplayStatics.PlaySoundAtLocation` "/Game/Audio/WAV_GeneratorDestroy.WAV_GeneratorDestroy" _returnvalue (struct) 1.0 1.0 0.0 null null null)
    (`GameplayStatics.PlaySoundAtLocation` "/Game/Audio/WAV_Explosion1_Reverb.WAV_Explosion1_Reverb" _returnvalue (struct) 1.0 1.0 0.0 null null null)
    (`ActorComponent.SetActive` (`self.P_FireBroken`) true false)
    (`ActorComponent.SetActive` (`self.P_Sparks`) true false)
    (bind _returnvalue_2 (`KismetMaterialLibrary.CreateDynamicMaterialInstance` (`self.CableMat`)))
    (for _array_element (`self.Cables`)
      (`PrimitiveComponent.SetMaterial` (`CableActor.CableComponent` _array_element) 0 _returnvalue_2))
    (bind (_direction _brightness) (`Timeline|Flicker`)
      (:`Update`
        (`MaterialInstanceDynamic.SetScalarParameterValue` _returnvalue_2 "Brightness" _brightness)))))

(fn `UserConstructionScript`)