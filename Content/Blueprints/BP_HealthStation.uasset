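; Health station actor that gradually heals PlayerCharacter_Final while it stands inside the Box trigger.
; Entering the box enables Tick, plays the looping station arm animation and activates sparks, caching the player reference only on the first entry.
; Tick adds a fixed, frame-rate-dependent amount to the player's Health, clamped to one.
; Full health or leaving the box disables Tick and stops the animation and sparks.
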(event `self.ReceiveBeginPlay`
  (bind _skeletalmesh (`self.SkeletalMesh`))
  (`SkeletalMeshComponent.PlayAnimation` _skeletalmesh "/Game/Meshes/HealingStation_Animated_Anim_StationArm_StationArmAction_001.HealingStation_Animated_Anim_StationArm_StationArmAction_001" true)
  (`SkeletalMeshComponent.Stop` _skeletalmesh))

(event `self.ReceiveTick`
  (params (DeltaSeconds :type "Float (single-precision)"))
  (bind _player (`self.Player`))
  (bind _output_get (set `/Game/Blueprints/PlayerCharacter_Final.Health` (`KismetMathLibrary.FClamp` (+ (`/Game/Blueprints/PlayerCharacter_Final.Health` _player) 0.002)) _player))
  (if (== _output_get 1.0)
    (`self.SetActorTickEnabled` false :!label _label)
    (`SkeletalMeshComponent.Stop` (`self.SkeletalMesh`))
    (`ActorComponent.SetActive` (`self.P_Sparks`) false false)))

(event `self.Box.OnComponentBeginOverlap`
  (params (OverlappedComponent :type "PrimitiveComponent Object Reference") (OtherActor :type "Actor Object Reference") (OtherComp :type "PrimitiveComponent Object Reference") (OtherBodyIndex :type Integer) (bFromSweep :type Boolean) (SweepResult :type "HitResult Structure (by ref)"))
  (bind _asplayer_character_final (cast `/Game/Blueprints/PlayerCharacter_Final` OtherActor))
  (`self.SetActorTickEnabled` true)
  (`SkeletalMeshComponent.Play` (`self.SkeletalMesh`) true)
  (`ActorComponent.SetActive` (`self.P_Sparks`) true false)
  (`/Engine/EditorBlueprintResources/StandardMacros.DoOnce` false
    (:`Completed`
      (set `self.Player` _asplayer_character_final))))

(event `self.Box.OnComponentEndOverlap`
  (params (OverlappedComponent :type "PrimitiveComponent Object Reference") (OtherActor :type "Actor Object Reference") (OtherComp :type "PrimitiveComponent Object Reference") (OtherBodyIndex :type Integer))
  (cast `/Game/Blueprints/PlayerCharacter_Final` OtherActor)
  (goto _label))

(fn `UserConstructionScript`)