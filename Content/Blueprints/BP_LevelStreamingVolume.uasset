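; Trigger actor that streams levels in and out as the player character moves through it.
; Overlapping LoadBox loads LoadLevelName as visible, blocking until done, and overlapping UnloadBox unloads UnloadLevelName without blocking.
; The Load and Unload booleans gate each box, only PlayerCharacter_Final triggers them, and each action prints the level name for debugging.
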(event `self.LoadBox.OnComponentBeginOverlap`
  (params (OverlappedComponent :type "PrimitiveComponent Object Reference") (OtherActor :type "Actor Object Reference") (OtherComp :type "PrimitiveComponent Object Reference") (OtherBodyIndex :type Integer) (bFromSweep :type Boolean) (SweepResult :type "HitResult Structure (by ref)"))
  (bind _loadlevelname (`self.LoadLevelName`))
  (cast `/Game/Blueprints/PlayerCharacter_Final` OtherActor)
  (if (`self.Load`)
    (`GameplayStatics.LoadStreamLevel` _loadlevelname true true)
    (`KismetSystemLibrary.PrintString` (`KismetStringLibrary.Concat_StrStr` "Loaded: " (`KismetStringLibrary.Conv_NameToString` _loadlevelname)))))

(event `self.UnloadBox.OnComponentBeginOverlap`
  (params (OverlappedComponent :type "PrimitiveComponent Object Reference") (OtherActor :type "Actor Object Reference") (OtherComp :type "PrimitiveComponent Object Reference") (OtherBodyIndex :type Integer) (bFromSweep :type Boolean) (SweepResult :type "HitResult Structure (by ref)"))
  (bind _unloadlevelname (`self.UnloadLevelName`))
  (cast `/Game/Blueprints/PlayerCharacter_Final` OtherActor)
  (if (`self.Unload`)
    (`GameplayStatics.UnloadStreamLevel` _unloadlevelname)
    (`KismetSystemLibrary.PrintString` (`KismetStringLibrary.Concat_StrStr` "Unloaded: " (`KismetStringLibrary.Conv_NameToString` _unloadlevelname)))))

(fn `UserConstructionScript`)