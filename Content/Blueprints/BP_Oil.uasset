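; Oil puddle actor that grows a decal when spawned and can be set on fire through Burn.
; While burning, it activates two particle systems and a looping timer damages CanTakeDamage actors overlapping BurnRadius.
; Igniting also reverses the Grow timeline, so the puddle shrinks as it burns.
; When the timeline finishes, the fire stops and the actor destroys itself after a short delay.
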(event `Reverse`
  (bind (_direction _size) (`Timeline|Grow` :!via `Reverse` :!label _label)
    (:`Update`
      (`SceneComponent.SetRelativeScale3D` (`self.Decal`) (`KismetMathLibrary.MakeVector` 1.0 _size _size)))
    (:`Finished`
      (if (`self.Burning`)
        (`self.Burn` false)))))

(event `self.ReceiveBeginPlay`
  (goto _label))

(fn `Burn`
  (params (StartBurn :type Boolean))
  (`ActorComponent.SetActive` (`self.ParticleSystem1`) StartBurn false)
  (`ActorComponent.SetActive` (`self.ParticleSystem2`) StartBurn false)
  (bind _output_get (set `self.Burning` StartBurn))
  (if _output_get
    (`self.Reverse`)
    (`KismetSystemLibrary.K2_SetTimer` self "BurnTargets" 0.25 true)
    (else
      (`KismetSystemLibrary.K2_PauseTimer` self "BurnTargets")
      (`KismetSystemLibrary.K2_SetTimer` self "DestroySelf" 2.0))))

(fn `BurnTargets`
  (for _array_element (`PrimitiveComponent.GetOverlappingActors` (`self.BurnRadius`) null)
    (if (`KismetSystemLibrary.DoesImplementInterface` _array_element "/Game/Blueprints/CanTakeDamage.CanTakeDamage_C")
      (message `/Game/Blueprints/CanTakeDamage.TakeDamage` _array_element 0.1 "NewEnumerator4"))))

(fn `DestroySelf`
  (`self.K2_DestroyActor`))

(fn `UserConstructionScript`)