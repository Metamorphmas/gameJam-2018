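; Modular robot enemy whose leg type (biped, quad, tracked or turret) and two weapon arms (plasma, rocket, laser or sword) are assembled in the construction script.
; Leg type also scales movement speed and drives leg animation and footstep audio.
; A looping timer replaces Tick, lerping legs toward control rotation and chassis and arms toward Target.
; Paired DoOnce gates start and stop arm firing as Target validity changes; Death plays an explosion sound and destroys the actor.
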(event `self.ReceiveBeginPlay`
  (`self.Init`)
  (`self.SetSpeed`)
  (`self.SetHealthBar`)
  (bind _returnvalue (`KismetSystemLibrary.K2_SetTimerDelegate` (delegate `Update`) 0.04 true))
  (set `self.UpdateHandle` _returnvalue))

(event `Update`
  (bind _childactor (`ChildActorComponent.ChildActor` (`self.RightArm`)))
  (bind _childactor_2 (`ChildActorComponent.ChildActor` (`self.LeftArm`)))
  (`self.SetRot`)
  (`self.UpdateHealtbarLoc`)
  (`self.UpdateAnimSpeed`)
  (if (`KismetSystemLibrary.IsValid` (`self.Target`))
    (`/Engine/EditorBlueprintResources/StandardMacros.DoOnce` false :!label _label
      (:`Completed`
        (bind _asbp_enemy_arm (cast `/Game/Blueprints/Enemies/EnemyWeapons/BP_EnemyArm` _childactor_2))
        (`/Game/Blueprints/Enemies/EnemyWeapons/BP_EnemyArm.BeginFiring` _asbp_enemy_arm)
        (bind _asbp_enemy_arm_2 (cast `/Game/Blueprints/Enemies/EnemyWeapons/BP_EnemyArm` _childactor))
        (`/Game/Blueprints/Enemies/EnemyWeapons/BP_EnemyArm.BeginFiring` _asbp_enemy_arm_2)
        (set `self.DoRotateArms` true)
        (`AudioComponent.Play` (`self.Cue_Alert`) 0.0)
        (goto _label_2 :!via `Reset`)))
    (else
      (`/Engine/EditorBlueprintResources/StandardMacros.DoOnce` false :!label _label_2
        (:`Completed`
          (bind _asbp_enemy_arm_3 (cast `/Game/Blueprints/Enemies/EnemyWeapons/BP_EnemyArm` _childactor_2))
          (`/Game/Blueprints/Enemies/EnemyWeapons/BP_EnemyArm.StopFiring` _asbp_enemy_arm_3)
          (bind _asbp_enemy_arm_4 (cast `/Game/Blueprints/Enemies/EnemyWeapons/BP_EnemyArm` _childactor))
          (`/Game/Blueprints/Enemies/EnemyWeapons/BP_EnemyArm.StopFiring` _asbp_enemy_arm_4)
          (set `self.DoRotateArms` false)
          (goto _label :!via `Reset`))))))

(event `self.Sphere.OnComponentBeginOverlap`
  (params (OverlappedComponent :type "PrimitiveComponent Object Reference") (OtherActor :type "Actor Object Reference") (OtherComp :type "PrimitiveComponent Object Reference") (OtherBodyIndex :type Integer) (bFromSweep :type Boolean) (SweepResult :type "HitResult Structure (by ref)"))
  (cast `/Game/Blueprints/PlayerCharacter_Final` OtherActor)
  (set `self.IsInRange` true))

(event `self.Sphere.OnComponentEndOverlap`
  (params (OverlappedComponent :type "PrimitiveComponent Object Reference") (OtherActor :type "Actor Object Reference") (OtherComp :type "PrimitiveComponent Object Reference") (OtherBodyIndex :type Integer))
  (cast `/Game/Blueprints/PlayerCharacter_Final` OtherActor)
  (set `self.IsInRange` false))

(event `self.Death`
  (`GameplayStatics.PlaySoundAtLocation` "/Game/Audio/WAV_Explosion1_Reverb.WAV_Explosion1_Reverb" (`self.K2_GetActorLocation`) (struct) 0.4 (`KismetMathLibrary.RandomFloatInRange` 0.7 1.2) 0.0 null null null)
  (`KismetSystemLibrary.K2_ClearAndInvalidateTimerHandle` (`self.UpdateHandle`))
  (`self.K2_DestroyActor`))

(fn `Init`)

(fn `ResetCanAttack`
  (set `self.CanAttack` true)
  (set `self.IsAttacking` false))

(fn `RotateArms`
  (bind _leftarm (`self.LeftArm`))
  (bind _rightarm (`self.RightArm`))
  (if (`KismetSystemLibrary.IsValid` (`self.Target`))
    (`|ExecutionSequence`
      (:`then_0`
        (bind _asbp_enemy_arm (cast `/Game/Blueprints/Enemies/EnemyWeapons/BP_EnemyArm` (`ChildActorComponent.ChildActor` _leftarm)))
        (bind (_returnvalue_roll _returnvalue_pitch _returnvalue_yaw) (`KismetMathLibrary.BreakRotator` (`KismetMathLibrary.FindLookAtRotation` (`SceneComponent.K2_GetComponentLocation` (`/Game/Blueprints/Enemies/EnemyWeapons/BP_EnemyArm.RotPos` _asbp_enemy_arm)) (`self.K2_GetActorLocation` (`self.Target`)))))
        (`SceneComponent.K2_SetWorldRotation` _leftarm (`KismetMathLibrary.RLerp` (`SceneComponent.K2_GetComponentRotation` _leftarm) (`KismetMathLibrary.MakeRotator` _returnvalue_roll _returnvalue_pitch (+ _returnvalue_yaw -90.0)) 0.12 true) false false))
      (:`then_1`
        (bind _asbp_enemy_arm_2 (cast `/Game/Blueprints/Enemies/EnemyWeapons/BP_EnemyArm` (`ChildActorComponent.ChildActor` _rightarm)))
        (bind (_returnvalue_roll_2 _returnvalue_pitch_2 _returnvalue_yaw_2) (`KismetMathLibrary.BreakRotator` (`KismetMathLibrary.FindLookAtRotation` (`SceneComponent.K2_GetComponentLocation` (`/Game/Blueprints/Enemies/EnemyWeapons/BP_EnemyArm.RotPos` _asbp_enemy_arm_2)) (`self.K2_GetActorLocation` (`self.Target`)))))
        (`SceneComponent.K2_SetWorldRotation` _rightarm (`KismetMathLibrary.RLerp` (`SceneComponent.K2_GetComponentRotation` _rightarm) (`KismetMathLibrary.MakeRotator` _returnvalue_roll_2 _returnvalue_pitch_2 (+ _returnvalue_yaw_2 -90.0)) 0.12 true) false false)))))

(fn `SetRot`
  (bind _target (`self.Target`))
  (bind _chassis (`self.Chassis`))
  (bind _legs (`self.Legs`))
  (bind (_returnvalue_roll _returnvalue_pitch _returnvalue_yaw) (`KismetMathLibrary.BreakRotator` (`KismetMathLibrary.FindLookAtRotation` (`self.K2_GetActorLocation`) (`self.K2_GetActorLocation` _target))))
  (`|ExecutionSequence`
    (:`then_0`
      (if (`self.DoRotate`)
        (`SceneComponent.K2_SetWorldRotation` _legs (`KismetMathLibrary.RLerp` (`SceneComponent.K2_GetComponentRotation` _legs) (`self.GetControlRotation`) 0.3 true) false false)))
    (:`then_1`
      (if (`KismetSystemLibrary.IsValid` _target)
        (`SceneComponent.K2_SetWorldRotation` _chassis (`KismetMathLibrary.RLerp` (`SceneComponent.K2_GetComponentRotation` _chassis) (`KismetMathLibrary.MakeRotator` 0.0 0.0 (+ _returnvalue_yaw -90.0)) 0.1 true) false false)))
    (:`then_2`
      (if (`self.DoRotateArms`)
        (`self.RotateArms`)))))

(fn `SetSpeed`
  (bind _footsteps (`self.Footsteps`))
  (bind _speed (`self.Speed`))
  (bind _legs (`self.Legs`))
  (bind _relativescale3d_x (`KismetMathLibrary.BreakVector` (`SceneComponent.RelativeScale3D` (`self.CapsuleComponent`))))
  (bind _returnvalue (/ (`self.Speed`) _relativescale3d_x))
  (switch `/Game/Blueprints/Enums/LegType` (`self.LegType`)
    (:`NewEnumerator0`
      (`AudioComponent.SetPitchMultiplier` _footsteps (* _returnvalue 1.2))
      (set `self.Speed` (* _speed 5.0))
      (`SkeletalMeshComponent.SetAnimation` _legs "/Game/Animations/BipedLegs/Mech_Legs_Biped1_RIGTEST2_Anim.Mech_Legs_Biped1_RIGTEST2_Anim")
      (`SkeletalMeshComponent.Play` _legs true))
    (:`NewEnumerator1`
      (`AudioComponent.SetPitchMultiplier` _footsteps (* _returnvalue 1.4))
      (set `self.Speed` (* _speed 3.0))
      (`SkeletalMeshComponent.SetAnimation` _legs "/Game/Animations/QuadLegs/Mech_QuadLegs1_Anim.Mech_QuadLegs1_Anim")
      (`SkeletalMeshComponent.Play` _legs true))
    (:`NewEnumerator2`
      (set `self.Speed` (* _speed 11.0)))
    (:`NewEnumerator3`
      (set `self.Speed` (* _speed 0.0))))
  (set `CharacterMovementComponent.MaxWalkSpeed` (* (/ (`self.Speed`) 5.0) 600.0) (`self.CharacterMovement`)))

(fn `SetupRobot`
  (bind _legs (`self.Legs`))
  (bind _leftarm (`self.LeftArm`))
  (bind _rightarm (`self.RightArm`))
  (set `self.Health` (`self.MaxHealth`))
  (`|ExecutionSequence`
    (:`then_0`
      (switch `/Game/Blueprints/Enums/LegType` (`self.LegType`)
        (:`NewEnumerator0`
          (`SkinnedMeshComponent.SetSkinnedAssetAndUpdate` _legs "/Game/Meshes/MechParts/Mesh_BipedLegs/Mech_Legs_Biped1_RIGTEST2.Mech_Legs_Biped1_RIGTEST2" true))
        (:`NewEnumerator1`
          (`SkinnedMeshComponent.SetSkinnedAssetAndUpdate` _legs "/Game/Meshes/MechParts/Mesh_QuadLegs/Mech_QuadLegs1.Mech_QuadLegs1" true))
        (:`NewEnumerator2`
          (`SkinnedMeshComponent.SetSkinnedAssetAndUpdate` _legs "/Game/Meshes/MechParts/Mesh_TreadLegs/Mech_TreadLegs1.Mech_TreadLegs1" true))
        (:`NewEnumerator3`
          (`SkinnedMeshComponent.SetSkinnedAssetAndUpdate` _legs "/Game/Meshes/MechParts/Mech_TurretBase.Mech_TurretBase" true)
          (`SkinnedMeshComponent.SetSkinnedAssetAndUpdate` (`self.Chassis`) "/Game/Meshes/MechParts/Mech_Chassis/Mech_TurretChassis.Mech_TurretChassis" true))))
    (:`then_1`
      (switch `/Game/Blueprints/Enums/ArmType` (`self.Arm1Type`)
        (:`NewEnumerator1`
          (`ChildActorComponent.SetChildActorClass` _leftarm "/Game/Blueprints/Enemies/EnemyWeapons/BP_EnemyPlasmaArm.BP_EnemyPlasmaArm_C"))
        (:`NewEnumerator3`
          (`ChildActorComponent.SetChildActorClass` _leftarm "/Game/Blueprints/Enemies/EnemyWeapons/BP_EnemyRocketArm.BP_EnemyRocketArm_C"))
        (:`NewEnumerator4`
          (`ChildActorComponent.SetChildActorClass` _leftarm "/Game/Blueprints/Enemies/EnemyWeapons/BP_EnemyLaserArm.BP_EnemyLaserArm_C"))
        (:`NewEnumerator5`
          (`ChildActorComponent.SetChildActorClass` _leftarm "/Game/Blueprints/Enemies/EnemyWeapons/BP_EnemySwordArm.BP_EnemySwordArm_C"))))
    (:`then_2`
      (switch `/Game/Blueprints/Enums/ArmType` (`self.Arm2Type`)
        (:`NewEnumerator1`
          (`ChildActorComponent.SetChildActorClass` _rightarm "/Game/Blueprints/Enemies/EnemyWeapons/BP_EnemyPlasmaArm.BP_EnemyPlasmaArm_C")
          (bind _asbp_enemy_arm (cast `/Game/Blueprints/Enemies/EnemyWeapons/BP_EnemyArm` (`ChildActorComponent.ChildActor` _rightarm) :!label _label))
          (set `/Game/Blueprints/Enemies/EnemyWeapons/BP_EnemyArm.Direction` true _asbp_enemy_arm))
        (:`NewEnumerator3`
          (`ChildActorComponent.SetChildActorClass` _rightarm "/Game/Blueprints/Enemies/EnemyWeapons/BP_EnemyRocketArm.BP_EnemyRocketArm_C")
          (goto _label))
        (:`NewEnumerator4`
          (`ChildActorComponent.SetChildActorClass` _rightarm "/Game/Blueprints/Enemies/EnemyWeapons/BP_EnemyLaserArm.BP_EnemyLaserArm_C")
          (goto _label))
        (:`NewEnumerator5`
          (`ChildActorComponent.SetChildActorClass` _rightarm "/Game/Blueprints/Enemies/EnemyWeapons/BP_EnemySwordArm.BP_EnemySwordArm_C"))))))

(fn `SpinAttack`
  (bind _chassis (`self.Chassis`))
  (`SkeletalMeshComponent.PlayAnimation` _chassis "/Game/Animations/Mech_Chassis_StrongAnimations_ChassisRoot_SpinReversed.Mech_Chassis_StrongAnimations_ChassisRoot_SpinReversed" false)
  (`SkeletalMeshComponent.SetPlayRate` _chassis 6.0))

(fn `UpdateAnimSpeed`
  (bind (_returnvalue_x _returnvalue_y _returnvalue_z) (`KismetMathLibrary.BreakVector` (`self.GetVelocity`)))
  (bind _legs (`self.Legs`))
  (bind _returnvalue (* (`self.Speed`) 2.0))
  (if (and (== _returnvalue_x 0.0) (== _returnvalue_y 0.0) (== _returnvalue_z 0.0))
    (if (not (`self.Stopped`))
      (set `self.Stopped` true)
      (`SkeletalMeshComponent.SetPlayRate` _legs 0.0)
      (set `self.DoRotate` false)
      (`AudioComponent.FadeOut` (`self.Footsteps`) 0.05 0.0))
    (elif (`self.Stopped`)
      (set `self.Stopped` false)
      (set `self.DoRotate` true)
      (`AudioComponent.FadeIn` (`self.Footsteps`) 0.05 1.0 0.0)
      (`|ExecutionSequence`
        (:`then_0`
          (switch `/Game/Blueprints/Enums/LegType` (`self.LegType`)
            (:`NewEnumerator0`
              (`SkeletalMeshComponent.SetPlayRate` _legs (/ _returnvalue 3.0)))
            (:`NewEnumerator1`
              (`SkeletalMeshComponent.SetPlayRate` _legs (/ _returnvalue 1.5)))))))))

(fn `UserConstructionScript`
  (`self.SetupRobot`))