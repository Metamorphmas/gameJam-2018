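; Base enemy pawn that handles damage, a floating health bar and death with mech part loot.
; Damage is reduced by armor, scaled by weakness or resistance type, then checked, revealing the health bar while the enemy lives.
; At zero health it spawns an explosion and fragment spawner, rolls per-part chances for arm and leg pickups with random condition, then plays a sound and destroys itself.
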(event `UpdateHealtbarLoc`
  (bind (_returnvalue_x _returnvalue_y _returnvalue_z) (`KismetMathLibrary.BreakVector` (`self.K2_GetActorLocation`)))
  (bind _healthbar (`self.HealthBar`))
  (`SceneComponent.K2_SetWorldRotation` _healthbar (struct :`Yaw` 180.0) false false)
  (`SceneComponent.K2_SetWorldLocation` _healthbar (`KismetMathLibrary.MakeVector` _returnvalue_x _returnvalue_y (+ (`self.HealthBarHeight`) _returnvalue_z)) false false))

(event `SetHealthBar`
  (bind _asenemy_health_bar (cast `/Game/UI/EnemyHealthBar` (`WidgetComponent.GetUserWidgetObject` (`self.HealthBar`))))
  (set `/Game/UI/EnemyHealthBar.Enemy` self _asenemy_health_bar)
  (`SceneComponent.SetWorldScale3D` (`self.HealthBar`) (1.0 1.0 1.0)))

(event `/Game/Blueprints/CanTakeDamage.TakeDamage`
  (params (Damage :type "Float (single-precision)") (DamageType :type "/Game/Blueprints/Enums/DamageType Enum" :default "NewEnumerator5"))
  (bind _health (`self.Health`))
  (bind _returnvalue (* Damage (- 1.0 (`self.Armor`))))
  (if (== DamageType (`self.Weakness`))
    (set `self.Health` (- _health (* _returnvalue 2.0)))
    (elif (== DamageType (`self.Resistance`))
      (set `self.Health` (- _health (* _returnvalue 0.5)))
      (else
        (set `self.Health` (- _health _returnvalue)))))
  (`/Game/Blueprints/CanTakeDamage.CheckHealth`)
  (set `self.HealthPercent` (/ (`self.Health`) (`self.MaxHealth`))))

(event `/Game/Blueprints/CanTakeDamage.CheckHealth`
  (bind _expsize (`self.ExpSize`))
  (if (<= (`self.Health`) 0.0)
    (`/Engine/EditorBlueprintResources/StandardMacros.DoOnce` false
      (:`Completed`
        (`GameplayStatics.SpawnEmitterAtLocation` "/Game/ParticleEffects/P_Explosion.P_Explosion" (`SceneComponent.K2_GetComponentLocation` (`self.CapsuleComponent`)) (struct) (`KismetMathLibrary.MakeVector` _expsize _expsize _expsize))
        (`self.DropParts`)
        (`|SpawnActorFromClass` "/Game/Blueprints/BP_FragmentSpawner.BP_FragmentSpawner_C" (`self.GetTransform`) "Undefined" "OverrideRootScale" null (`self.FragmentSpawnNum`) null)
        (`self.Death`)))
    (else
      (`/Engine/EditorBlueprintResources/StandardMacros.DoOnce` false
        (:`Completed`
          (`SceneComponent.SetHiddenInGame` (`self.HealthBar`) false false))))))

(fn `Death`
  (bind _asenemy (cast `/Game/Blueprints/Enemies/Enemy` self))
  (`GameplayStatics.PlaySoundAtLocation` (`AudioComponent.Sound` (`/Game/Blueprints/Enemies/Enemy.Cue_Alert` _asenemy)) (`self.K2_GetActorLocation`) (struct) 1.0 1.0 0.0 null null null)
  (`self.K2_DestroyActor`))

(fn `DropParts`
  (bind (_returnvalue_location _returnvalue_rotation) (`KismetMathLibrary.BreakTransform` (`self.GetTransform`)))
  (bind (_returnvalue_location_2 _returnvalue_rotation_2) (`KismetMathLibrary.BreakTransform` (`self.GetTransform`)))
  (bind (_returnvalue_location_3 _returnvalue_rotation_3) (`KismetMathLibrary.BreakTransform` (`self.GetTransform`)))
  (`|ExecutionSequence`
    (:`then_0`
      (if (> (`self.Arm1DropChance`) (`KismetMathLibrary.RandomFloatInRange` 0.0 1.0))
        (`|SpawnActorFromClass` "/Game/Blueprints/BP_MechPartPickup.BP_MechPartPickup_C" (`KismetMathLibrary.MakeTransform` _returnvalue_location_2 _returnvalue_rotation_2 (0.5 0.5 0.5)) "Undefined" "OverrideRootScale" null "NewEnumerator0" (`self.Arm1Type`) "NewEnumerator0" "NewEnumerator0" (/ (`KismetMathLibrary.Conv_IntToDouble` (`KismetMathLibrary.RandomIntegerInRange` 25 100)) 100.0) 0.0 false null)))
    (:`then_1`
      (if (> (`self.Arm2DropChance`) (`KismetMathLibrary.RandomFloatInRange` 0.0 1.0))
        (`|SpawnActorFromClass` "/Game/Blueprints/BP_MechPartPickup.BP_MechPartPickup_C" (`KismetMathLibrary.MakeTransform` _returnvalue_location_3 _returnvalue_rotation_3 (0.5 0.5 0.5)) "Undefined" "OverrideRootScale" null "NewEnumerator0" (`self.Arm2Type`) "NewEnumerator0" "NewEnumerator0" (/ (`KismetMathLibrary.Conv_IntToDouble` (`KismetMathLibrary.RandomIntegerInRange` 25 100)) 100.0) 0.0 false null)))
    (:`then_2`
      (if (> (`self.LegDropChance`) (`KismetMathLibrary.RandomFloatInRange` 0.0 1.0))
        (`|SpawnActorFromClass` "/Game/Blueprints/BP_MechPartPickup.BP_MechPartPickup_C" (`KismetMathLibrary.MakeTransform` _returnvalue_location _returnvalue_rotation (0.5 0.5 0.5)) "Undefined" "OverrideRootScale" null "NewEnumerator1" "NewEnumerator0" (`self.LegType`) "NewEnumerator0" (/ (`KismetMathLibrary.Conv_IntToDouble` (`KismetMathLibrary.RandomIntegerInRange` 25 100)) 100.0) 0.0 false null)))))

(fn `UserConstructionScript`)