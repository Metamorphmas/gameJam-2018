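; Sword arm weapon part for melee enemy mechs, swapping to a variant mesh and animation on quadruped or tracked parents.
; Attacking plays the swing animation and triggers the parent's SpinAttack; sword overlaps while the parent attacks damage valid targets and flash brief sparks.
; Incoming damage passes a quarter to the enemy pawn and reduces the arm's own armor-mitigated health.
; Breaking enables a second particle effect and sharply lowers sword damage.
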(event `self.ReceiveBeginPlay`
  (bind _mechpart (`self.MechPart`))
  (bind _asmelee (cast `/Game/Blueprints/Enemies/MeleeEnemy/Melee` (`self.GetParentActor`)))
  (switch `/Game/Blueprints/Enums/LegType` (`/Game/Blueprints/Enemies/MeleeEnemy/Melee.LegType_0` _asmelee)
    (:`NewEnumerator1`
      _)
    (:`NewEnumerator2`
      _))
  (`SkinnedMeshComponent.SetSkinnedAssetAndUpdate` _mechpart "/Game/Meshes/MechParts/Mesh_Arms/Mech_SwordArm2.Mech_SwordArm2" true)
  (`SkeletalMeshComponent.SetAnimation` _mechpart "/Game/Animations/Arms/Mech_SwordArm2_Anim.Mech_SwordArm2_Anim"))

(event `/Game/Blueprints/CanTakeDamage.TakeDamage`
  (params (Damage :type "Float (single-precision)") (DamageType :type "/Game/Blueprints/Enums/DamageType Enum" :default "NewEnumerator5"))
  (bind _asbp_enemy_pawn (cast `/Game/Blueprints/Enemies/BP_EnemyPawn` (`self.GetParentActor`)))
  (`/Game/Blueprints/Enemies/BP_EnemyPawn.TakeDamage` _asbp_enemy_pawn (* Damage 0.25) DamageType)
  (set `self.Health` (`KismetMathLibrary.FClamp` (- (`self.Health`) (* Damage (- 1.0 (`self.Armor`))))))
  (`/Game/Blueprints/CanTakeDamage.CheckHealth`))

(event `self.EnemyAttack_Once`
  (bind _mechpart (`self.MechPart`))
  (`SkeletalMeshComponent.SetPlayRate` _mechpart 3.2)
  (`SkeletalMeshComponent.Play` _mechpart false)
  (bind _asmelee (cast `/Game/Blueprints/Enemies/MeleeEnemy/Melee` (`self.GetParentActor`)))
  (`/Game/Blueprints/Enemies/MeleeEnemy/Melee.SpinAttack` _asmelee))

(event `self.SwordColl.OnComponentBeginOverlap`
  (params (OverlappedComponent :type "PrimitiveComponent Object Reference") (OtherActor :type "Actor Object Reference") (OtherComp :type "PrimitiveComponent Object Reference") (OtherBodyIndex :type Integer) (bFromSweep :type Boolean) (SweepResult :type "HitResult Structure (by ref)"))
  (bind _returnvalue (`self.GetParentActor`))
  (bind _asmelee (cast `/Game/Blueprints/Enemies/MeleeEnemy/Melee` _returnvalue))
  (if (`/Game/Blueprints/Enemies/MeleeEnemy/Melee.IsAttacking` _asmelee)
    (if (and (`KismetSystemLibrary.DoesImplementInterface` OtherActor "/Game/Blueprints/CanTakeDamage.CanTakeDamage_C") (!= OtherActor _returnvalue))
      (message `/Game/Blueprints/CanTakeDamage.TakeDamage` OtherActor (`self.Damage`) "NewEnumerator0"))
    (`ActorComponent.SetActive` (`self.ParticleSystem`) true false)
    (`KismetSystemLibrary.K2_SetTimerDelegate` (delegate `StopSparks`) (`KismetMathLibrary.RandomFloatInRange` 0.01 0.1))))

(event `StopSparks`
  (`ActorComponent.SetActive` (`self.ParticleSystem`) false false))

(event `self.MakeBroken`
  (`ActorComponent.SetActive` (`self.ParticleSystem1`) true false)
  (set `self.Broken` true)
  (set `self.Damage` 0.01))

(fn `UserConstructionScript`)