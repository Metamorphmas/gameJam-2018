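; Enemy plasma arm weapon that fires plasma orbs from its fire location on behalf of its parent actor.
; BeginFiring schedules a shot after a random delay, and each shot re-arms a randomly timed timer for irregular bursts until StopFiring clears it.
; Each shot passes Damage to the orb and plays a pitch-varied gun sound.
; It checks health on BeginPlay and activates a particle effect when broken.
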(event `self.ReceiveBeginPlay`
  (`self.CheckHealth`))

(event `self.BeginFiring`
  (`KismetSystemLibrary.K2_SetTimerDelegate` (delegate `self.EnemyAttack_Once`) (`KismetMathLibrary.RandomFloatInRange` 0.15 1.0)))

(event `self.StopFiring`
  (`KismetSystemLibrary.K2_ClearAndInvalidateTimerHandle` (stale `self.EnemyAttack_Once` _returnvalue)))

(event `self.EnemyAttack_Once`
  (bind _firelocation (`self.FireLocation`))
  (bind _wav_gunsound2 (`self.WAV_GunSound2`))
  (bind (_returnvalue_roll _returnvalue_pitch _returnvalue_yaw) (`KismetMathLibrary.BreakRotator` (`SceneComponent.K2_GetComponentRotation` _firelocation)))
  (`|SpawnActorFromClass` "/Game/Blueprints/Projectiles/BP_PlasmaOrb.BP_PlasmaOrb_C" (`KismetMathLibrary.MakeTransform` (`SceneComponent.K2_GetComponentLocation` _firelocation) (`KismetMathLibrary.MakeRotator` _returnvalue_roll _returnvalue_pitch (+ _returnvalue_yaw 90.0)) (0.6 0.6 0.6)) "Undefined" "OverrideRootScale" null null (`self.GetParentActor`) 15.0 false (`self.Damage`) null)
  (`AudioComponent.SetPitchMultiplier` _wav_gunsound2 (`KismetMathLibrary.RandomFloatInRange` 0.5 0.6))
  (`AudioComponent.Play` _wav_gunsound2 0.0)
  (bind _returnvalue (`KismetSystemLibrary.K2_SetTimerDelegate` (delegate `self.EnemyAttack_Once`) (`KismetMathLibrary.RandomFloatInRange` 0.15 0.6))))

(event `/Game/Blueprints/BPMechParts/BP_MechPart.MakeBroken`
  (`ActorComponent.SetActive` (`self.ParticleSystem`) true false))

(fn `UserConstructionScript`)