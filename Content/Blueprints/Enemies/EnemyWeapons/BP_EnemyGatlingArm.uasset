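; Enemy gatling arm weapon that fires in randomly timed bursts with random pauses until stopped or broken.
; A looping timer ramps a spin value that drives the MechPart play rate, with DoOnce gates switching effects, audio and the Fire loop near full speed.
; Fire line-traces to place impact particles, flicker the light and send damage through the CanTakeDamage interface.
; MakeBroken halts firing and calls SetArmorVal on the player.
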(event `self.ReceiveBeginPlay`)

(event `self.ReceiveTick`
  (params (DeltaSeconds :type "Float (single-precision)"))
  (`SkeletalMeshComponent.SetPlayRate` (`self.MechPart`) (`self.Rot`)))

(event `self.BeginFiring`
  (if (not (`self.Broken`))
    (bind _returnvalue (`KismetSystemLibrary.K2_SetTimerDelegate` (delegate `BreakFiring`) (`KismetMathLibrary.RandomFloatInRange` 1.0 6.0)))
    (`KismetSystemLibrary.K2_SetTimerDelegate` (delegate `self.EnemyAttack_Constant`) 0.02 true)
    (set `self.Input` 1.0)
    (set `self.Stopped` false)))

(event `BreakFiring`
  (set `self.Input` 0.0)
  (bind _returnvalue (`KismetSystemLibrary.K2_SetTimerDelegate` (delegate `self.BeginFiring`) (`KismetMathLibrary.RandomFloatInRange` 2.0 4.0))))

(event `self.StopFiring`
  (`KismetSystemLibrary.K2_ClearAndInvalidateTimerHandle` (stale `BreakFiring` _returnvalue))
  (`KismetSystemLibrary.K2_ClearAndInvalidateTimerHandle` (stale `self.BeginFiring` _returnvalue))
  (set `self.Input` 0.0)
  (set `self.Stopped` true))

(event `self.EnemyAttack_Constant`
  (bind _pointlight (`self.PointLight`))
  (bind _audio (`self.Audio`))
  (if (> (`self.Input`) 0.0)
    (`|ExecutionSequence`
      (:`then_0`
        (goto _label_3 :!via `Reset`))
      (:`then_1`
        (bind _output_get (set `self.Rot` (`KismetMathLibrary.FClamp` (+ (`self.Rot`) 0.14) 0.0 10.0)))
        (if (> _output_get 9.0)
          (`/Engine/EditorBlueprintResources/StandardMacros.DoOnce` false :!label _label
            (:`Completed`
              (`ActorComponent.SetActive` (`self.ParticleSystem1`) true false)
              (`ActorComponent.SetActive` (`self.ParticleSystem`) true false)
              (`SceneComponent.SetHiddenInGame` (`self.PointLight`) false false)
              (`KismetSystemLibrary.K2_SetTimer` self "Fire" 0.08 true)
              (`AudioComponent.Play` _audio 0.0)))))
      (:`then_2`
        (`/Engine/EditorBlueprintResources/StandardMacros.DoOnce` false :!label _label_2
          (:`Completed`
            (`AudioComponent.Play` (`self.Audio1`) 0.0)))))
    (else
      (set `self.Rot` (`KismetMathLibrary.FClamp` (+ (`self.Rot`) -0.12) 0.0 10.0))
      (`/Engine/EditorBlueprintResources/StandardMacros.DoOnce` false :!label _label_3
        (:`Completed`
          (`ActorComponent.SetActive` (`self.ParticleSystem`) false false)
          (`ActorComponent.SetActive` (`self.ParticleSystem1`) false false)
          (`KismetSystemLibrary.K2_ClearTimer` self "Fire")
          (`LightComponent.SetIntensity` _pointlight 0.0)
          (`SceneComponent.SetHiddenInGame` _pointlight true false)
          (`AudioComponent.Play` (`self.Audio2`) 0.0)
          (`AudioComponent.FadeOut` _audio 0.2 0.0)
          (`|ExecutionSequence`
            (:`then_0`
              (goto _label :!via `Reset`))
            (:`then_1`
              (goto _label_2 :!via `Reset`))))))))

(event `self.MakeBroken`
  (bind _particlesystem (`self.ParticleSystem`))
  (bind _particlesystem2 (`self.ParticleSystem2`))
  (bind _particlesystem1 (`self.ParticleSystem1`))
  (if (`KismetSystemLibrary.IsValid` _particlesystem)
    (`ActorComponent.SetActive` _particlesystem true false))
  (if (`KismetSystemLibrary.IsValid` _particlesystem1)
    (`ActorComponent.SetActive` _particlesystem1 false false))
  (if (`KismetSystemLibrary.IsValid` _particlesystem2)
    (`ActorComponent.SetActive` _particlesystem2 false false))
  (`KismetSystemLibrary.K2_ClearTimer` self "Fire")
  (`SceneComponent.SetHiddenInGame` (`self.PointLight`) true false)
  (set `self.Rot` 0.0)
  (`AudioComponent.Stop` (`self.Audio`))
  (`AudioComponent.Stop` (`self.Audio1`))
  (`AudioComponent.Stop` (`self.Audio2`))
  (bind _asplayer_character_final (cast `/Game/Blueprints/PlayerCharacter_Final` (`GameplayStatics.GetPlayerPawn` 0)))
  (`/Game/Blueprints/PlayerCharacter_Final.SetArmorVal` _asplayer_character_final))

(fn `Fire`
  (bind _scene (`self.Scene`))
  (bind _returnvalue (`SceneComponent.K2_GetComponentLocation` _scene))
  (if (not (`self.Stopped`))
    (`LightComponent.SetIntensity` (`self.PointLight`) (`KismetMathLibrary.RandomFloatInRange` 1000.0 3000.0))
    (bind _outhit (`KismetSystemLibrary.LineTraceSingleForObjects` _returnvalue (+ _returnvalue (* (`SceneComponent.GetRightVector` _scene) (* (`self.Range`) -1.0))) (`|MakeArray` "ObjectTypeQuery1" "ObjectTypeQuery2" "ObjectTypeQuery3" :!type "EObjectTypeQuery Enum")))
    (bind (_bblockinghit _binitialoverlap _time _distance _location _impactpoint _normal _impactnormal _physmat _hitactor) (`GameplayStatics.BreakHitResult` _outhit))
    (`SceneComponent.K2_SetWorldLocation` (`self.ParticleSystem`) _location false false)
    (if (`KismetSystemLibrary.DoesImplementInterface` _hitactor "/Game/Blueprints/CanTakeDamage.CanTakeDamage_C")
      (message `/Game/Blueprints/CanTakeDamage.TakeDamage` _hitactor (`self.Damage`) "NewEnumerator0"))))

(fn `UserConstructionScript`)