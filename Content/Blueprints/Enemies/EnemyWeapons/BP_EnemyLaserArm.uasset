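; Enemy laser arm weapon that fires a continuous beam in random-length bursts separated by random pauses, until MakeBroken disables it.
; A fast looping timer line-traces forward or backward by Direction, stretching the beam mesh, placing sparks and damaging CanTakeDamage actors.
; While firing, damage, glow and a burnout value ramp up, then decay during pauses.
; Burnout drives the arm's color curve and the laser sound's volume and pitch.
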(event `self.ReceiveBeginPlay`
  (bind _returnvalue (`KismetMaterialLibrary.CreateDynamicMaterialInstance` "/Game/Materials/M_lightning.M_lightning"))
  (bind _output_get (set `self.LaserMat` _returnvalue))
  (`PrimitiveComponent.SetMaterial` (`self.LaserMesh`) 0 _output_get)
  (bind _returnvalue_2 (`KismetMaterialLibrary.CreateDynamicMaterialInstance` "/Game/Materials/M_LaserArm.M_LaserArm"))
  (bind _output_get_2 (set `self.Mat` _returnvalue_2))
  (`PrimitiveComponent.SetMaterial` (`self.MechPart`) 0 _output_get_2)
  (`MaterialInstanceDynamic.SetScalarParameterValue` _output_get_2 "Glow" 0.5)
  (`MaterialInstanceDynamic.SetScalarParameterValue` (`self.Mat`) "Glow" 0.5)
  (`MaterialInstanceDynamic.SetScalarParameterValue` (`self.Mat`) "ChargeAmount" 1.0)
  (`self.ResetLaser`))

(event `self.StopFiring`
  (`KismetSystemLibrary.K2_ClearAndInvalidateTimerHandle` (stale `self.BeginFiring` _returnvalue_2))
  (`KismetSystemLibrary.K2_ClearAndInvalidateTimerHandle` (stale `BreakFiring` _returnvalue))
  (`KismetSystemLibrary.K2_ClearAndInvalidateTimerHandle` (stale `self.BeginFiring` _returnvalue))
  (set `self.Input` 0.0)
  (`self.ResetLaser`))

(event `self.BeginFiring`
  (if (not (`self.Broken`))
    (bind _returnvalue (`KismetSystemLibrary.K2_SetTimerDelegate` (delegate `BreakFiring`) (`KismetMathLibrary.RandomFloatInRange` 1.5 6.0)))
    (bind _returnvalue_2 (`KismetSystemLibrary.K2_SetTimerDelegate` (delegate `self.EnemyAttack_Constant`) 0.01 true))
    (set `self.Input` 1.0)))

(event `BreakFiring`
  (set `self.Input` 0.0)
  (bind _returnvalue (`KismetSystemLibrary.K2_SetTimerDelegate` (delegate `self.BeginFiring`) (`KismetMathLibrary.RandomFloatInRange` 3.0 5.0))))

(event `self.EnemyAttack_Constant`
  (bind _lasermesh (`self.LaserMesh`))
  (bind _damage (`self.Damage`))
  (bind _basedamage (`self.BaseDamage`))
  (bind _maxdamage (`self.MaxDamage`))
  (bind _timetoburnout (`self.TimeToBurnout`))
  (bind _glowval (`self.GlowVal`))
  (bind _wav_laser (`self.WAV_Laser`))
  (bind _returnvalue (/ (`self.CurrentBurnout`) (`self.TimeToBurnout`)))
  (bind _returnvalue_2 (+ (`self.CurrentBurnout`) (`GameplayStatics.GetWorldDeltaSeconds`)))
  (if (> (`self.Input`) 0.0)
    (`self.LaserTrace`)
    (`ParticleSystemComponent.SetFloatParameter` (`self.P_Sparks`) "Rate" (+ (* _glowval 6.0) 50.0))
    (bind _output_get (set `self.GlowVal` (`KismetMathLibrary.FClamp` (+ _glowval 0.5) 0.0 150.0)))
    (`MaterialInstanceDynamic.SetScalarParameterValue` (`self.LaserMat`) "Glow" _output_get)
    (set `self.Damage` (`KismetMathLibrary.FClamp` (+ _damage 1.2e-05) _basedamage _maxdamage))
    (`AudioComponent.SetFloatParameter` _wav_laser "LaserVol" _returnvalue)
    (`AudioComponent.SetFloatParameter` _wav_laser "LaserPitch" _returnvalue)
    (`MaterialInstanceDynamic.SetVectorParameterValue` (`self.Mat`) "Color" (`CurveLinearColor.GetLinearColorValue` (`self.ColorCurve`) (/ (`self.CurrentBurnout`) (`self.TimeToBurnout`))))
    (set `self.CurrentBurnout` (`KismetMathLibrary.FClamp` _returnvalue_2 0.0 _timetoburnout))
    (if (not (>= _returnvalue_2 _timetoburnout))
      (`/Engine/EditorBlueprintResources/StandardMacros.DoOnce` false :!label _label
        (:`Completed`
          (`SceneComponent.SetHiddenInGame` _lasermesh false false)
          (`AudioComponent.FadeIn` (`self.WAV_Laser`) 0.005 1.0 0.0)
          (`ActorComponent.SetActive` (`self.P_Sparks`) true false)
          (goto _label_2 :!via `Reset`))))
    (else
      (set `self.Damage` (`KismetMathLibrary.FClamp` (+ _damage -6e-05) _basedamage _maxdamage))
      (set `self.GlowVal` (`KismetMathLibrary.FClamp` (+ _glowval -1.0) 0.0 150.0))
      (`MaterialInstanceDynamic.SetVectorParameterValue` (`self.Mat`) "Color" (`CurveLinearColor.GetLinearColorValue` (`self.ColorCurve`) (/ (`self.CurrentBurnout`) (`self.TimeToBurnout`))))
      (set `self.CurrentBurnout` (`KismetMathLibrary.FClamp` (- (`self.CurrentBurnout`) (* (`GameplayStatics.GetWorldDeltaSeconds`) 2.0)) 0.0 (`self.TimeToBurnout`)))
      (`/Engine/EditorBlueprintResources/StandardMacros.DoOnce` false :!label _label_2
        (:`Completed`
          (`SceneComponent.SetHiddenInGame` _lasermesh true false :!label _label_3)
          (`AudioComponent.FadeOut` (`self.WAV_Laser`) 0.1 0.0)
          (`ActorComponent.SetActive` (`self.P_Sparks`) false false)
          (goto _label :!via `Reset`))))))

(event `ResetLaser`
  (goto _label_3))

(event `self.MakeBroken`
  (bind _p_sparks (`self.P_Sparks`))
  (bind _lasermesh (`self.LaserMesh`))
  (`ActorComponent.SetActive` _p_sparks true false)
  (`SceneComponent.K2_SetWorldLocation` _p_sparks (`SceneComponent.K2_GetComponentLocation` _lasermesh) false false)
  (`SceneComponent.SetHiddenInGame` _lasermesh true false)
  (`ActorComponent.SetActive` (`self.P_Broken`) true false)
  (`AudioComponent.Stop` (`self.WAV_Laser`))
  (`self.StopFiring`)
  (set `self.Broken` true))

(fn `LaserTrace`
  (bind _array (`|MakeArray` "ObjectTypeQuery1" "ObjectTypeQuery2" :!type "EObjectTypeQuery Enum"))
  (bind _lasermesh (`self.LaserMesh`))
  (bind _lasermesh_2 (`self.LaserMesh`))
  (bind _p_sparks (`self.P_Sparks`))
  (bind _lasermesh_3 (`self.LaserMesh`))
  (bind _lasermesh_4 (`self.LaserMesh`))
  (bind _p_sparks_2 (`self.P_Sparks`))
  (bind _returnvalue (`SceneComponent.K2_GetComponentLocation` _lasermesh))
  (bind _returnvalue_2 (`SceneComponent.K2_GetComponentLocation` _lasermesh_3))
  (if (`self.Direction`)
    (bind (_outhit _returnvalue_3) (`KismetSystemLibrary.LineTraceSingleForObjects` _returnvalue_2 (+ _returnvalue_2 (* (`SceneComponent.GetForwardVector` _lasermesh_3) (* (`self.Range`) -1.0))) _array))
    (if _returnvalue_3
      (bind (_bblockinghit _binitialoverlap _time _distance _location _impactpoint _normal _impactnormal _physmat _hitactor _hitcomponent _hitbonename _hititem _faceindex _tracestart) (`GameplayStatics.BreakHitResult` _outhit))
      (`SceneComponent.SetWorldScale3D` _lasermesh_4 (`KismetMathLibrary.MakeVector` (* (/ (`KismetMathLibrary.VSize` (- _location _tracestart)) 195.0) -1.0) 0.5 0.5))
      (`SceneComponent.K2_SetWorldLocation` _p_sparks_2 _location false false)
      (if (`KismetSystemLibrary.DoesImplementInterface` _hitactor "/Game/Blueprints/CanTakeDamage.CanTakeDamage_C")
        (message `/Game/Blueprints/CanTakeDamage.TakeDamage` _hitactor (`self.Damage`) "NewEnumerator1"))
      (else
        (`SceneComponent.SetWorldScale3D` _lasermesh_4 (-3000.0 0.5 0.5))
        (`SceneComponent.K2_SetWorldLocation` _p_sparks_2 (0.0 0.0 -500.0) false false)))
    (else
      (bind (_outhit_2 _returnvalue_4) (`KismetSystemLibrary.LineTraceSingleForObjects` _returnvalue (+ _returnvalue (* (`SceneComponent.GetForwardVector` _lasermesh) (`self.Range`))) _array))
      (if _returnvalue_4
        (bind (_bblockinghit_2 _binitialoverlap_2 _time_2 _distance_2 _location_2 _impactpoint_2 _normal_2 _impactnormal_2 _physmat_2 _hitactor_2 _hitcomponent_2 _hitbonename_2 _hititem_2 _faceindex_2 _tracestart_2) (`GameplayStatics.BreakHitResult` _outhit_2))
        (`SceneComponent.SetWorldScale3D` _lasermesh_2 (`KismetMathLibrary.MakeVector` (/ (`KismetMathLibrary.VSize` (- _location_2 _tracestart_2)) 195.0) 0.5 0.5))
        (`SceneComponent.K2_SetWorldLocation` _p_sparks _location_2 false false)
        (if (`KismetSystemLibrary.DoesImplementInterface` _hitactor_2 "/Game/Blueprints/CanTakeDamage.CanTakeDamage_C")
          (message `/Game/Blueprints/CanTakeDamage.TakeDamage` _hitactor_2 (`self.Damage`) "NewEnumerator1"))
        (else
          (`SceneComponent.SetWorldScale3D` _lasermesh_2 (3000.0 0.5 0.5))
          (`SceneComponent.K2_SetWorldLocation` _p_sparks (0.0 0.0 -500.0) false false))))))

(fn `UserConstructionScript`)