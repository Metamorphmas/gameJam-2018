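; BP_EnemyArm is an enemy arm actor that takes damage as an attached part of a BP_EnemyPawn.
; On damage it casts its parent actor to BP_EnemyPawn and forwards a quarter of the hit, stopping if the cast fails.
; It then reduces its own Health by armor-scaled damage, clamped between zero and one, and calls CheckHealth.
; Init, firing and attack functions are empty stubs.
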(event `self.ReceiveBeginPlay`)

(event `self.TakeDamage`
  (params (Damage :type "Float (single-precision)") (DamageType :type "/Game/Blueprints/Enums/DamageType Enum" :default "NewEnumerator5"))
  (bind _asbp_enemy_pawn (cast `/Game/Blueprints/Enemies/BP_EnemyPawn` (`self.GetParentActor`)))
  (`/Game/Blueprints/Enemies/BP_EnemyPawn.TakeDamage` _asbp_enemy_pawn (* Damage 0.25) DamageType)
  (set `self.Health` (`KismetMathLibrary.FClamp` (- (`self.Health`) (* Damage (- 1.0 (`self.Armor`))))))
  (`/Game/Blueprints/CanTakeDamage.CheckHealth`))

(fn `BeginFiring`)

(fn `EnemyAttack_Constatnt`)

(fn `EnemyAttack_Once`)

(fn `Init`)

(fn `StopFiring`)

(fn `UserConstructionScript`)