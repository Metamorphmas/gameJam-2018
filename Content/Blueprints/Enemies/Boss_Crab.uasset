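; Giant crab boss fight that sidesteps across its arena, tracks the player and alternates between firing and blocking with its claws.
; A looping Update timer drives random walking and lerped aiming of child-actor gatling and laser arms, alongside guided rocket arms.
; Per-part damage destroys claws and escalates speed or rocket fire, while body damage triggers phase reactions.
; Low health starts a recurring charged mega-laser, and death spawns a shell and fragments.
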(event `HasKilledPlayer`
  (set `self.IsFiring` false)
  (`KismetSystemLibrary.K2_ClearAndInvalidateTimerHandle` (stale `StartFight` _returnvalue)))

(event `BeginChargingLaser`
  (`AudioComponent.FadeIn` (`self.WAV_JavelinCharge`) 1.0 1.0 0.0)
  (`KismetSystemLibrary.K2_SetTimerDelegate` (delegate `FireLaser`) 5.0)
  (`/Engine/EditorBlueprintResources/StandardMacros.DoOnce` false
    (:`Completed`
      (bind _returnvalue (`KismetMaterialLibrary.CreateDynamicMaterialInstance` "/Game/Materials/MI_BigLaser.MI_BigLaser"))
      (bind _output_get (set `self.LaserMat` _returnvalue))
      (`PrimitiveComponent.SetMaterial` (`self.BigAssLaser`) 0 _output_get)
      (set `self.BigLaser` true))))

(event `MoveClawsToBlock`
  (bind _gat (`self.Gat`))
  (bind _laser (`self.Laser`))
  (bind _boss_crab_clawleft_lower (`self.Boss_Crab_ClawLeft_Lower`))
  (bind _gat_2 (`self.Gat`))
  (bind _boss_crab_clawright_lower (`self.Boss_Crab_ClawRight_Lower`))
  (bind _laser_2 (`self.Laser`))
  ;[1 1 1] Blocking
  (`|ExecutionSequence`
    (:`then_0`
      (if (`KismetSystemLibrary.IsValid` _boss_crab_clawleft_lower)
        (`SceneComponent.K2_SetWorldRotation` _boss_crab_clawleft_lower (`KismetMathLibrary.RLerp` (`SceneComponent.K2_GetComponentRotation` _boss_crab_clawleft_lower) (`self.LeftClawRot`) 0.02 true) false false)
        (`/Engine/EditorBlueprintResources/StandardMacros.DoOnce` false :!label _label
          (:`Completed`
            (if (`KismetSystemLibrary.IsValid` _gat)
              (`/Game/Blueprints/Enemies/EnemyWeapons/BP_EnemyArm.StopFiring` _gat)
              (`self.CloseLeft`)
              (goto _label_4 :!via `Reset`))))))
    (:`then_1`
      (if (`KismetSystemLibrary.IsValid` _boss_crab_clawright_lower)
        (`SceneComponent.K2_SetWorldRotation` _boss_crab_clawright_lower (`KismetMathLibrary.RLerp` (`SceneComponent.K2_GetComponentRotation` _boss_crab_clawright_lower) (`self.RightClawRot`) 0.02 true) false false)
        (`/Engine/EditorBlueprintResources/StandardMacros.DoOnce` false :!label _label_2
          (:`Completed`
            (if (`KismetSystemLibrary.IsValid` _laser)
              (`/Game/Blueprints/Enemies/EnemyWeapons/BP_EnemyArm.StopFiring` _laser)
              (`self.CloseRight`)
              (goto _label_5 :!via `Reset`))))))
    (:`then_2`
      (`/Engine/EditorBlueprintResources/StandardMacros.DoOnce` false :!label _label_3
        (:`Completed`
          (`KismetSystemLibrary.K2_SetTimerDelegate` (delegate `StopBlocking`) (`KismetMathLibrary.RandomFloatInRange` 9.0 12.0))
          (goto _label_6 :!via `Reset`))))))

(event `FireLaser`
  (`SceneComponent.SetHiddenInGame` (`self.BigAssLaser`) false false)
  (`PrimitiveComponent.SetCollisionEnabled` (`self.LaserColl`) "QueryAndPhysics")
  (`KismetSystemLibrary.K2_SetTimerDelegate` (delegate `StopLaser`) 2.2)
  (`GameplayStatics.PlaySoundAtLocation` "/Game/Audio/WAV_JavelinFire.WAV_JavelinFire" (0.0 0.0 0.0) (struct) 0.7 0.4 0.0 null null null)
  (`GameplayStatics.PlaySoundAtLocation` "/Game/Audio/WAV_JavelinFire.WAV_JavelinFire" (0.0 0.0 0.0) (struct) 0.7 1.0 0.0 null null null)
  (bind (_direction _laserglow) (`Timeline|LaserGlow` :!via `PlayFromStart`)
    (:`Update`
      (`MaterialInstanceDynamic.SetScalarParameterValue` (`self.LaserMat`) "Glow" _laserglow))))

(event `StopBlocking`
  ;[1 1 1] Blocking
  (set `self.IsFiring` true))

(event `StopLaser`
  (`SceneComponent.SetHiddenInGame` (`self.BigAssLaser`) true false)
  (`PrimitiveComponent.SetCollisionEnabled` (`self.LaserColl`) "NoCollision")
  (`KismetSystemLibrary.K2_SetTimerDelegate` (delegate `BeginChargingLaser`) (`KismetMathLibrary.RandomFloatInRange` 3.0 6.0))
  (set `self.Glow` 0.0))

(event `Update`
  (bind _mech_head1 (`self.Mech_Head1`))
  (bind (_returnvalue_roll _returnvalue_pitch _returnvalue_yaw) (`KismetMathLibrary.BreakRotator` (`KismetMathLibrary.FindLookAtRotation` (`SceneComponent.K2_GetComponentLocation` _mech_head1) (`self.K2_GetActorLocation` (`self.Target`)))))
  ;[1 1 1] Update
  (if (`KismetSystemLibrary.IsValid` (`self.Target`))
    (`|ExecutionSequence`
      (:`then_0`
        (if (`self.Walking`)
          _
          (elif (== (`KismetMathLibrary.RandomIntegerInRange` 0 (`self.MoveChance`)) 0)
            (if (== (`KismetMathLibrary.RandomIntegerInRange` 0 1) 0)
              (`self.StartWalkRight`)
              (else
                (`self.StartWalkLeft`))))))
      (:`then_1`
        (`SceneComponent.K2_SetWorldRotation` _mech_head1 (`KismetMathLibrary.RLerp` (`SceneComponent.K2_GetComponentRotation` _mech_head1) (`KismetMathLibrary.MakeRotator` 0.0 0.0 (+ _returnvalue_yaw -90.0)) 0.02 true) false false))
      (:`then_2`
        (if (`self.IsFiring`)
          (`self.FireClawWeapons`)
          (else
            (`self.MoveClawsToBlock`)))))
    (else
      (`self.HasKilledPlayer`))))

(event `FireClawWeapons`
  (bind _boss_crab_clawleft_lower (`self.Boss_Crab_ClawLeft_Lower`))
  (bind _boss_crab_clawright_lower (`self.Boss_Crab_ClawRight_Lower`))
  (bind _gat (`self.Gat`))
  (bind _laser (`self.Laser`))
  (bind (_returnvalue_x _returnvalue_y _returnvalue_z) (`KismetMathLibrary.BreakVector` (`self.K2_GetActorLocation` (`self.Target`))))
  (bind (_returnvalue_roll _returnvalue_pitch _returnvalue_yaw) (`KismetMathLibrary.BreakRotator` (`KismetMathLibrary.FindLookAtRotation` (`SceneComponent.K2_GetComponentLocation` _boss_crab_clawleft_lower) (`self.K2_GetActorLocation` (`self.Target`)))))
  (bind (_returnvalue_roll_2 _returnvalue_pitch_2 _returnvalue_yaw_2) (`KismetMathLibrary.BreakRotator` (`KismetMathLibrary.FindLookAtRotation` (`SceneComponent.K2_GetComponentLocation` _boss_crab_clawright_lower) (`KismetMathLibrary.MakeVector` _returnvalue_x _returnvalue_y (+ _returnvalue_z 300.0)))))
  ;[1 1 1] Attacking
  (`|ExecutionSequence`
    (:`then_0`
      (if (`KismetSystemLibrary.IsValid` _boss_crab_clawleft_lower)
        (`SceneComponent.K2_SetWorldRotation` _boss_crab_clawleft_lower (`KismetMathLibrary.RLerp` (`SceneComponent.K2_GetComponentRotation` _boss_crab_clawleft_lower) (`KismetMathLibrary.MakeRotator` _returnvalue_roll _returnvalue_pitch (+ _returnvalue_yaw -20.0)) 0.06 true) false false)
        (`/Engine/EditorBlueprintResources/StandardMacros.DoOnce` false :!label _label_4
          (:`Completed`
            (if (`KismetSystemLibrary.IsValid` _gat)
              (`/Game/Blueprints/Enemies/EnemyWeapons/BP_EnemyArm.BeginFiring` _gat)
              (`self.OpenLeft`)
              (goto _label :!via `Reset`))))))
    (:`then_1`
      (if (`KismetSystemLibrary.IsValid` _boss_crab_clawright_lower)
        (`SceneComponent.K2_SetWorldRotation` _boss_crab_clawright_lower (`KismetMathLibrary.RLerp` (`SceneComponent.K2_GetComponentRotation` _boss_crab_clawright_lower) (`KismetMathLibrary.MakeRotator` _returnvalue_roll_2 _returnvalue_pitch_2 (+ _returnvalue_yaw_2 200.0)) 0.06 true) false false)
        (`/Engine/EditorBlueprintResources/StandardMacros.DoOnce` false :!label _label_5
          (:`Completed`
            (if (`KismetSystemLibrary.IsValid` _laser)
              (`/Game/Blueprints/Enemies/EnemyWeapons/BP_EnemyArm.BeginFiring` _laser)
              (`self.OpenLeft`)
              (goto _label_2 :!via `Reset`))))))
    (:`then_2`
      (`/Engine/EditorBlueprintResources/StandardMacros.DoOnce` false :!label _label_6
        (:`Completed`
          (goto _label_3 :!via `Reset`))))))

(event `OpenLeft`
  ;[1 1 1] Attacking
  (bind (_direction _rot) (`Timeline|ClawLeftOpen` :!via `PlayFromStart` :!label _label_7)
    (:`Update`
      (`SceneComponent.K2_SetRelativeRotation` (`self.Boss_Crab_ClawLeft_Upper`) (`KismetMathLibrary.MakeRotator` 0.0 _rot 20.0) false false))))

(event `CloseLeft`
  ;[1 1 1] Attacking
  (goto _label_7 :!via `ReverseFromEnd`))

(event `OpenRight`
  ;[1 1 1] Attacking
  (bind (_direction _rot) (`Timeline|ClawRightOpen` :!via `PlayFromStart` :!label _label_8)
    (:`Update`
      (`SceneComponent.K2_SetRelativeRotation` (`self.Boss_Crab_ClawRight_Upper`) (`KismetMathLibrary.MakeRotator` 0.0 _rot -20.0) false false))))

(event `CloseRight`
  ;[1 1 1] Attacking
  (goto _label_8 :!via `ReverseFromEnd`))

(event `StartFight`
  ;[1 1 1] BeginPlay
  (`KismetSystemLibrary.PrintString` "STARTED")
  (bind _returnvalue (`KismetSystemLibrary.K2_SetTimerDelegate` (delegate `Update`) 0.02 true))
  (`self.Init`)
  (`SkeletalMeshComponent.SetPlayRate` (`self.Boss_Crab_Claws_Skeleton`) 2.0)
  (`self.Stage1`))

(event `StartWalkLeft`
  ;[1 1 1] Walking
  (bind _returnvalue (`KismetSystemLibrary.K2_SetTimerDelegate` (delegate `Walk`) 0.02 true))
  (set `self.WalkTimer` _returnvalue)
  (set `self.Walking` true)
  (bind _returnvalue_2 (`KismetSystemLibrary.K2_SetTimerDelegate` (delegate `StopWalking`) (`KismetMathLibrary.RandomFloatInRange` 3.0 9.0)))
  (set `self.StopWalkingTimer` _returnvalue_2)
  (set `self.Speed` (* (`self.SpeedMax`) -1.0))
  (`AudioComponent.FadeIn` (`self.WAV_BipedFootsteps`) 0.1 1.0 0.0 :!label _label_9)
  (bind _asbp_dmg_taking_vol (cast `/Game/Meshes/Characters/Crab/BP_DmgTakingVol` (`ChildActorComponent.ChildActor` (`self.Legs1_DmgTakingVol`))))
  (set `/Game/Meshes/Characters/Crab/BP_DmgTakingVol.DealDmg` true _asbp_dmg_taking_vol)
  (bind _asbp_dmg_taking_vol_2 (cast `/Game/Meshes/Characters/Crab/BP_DmgTakingVol` (`ChildActorComponent.ChildActor` (`self.Legs2_DmgTakingVol`))))
  (set `/Game/Meshes/Characters/Crab/BP_DmgTakingVol.DealDmg` true _asbp_dmg_taking_vol_2))

(event `Stage1`
  ;[1 1 1] Boss Stages
  (set `self.IsFiring` false)
  (`KismetSystemLibrary.K2_SetTimerDelegate` (delegate `Stage2`) 10.0))

(event `Stage2`
  ;[1 1 1] Boss Stages
  (set `self.IsFiring` true))

(event `StartWalkRight`
  ;[1 1 1] Walking
  (bind _returnvalue (`KismetSystemLibrary.K2_SetTimerDelegate` (delegate `Walk`) 0.02 true))
  (set `self.WalkTimer` _returnvalue)
  (set `self.Walking` true)
  (bind _returnvalue_2 (`KismetSystemLibrary.K2_SetTimerDelegate` (delegate `StopWalking`) (`KismetMathLibrary.RandomFloatInRange` 3.0 9.0)))
  (set `self.StopWalkingTimer` _returnvalue_2)
  (set `self.Speed` (`self.SpeedMax`))
  (goto _label_9))

(event `Walk`
  (bind _boss_crab_shell (`self.Boss_Crab_Shell`))
  (bind (_relativelocation_x _relativelocation_y _relativelocation_z) (`KismetMathLibrary.BreakVector` (`SceneComponent.RelativeLocation` _boss_crab_shell)))
  (bind _returnvalue (+ _relativelocation_y (`self.Speed`)))
  ;[1 1 1] Walking
  (`SceneComponent.K2_SetRelativeLocation` _boss_crab_shell (`KismetMathLibrary.MakeVector` _relativelocation_x _returnvalue _relativelocation_z) true false)
  (if (>= _returnvalue (`self.WalkMax`))
    (`self.StopWalking`)
    (`/Engine/EditorBlueprintResources/StandardMacros.IncrementFloat` (`self.WalkMax`))
    (elif (<= _returnvalue (`self.WalkMin`))
      (`self.StopWalking`)
      (`/Engine/EditorBlueprintResources/StandardMacros.DecrementFloat` (`self.WalkMin`)))))

(event `self.ReceiveBeginPlay`
  (`PrimitiveComponent.SetCollisionEnabled` (`self.LaserColl`) "NoCollision"))

(event `StopWalking`
  ;[1 1 1] Walking
  (`SkeletalMeshComponent.Stop` (`self.Legs1`))
  (`SkeletalMeshComponent.Stop` (`self.Legs2`))
  (`KismetSystemLibrary.K2_ClearAndInvalidateTimerHandle` (`self.WalkTimer`))
  (`KismetSystemLibrary.K2_ClearAndInvalidateTimerHandle` (`self.StopWalkingTimer`))
  (set `self.Walking` false)
  (set `self.Speed` 0.0)
  (`AudioComponent.FadeOut` (`self.WAV_BipedFootsteps`) 0.1 0.0)
  (bind _asbp_dmg_taking_vol (cast `/Game/Meshes/Characters/Crab/BP_DmgTakingVol` (`ChildActorComponent.ChildActor` (`self.Legs1_DmgTakingVol`))))
  (set `/Game/Meshes/Characters/Crab/BP_DmgTakingVol.DealDmg` true _asbp_dmg_taking_vol)
  (bind _asbp_dmg_taking_vol_2 (cast `/Game/Meshes/Characters/Crab/BP_DmgTakingVol` (`ChildActorComponent.ChildActor` (`self.Legs2_DmgTakingVol`))))
  (set `/Game/Meshes/Characters/Crab/BP_DmgTakingVol.DealDmg` true _asbp_dmg_taking_vol_2))

(event `Init`
  (bind _arenawidth (`self.ArenaWidth`))
  (bind (_relativelocation_x _relativelocation_y) (`KismetMathLibrary.BreakVector` (`SceneComponent.RelativeLocation` (`self.Boss_Crab_Shell`))))
  ;[1 1 1] Initialization
  (`|ExecutionSequence`
    (:`then_0`
      (set `self.WalkMax` (+ _relativelocation_y _arenawidth))
      (set `self.WalkMin` (- _relativelocation_y _arenawidth))
      (bind _asbp_enemy_arm (cast `/Game/Blueprints/Enemies/EnemyWeapons/BP_EnemyArm` (`ChildActorComponent.ChildActor` (`self.BP_EnemyLaserArm`))))
      (bind _output_get (set `self.Laser` _asbp_enemy_arm))
      (set `/Game/Blueprints/Enemies/EnemyWeapons/BP_EnemyArm.Damage` (* (`/Game/Blueprints/Enemies/EnemyWeapons/BP_EnemyArm.Damage` _output_get) 2.2) _output_get)
      (bind _asbp_enemy_arm_2 (cast `/Game/Blueprints/Enemies/EnemyWeapons/BP_EnemyArm` (`ChildActorComponent.ChildActor` (`self.BP_EnemyGatlingArm`))))
      (bind _output_get_2 (set `self.Gat` _asbp_enemy_arm_2))
      (set `/Game/Blueprints/Enemies/EnemyWeapons/BP_EnemyArm.Damage` (* (`/Game/Blueprints/Enemies/EnemyWeapons/BP_EnemyArm.Damage` _output_get_2) 4.0) _output_get_2)
      (bind _outactors (`GameplayStatics.GetAllActorsOfClass` "/Game/Blueprints/PlayerCharacter_Final.PlayerCharacter_Final_C"))
      (bind _output_get_3 (set `self.Target` (`|GetArrayItem` _outactors)))
      (bind _asbp_enemy_rocket_arm (cast `/Game/Blueprints/Enemies/EnemyWeapons/BP_EnemyRocketArm` (`ChildActorComponent.ChildActor` (`self.RocketArm1`))))
      (set `/Game/Blueprints/Enemies/EnemyWeapons/BP_EnemyRocketArm.Target` _output_get_3 _asbp_enemy_rocket_arm)
      (set `/Game/Blueprints/Enemies/EnemyWeapons/BP_EnemyRocketArm.Guided` true _asbp_enemy_rocket_arm)
      (bind _asbp_enemy_rocket_arm_2 (cast `/Game/Blueprints/Enemies/EnemyWeapons/BP_EnemyRocketArm` (`ChildActorComponent.ChildActor` (`self.RocketArm2`))))
      (set `/Game/Blueprints/Enemies/EnemyWeapons/BP_EnemyRocketArm.Target` _output_get_3 _asbp_enemy_rocket_arm_2)
      (set `/Game/Blueprints/Enemies/EnemyWeapons/BP_EnemyRocketArm.Guided` true _asbp_enemy_rocket_arm_2)
      (`/Game/Blueprints/Enemies/EnemyWeapons/BP_EnemyArm.BeginFiring` _asbp_enemy_rocket_arm))
    (:`then_1`
      (set `self.LeftClawRot` (`SceneComponent.K2_GetComponentRotation` (`self.Boss_Crab_ClawLeft_Lower`)))
      (set `self.RightClawRot` (`SceneComponent.K2_GetComponentRotation` (`self.Boss_Crab_ClawRight_Lower`)))
      (`PrimitiveComponent.SetCollisionEnabled` (`self.LaserColl`) "NoCollision")
      (bind _ascrab_boss_health_bar (cast `/Game/UI/CrabBossHealthBar` (`WidgetComponent.GetUserWidgetObject` (`self.HealthBar`))))
      (set `/Game/UI/CrabBossHealthBar.Enemy` self _ascrab_boss_health_bar))))

(event `TakePartDmg`
  (params (LeftLeg :type Boolean) (RightLeg :type Boolean) (LeftClaw :type Boolean) (RightClaw :type Boolean) (Center :type Boolean) (Dmg :type "Float (double-precision)"))
  (bind _boss_crab_clawleft_lower (`self.Boss_Crab_ClawLeft_Lower`))
  (bind _boss_crab_clawright_lower (`self.Boss_Crab_ClawRight_Lower`))
  (bind _returnvalue (`SceneComponent.K2_GetComponentLocation` _boss_crab_clawright_lower))
  (bind _returnvalue_2 (`SceneComponent.K2_GetComponentLocation` _boss_crab_clawleft_lower))
  ;[1 1 1] Take damage and destroy parts
  (`|ExecutionSequence`
    (:`then_0`
      (if LeftLeg
        (bind _output_get (set `self.LeftLegHealth` (- (`self.LeftLegHealth`) Dmg)))
        (`KismetSystemLibrary.PrintString` (`KismetStringLibrary.Concat_StrStr` "LeftLegHealth:" (`KismetStringLibrary.Conv_DoubleToString` _output_get)))
        (elif RightLeg
          (bind _output_get_2 (set `self.RightLegHealth` (- (`self.RightLegHealth`) Dmg)))
          (`KismetSystemLibrary.PrintString` (`KismetStringLibrary.Concat_StrStr` "RightLegHealth:" (`KismetStringLibrary.Conv_DoubleToString` _output_get_2)))
          (elif LeftClaw
            (bind _output_get_3 (set `self.LeftClawHealth` (- (`self.LeftClawHealth`) Dmg)))
            (`KismetSystemLibrary.PrintString` (`KismetStringLibrary.Concat_StrStr` "LeftClawHealth:" (`KismetStringLibrary.Conv_DoubleToString` _output_get_3)))
            (if (<= _output_get_3 0.0)
              (`SceneComponent.SetHiddenInGame` _boss_crab_clawleft_lower true true)
              (`self.K2_DestroyActor` (`ChildActorComponent.ChildActor` (`self.LeftClaw_DmgTakingVol`)))
              (`GameplayStatics.SpawnEmitterAtLocation` "/Game/ParticleEffects/P_Explosion.P_Explosion" _returnvalue_2 (struct) (5.0 5.0 5.0))
              (`GameplayStatics.PlaySoundAtLocation` "/Game/Audio/WAV_Explosion1_Reverb.WAV_Explosion1_Reverb" _returnvalue_2 (struct) 0.5 1.0 0.0 null null null)
              (`ActorComponent.SetActive` (`self.Fire_LeftClaw`) true false)
              (`self.K2_DestroyActor` (`ChildActorComponent.ChildActor` (`self.BP_EnemyGatlingArm`)))
              (if (`self.IsFiring`) :!label _label_10
                (set `self.IsFiring` true))
              (bind _result (`/Engine/EditorBlueprintResources/StandardMacros.DecrementInt` (`self.RemainingClaws`))
                (:`  `
                  (`AudioComponent.Play` (`self.WAV_Alert`) 0.0)
                  (switch `int` _result
                    (:`0`
                      (`self.StopLaser`)
                      (set `self.SpeedMax` 16.0)
                      (set `self.MoveChance` 30)
                      (`AudioComponent.SetPitchMultiplier` (`self.WAV_BipedFootsteps`) 2.1))
                    (:`1`
                      (bind _asbp_enemy_arm (cast `/Game/Blueprints/Enemies/EnemyWeapons/BP_EnemyArm` (`ChildActorComponent.ChildActor` (`self.RocketArm2`))))
                      (`/Game/Blueprints/Enemies/EnemyWeapons/BP_EnemyArm.BeginFiring` _asbp_enemy_arm)
                      (set `self.SpeedMax` 11.0)
                      (set `self.MoveChance` 40)
                      (set `self.IsFiring` true)
                      (`AudioComponent.SetPitchMultiplier` (`self.WAV_BipedFootsteps`) 1.5))))))
            (elif RightClaw
              (bind _output_get_4 (set `self.RightClawHealth` (- (`self.RightClawHealth`) Dmg)))
              (`KismetSystemLibrary.PrintString` (`KismetStringLibrary.Concat_StrStr` "RightClawHealth:" (`KismetStringLibrary.Conv_DoubleToString` _output_get_4)))
              (if (<= _output_get_4 0.0)
                (`SceneComponent.SetHiddenInGame` _boss_crab_clawright_lower true true)
                (`self.K2_DestroyActor` (`ChildActorComponent.ChildActor` (`self.RightClaw_DmgTakingVol`)))
                (`GameplayStatics.SpawnEmitterAtLocation` "/Game/ParticleEffects/P_Explosion.P_Explosion" _returnvalue (struct) (3.0 3.0 3.0))
                (`GameplayStatics.PlaySoundAtLocation` "/Game/Audio/WAV_Explosion1_Reverb.WAV_Explosion1_Reverb" _returnvalue (struct) 0.5 1.0 0.0 null null null)
                (`ActorComponent.SetActive` (`self.Fire_RightClaw`) true false)
                (`self.K2_DestroyActor` (`ChildActorComponent.ChildActor` (`self.BP_EnemyLaserArm`)))
                (goto _label_10))
              (else
                (bind _output_get_5 (set `self.Health` (- (`self.Health`) Dmg)))
                (set `self.HealthChunk` (- (`self.HealthChunk`) Dmg))
                (`KismetSystemLibrary.PrintString` (`KismetStringLibrary.Concat_StrStr` "CenterHealth:" (`KismetStringLibrary.Conv_DoubleToString` _output_get_5)))
                (`|ExecutionSequence`
                  (:`then_0`
                    (if (<= (`self.HealthChunk`) 0.0)
                      (`AudioComponent.Play` (`self.WAV_Alert`) 0.0)
                      (set `self.HealthChunk` 2.0)
                      (switch `int` (`self.RemainingClaws`)
                        (:`0`
                          (`self.StopLaser`)
                          (bind _asbp_enemy_arm_2 (cast `/Game/Blueprints/Enemies/EnemyWeapons/BP_EnemyArm` (`ChildActorComponent.ChildActor` (`self.RocketArm2`)) :!label _label_11))
                          (`/Game/Blueprints/Enemies/EnemyWeapons/BP_EnemyArm.BeginFiring` _asbp_enemy_arm_2))
                        (:`1`
                          (set `self.IsFiring` false)
                          (goto _label_11))
                        (:`2`
                          (set `self.IsFiring` false)))))
                  (:`then_1`
                    (if (<= _output_get_5 4.0)
                      (if (not (`self.BigLaser`))
                        (`self.BeginChargingLaser`))))
                  (:`then_2`
                    (if (<= _output_get_5 0.0)
                      (`self.Death`))))))))))
    (:`then_1`
      (`/Engine/EditorBlueprintResources/StandardMacros.DoOnce` false
        (:`Completed`
          (`SceneComponent.SetHiddenInGame` (`self.HealthBar`) false false))))))

(event `self.LaserColl.OnComponentBeginOverlap`
  (params (OverlappedComponent :type "PrimitiveComponent Object Reference") (OtherActor :type "Actor Object Reference") (OtherComp :type "PrimitiveComponent Object Reference") (OtherBodyIndex :type Integer) (bFromSweep :type Boolean) (SweepResult :type "HitResult Structure (by ref)"))
  ;[1 1 1] LaserColl
  (if (`KismetSystemLibrary.DoesImplementInterface` OtherActor "/Game/Blueprints/CanTakeDamage.CanTakeDamage_C")
    (if (!= (`self.GetParentActor` OtherActor) self)
      (message `/Game/Blueprints/CanTakeDamage.TakeDamage` OtherActor 0.4 "NewEnumerator1"))))

(event `Death`
  (bind _returnvalue (`self.K2_GetActorLocation`))
  (bind _returnvalue_2 (`SceneComponent.K2_GetComponentToWorld` (`self.Boss_Crab_Shell`)))
  (`GameplayStatics.SpawnEmitterAtLocation` "/Game/ParticleEffects/P_Explosion.P_Explosion" _returnvalue (struct) (18.0 18.0 18.0))
  (`GameplayStatics.PlaySoundAtLocation` "/Game/Audio/WAV_Explosion1_Reverb.WAV_Explosion1_Reverb" _returnvalue (struct) 0.8 0.6 0.0 null null null)
  (`|SpawnActorFromClass` "/Game/Meshes/Characters/Crab/BP_CrabShell.BP_CrabShell_C" _returnvalue_2 "Undefined" "OverrideRootScale" null null)
  (`GameplayStatics.PlaySoundAtLocation` "/Game/Audio/Cue_HeavyAlert.Cue_HeavyAlert" _returnvalue (struct) 0.4 0.3 0.0 null null null)
  (`|SpawnActorFromClass` "/Game/Blueprints/BP_FragmentSpawner.BP_FragmentSpawner_C" _returnvalue_2 "Undefined" "OverrideRootScale" null 500 1.0 null)
  (`self.K2_DestroyActor`))

(fn `UserConstructionScript`)