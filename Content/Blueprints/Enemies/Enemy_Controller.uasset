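; AI controller for enemy pawns that runs the enemy behavior tree and picks their target from what they sense.
; On perception updates it checks only the player pawn's first stimulus, setting the target when sensed and clearing it when not.
; A separate PawnSensing hearing event targets the noise instigator.
; Targets are acquired only when none is held, and are written to both the Enemy blackboard key and the pawn's Target.
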(event `self.ReceiveBeginPlay`
  (`self.RunBehaviorTree` "/Game/Blueprints/Enemies/Enemy_BehaviorTree.Enemy_BehaviorTree"))

(event `self.AIPerception.OnPerceptionUpdated`
  (params (UpdatedActors :type "Array of Actor Object Reference (by ref)"))
  (bind _returnvalue (`AIBlueprintHelperLibrary.GetBlackboard` null))
  (bind _returnvalue_2 (`AIBlueprintHelperLibrary.GetBlackboard` null))
  (bind (_info _returnvalue_3) (`AIPerceptionComponent.GetActorsPerception` (`self.AIPerception`) (`GameplayStatics.GetPlayerPawn` 0)))
  (if _returnvalue_3
    (bind (_target _lastsensedstimuli) (break `ActorPerceptionBlueprintInfo` _info))
    (bind (_output_age _output_expirationage _output_strength _output_stimuluslocation _output_receiverlocation _output_tag _output_bsuccessfullysensed) (break `AIStimulus` (`|GetArrayItem` _lastsensedstimuli)))
    (if _output_bsuccessfullysensed
      (`/Engine/EditorBlueprintResources/StandardMacros.IsValid` (`BlackboardComponent.GetValueAsObject` _returnvalue_2 "Enemy")
        (:`Is Not Valid`
          (`BlackboardComponent.SetValueAsObject` _returnvalue_2 "Enemy" _target)
          (bind _asenemy (cast `/Game/Blueprints/Enemies/Enemy` (`self.K2_GetPawn`)))
          (set `/Game/Blueprints/Enemies/Enemy.Target` _target _asenemy)))
      (else
        (`/Engine/EditorBlueprintResources/StandardMacros.IsValid` (`BlackboardComponent.GetValueAsObject` _returnvalue "Enemy")
          (:`Is Valid`
            (`BlackboardComponent.SetValueAsObject` _returnvalue "Enemy" null)
            (bind _asenemy_2 (cast `/Game/Blueprints/Enemies/Enemy` (`self.K2_GetPawn`)))
            (set `/Game/Blueprints/Enemies/Enemy.Target` null _asenemy_2)))))))

(event `self.PawnSensing.OnHearNoise`
  (params (Instigator :type "Pawn Object Reference") (Location :type "Vector Structure (by ref)") (Volume :type "Float (single-precision)"))
  (bind _returnvalue (`AIBlueprintHelperLibrary.GetBlackboard` null))
  (`/Engine/EditorBlueprintResources/StandardMacros.IsValid` (`BlackboardComponent.GetValueAsObject` _returnvalue "Enemy")
    (:`Is Not Valid`
      (`BlackboardComponent.SetValueAsObject` _returnvalue "Enemy" Instigator)
      (bind _asenemy (cast `/Game/Blueprints/Enemies/Enemy` (`self.K2_GetPawn`)))
      (set `/Game/Blueprints/Enemies/Enemy.Target` Instigator _asenemy))))

(fn `UserConstructionScript`)