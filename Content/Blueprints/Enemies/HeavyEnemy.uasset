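; HeavyEnemy is a robot enemy variant with tougher, harder-hitting arms.
; Its construction script calls SetupRobot to build the robot.
; On Init, it casts the left and right arm child actors to BP_EnemyArm, multiplies each arm's damage and overrides its health.
; The right arm is only adjusted if the left arm cast succeeds.
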(event `self.Init`
  (bind _asbp_enemy_arm (cast `/Game/Blueprints/Enemies/EnemyWeapons/BP_EnemyArm` (`ChildActorComponent.ChildActor` (`self.LeftArm`))))
  (set `/Game/Blueprints/Enemies/EnemyWeapons/BP_EnemyArm.Damage` (* (`/Game/Blueprints/Enemies/EnemyWeapons/BP_EnemyArm.Damage` _asbp_enemy_arm) 2.5) _asbp_enemy_arm)
  (set `/Game/Blueprints/BPMechParts/BP_MechPart.Health` 2.2 _asbp_enemy_arm)
  (bind _asbp_enemy_arm_2 (cast `/Game/Blueprints/Enemies/EnemyWeapons/BP_EnemyArm` (`ChildActorComponent.ChildActor` (`self.RightArm`))))
  (set `/Game/Blueprints/Enemies/EnemyWeapons/BP_EnemyArm.Damage` (* (`/Game/Blueprints/Enemies/EnemyWeapons/BP_EnemyArm.Damage` _asbp_enemy_arm_2) 2.5) _asbp_enemy_arm_2)
  (set `/Game/Blueprints/BPMechParts/BP_MechPart.Health` 2.2 _asbp_enemy_arm_2))

(fn `UserConstructionScript`
  (`self.SetupRobot`))