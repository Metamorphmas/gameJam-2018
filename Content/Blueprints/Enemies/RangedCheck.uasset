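; RangedCheck is a Behavior Tree decorator that gates enemy AI branches, by its name on whether the enemy has a ranged weapon.
; Its AI condition check casts the controlled pawn to Enemy and passes when Arm1Type matches any of seven hard-coded enum values.
; Only the first arm's type is tested.
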(fn `PerformConditionCheckAI`
  (params (OwnerController :type "AIController Object Reference") (ControlledPawn :type "Pawn Object Reference"))
  (returns (ReturnValue :type Boolean))
  (bind _asenemy (cast `/Game/Blueprints/Enemies/Enemy` ControlledPawn))
  (bind _arm1type (`/Game/Blueprints/Enemies/BP_EnemyPawn.Arm1Type` _asenemy))
  (return (or (`|EnumEquality` _arm1type "NewEnumerator0") (`|EnumEquality` _arm1type "NewEnumerator1") (`|EnumEquality` _arm1type "NewEnumerator3") (`|EnumEquality` _arm1type "NewEnumerator4") (`|EnumEquality` _arm1type "NewEnumerator7") (`|EnumEquality` _arm1type "NewEnumerator8") (`|EnumEquality` _arm1type "NewEnumerator9"))))