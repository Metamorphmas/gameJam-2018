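; Player-controlled modular mech Character with independently rotating legs and chassis.
; BeginPlay creates the mouse widget and assembles legs, chassis and two arms from type enums using Child Actor components, with legs setting speed.
; Each tick lerps leg yaw toward eight-way input unless quad legs are locked, while the chassis faces the cursor hit.
; Inputs forward to arm attacks and leg ability; exposed events provide a timeline dash and timer-tracked chassis spin attack.
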(event `Update`
  (bind _mech_legs (`self.Mech_Legs`))
  (bind (_returnvalue_roll _returnvalue_pitch _returnvalue_yaw) (`KismetMathLibrary.BreakRotator` (`SceneComponent.K2_GetComponentRotation` _mech_legs)))
  (`self.SetTargetRot`)
  (bind _asbp_quad_leg (cast `/Game/Blueprints/BPMechParts/BPLegs/BP_QuadLeg` (`ChildActorComponent.ChildActor` _mech_legs))
    (:`then`
      (if (not (`/Game/Blueprints/BPMechParts/BPLegs/BP_QuadLeg.Locked` _asbp_quad_leg))
        (`SceneComponent.K2_SetWorldRotation` _mech_legs (`KismetMathLibrary.MakeRotator` 0.0 0.0 (`KismetMathLibrary.Lerp` _returnvalue_yaw (`self.TargetLegRot`) 0.15)) false false :!label _label)))
    (:`CastFailed`
      (goto _label))))

(event `Dash`
  (bind _dashparticle (`self.DashParticle`))
  (`ActorComponent.SetActive` _dashparticle true false)
  (bind (_direction _dist) (`Timeline|DashTimeline` :!via `PlayFromStart`)
    (:`Update`
      (`self.K2_SetActorLocation` (+ (* (`SceneComponent.GetForwardVector` (`self.Mech_Legs`)) (* _dist (`self.DashPower`))) (`self.K2_GetActorLocation`)) true))
    (:`Finished`
      (`ActorComponent.SetActive` _dashparticle false false))))

(event `self.ReceiveBeginPlay`
  (`self.SetupRobot`)
  (`self.SetupUI`))

(event `self.ReceiveTick`
  (params (DeltaSeconds :type "Float (single-precision)"))
  (`self.Update`))

(event `SpinAttack`
  (params (Directon :type Boolean) (SpinSpeed :type "Float (double-precision)"))
  (bind _returnvalue (* 5.0 SpinSpeed))
  (bind _mech_chassis (`self.Mech_Chassis`))
  (if Directon
    (`SkeletalMeshComponent.PlayAnimation` _mech_chassis "/Game/Animations/Mech_Chassis_StrongAnimations_ChassisRoot_SpinReversed.Mech_Chassis_StrongAnimations_ChassisRoot_SpinReversed" false)
    (`SkeletalMeshComponent.SetPlayRate` _mech_chassis _returnvalue)
    (else
      (`SkeletalMeshComponent.PlayAnimation` _mech_chassis "/Game/Animations/Mech_Chassis_StrongAnimations_ChassisRoot_Spin.Mech_Chassis_StrongAnimations_ChassisRoot_Spin" false)
      (`SkeletalMeshComponent.SetPlayRate` _mech_chassis _returnvalue)))
  (set `self.IsSpinning` true)
  (`KismetSystemLibrary.K2_SetTimer` null "SetIsSpinning" (`KismetMathLibrary.FClamp` (- 1.4 1.0) 0.01 2.0))
  (if (not (`self.V_SpinBreak`))
    (set `self.V_SpinBreak` true)
    (`KismetSystemLibrary.K2_SetTimer` null "SpinBreak" (`KismetMathLibrary.FClamp` (- 1.5 SpinSpeed) 0.01 2.0))))

(event `InputAxis|MoveForward`
  (params (AxisValue :type "Float (single-precision)"))
  (`self.AddMovementInput` (`self.GetActorForwardVector`) (* AxisValue (`self.Speed`))))

(event `InputAxis|MoveRight`
  (params (AxisValue :type "Float (single-precision)"))
  (`self.AddMovementInput` (`self.GetActorRightVector`) (* (`self.Speed`) AxisValue)))

(event `InputAction|FireLeft_Once`
  (params (Key :type "Key Structure"))
  (bind _childactor (`ChildActorComponent.ChildActor` (`self.Mech_Arm1`)))
  (:`Pressed`
    (bind _asbp_arm (cast `/Game/Blueprints/BPMechParts/BPArms/BP_Arm` _childactor))
    (`/Game/Blueprints/BPMechParts/BPArms/BP_Arm.Attack_Once` _asbp_arm))
  (:`Released`
    (bind _asbp_arm_2 (cast `/Game/Blueprints/BPMechParts/BPArms/BP_Arm` _childactor))
    (`/Game/Blueprints/BPMechParts/BPArms/BP_Arm.Attack_Once_Release` _asbp_arm_2)))

(event `InputAction|FireRight_Once`
  (params (Key :type "Key Structure"))
  (bind _childactor (`ChildActorComponent.ChildActor` (`self.Mech_Arm2`)))
  (:`Pressed`
    (bind _asbp_arm (cast `/Game/Blueprints/BPMechParts/BPArms/BP_Arm` _childactor))
    (`/Game/Blueprints/BPMechParts/BPArms/BP_Arm.Attack_Once` _asbp_arm))
  (:`Released`
    (bind _asbp_arm_2 (cast `/Game/Blueprints/BPMechParts/BPArms/BP_Arm` _childactor))
    (`/Game/Blueprints/BPMechParts/BPArms/BP_Arm.Attack_Once_Release` _asbp_arm_2)))

(event `InputAxis|FireLeft_Constant`
  (params (AxisValue :type "Float (single-precision)"))
  (bind _asbp_arm (cast `/Game/Blueprints/BPMechParts/BPArms/BP_Arm` (`ChildActorComponent.ChildActor` (`self.Mech_Arm1`))))
  (`/Game/Blueprints/BPMechParts/BPArms/BP_Arm.Attack_Constant` _asbp_arm AxisValue))

(event `InputAxis|FireRight_Constant`
  (params (AxisValue :type "Float (single-precision)"))
  (bind _asbp_arm (cast `/Game/Blueprints/BPMechParts/BPArms/BP_Arm` (`ChildActorComponent.ChildActor` (`self.Mech_Arm2`))))
  (`/Game/Blueprints/BPMechParts/BPArms/BP_Arm.Attack_Constant` _asbp_arm AxisValue))

(event `InputAction|MovementModifier`
  (params (Key :type "Key Structure"))
  (:`Pressed`
    (bind _asbp_leg (cast `/Game/Blueprints/BPMechParts/BPLegs/BP_Leg` (`ChildActorComponent.ChildActor` (`self.Mech_Legs`))))
    (`/Game/Blueprints/BPMechParts/BPLegs/BP_Leg.LegAbility` _asbp_leg)))

(fn `QueryIsSpinning`
  (returns (timeleft :type "Float (double-precision)"))
  (return (`KismetSystemLibrary.K2_GetTimerRemainingTime` self "SpinBreak")))

(fn `SetArm1`
  (bind _mech_arm1 (`self.Mech_Arm1`))
  (cast `/Game/Blueprints/BPMechParts/BPArms/BP_Arm` (`ChildActorComponent.ChildActor` (`self.Mech_Arm1`)))
  (switch `/Game/Blueprints/Enums/ArmType` (`self.Arm1Type`)
    (:`NewEnumerator0`
      (`ChildActorComponent.SetChildActorClass` _mech_arm1 "/Game/Blueprints/BPMechParts/BPArms/BP_GatlingArm.BP_GatlingArm_C"))
    (:`NewEnumerator1`
      (`ChildActorComponent.SetChildActorClass` _mech_arm1 "/Game/Blueprints/BPMechParts/BPArms/BP_PlasmaArm.BP_PlasmaArm_C"))
    (:`NewEnumerator3`
      (`ChildActorComponent.SetChildActorClass` _mech_arm1 "/Game/Blueprints/BPMechParts/BPArms/BP_RocketArm.BP_RocketArm_C"))
    (:`NewEnumerator4`
      (`ChildActorComponent.SetChildActorClass` _mech_arm1 "/Game/Blueprints/BPMechParts/BPArms/BP_LaserArm.BP_LaserArm_C"))
    (:`NewEnumerator5`
      (`ChildActorComponent.SetChildActorClass` _mech_arm1 "/Game/Blueprints/BPMechParts/BPArms/BP_SwordArm.BP_SwordArm_C"))
    (:`NewEnumerator7`
      (`ChildActorComponent.SetChildActorClass` _mech_arm1 "/Game/Blueprints/BPMechParts/BPArms/BP_CorrosionArm.BP_CorrosionArm_C")))
  (bind _asbp_arm (cast `/Game/Blueprints/BPMechParts/BPArms/BP_Arm` (`ChildActorComponent.ChildActor` _mech_arm1)))
  (`/Game/Blueprints/BPMechParts/BPArms/BP_Arm.Init` _asbp_arm))

(fn `SetArm2`
  (bind _mech_arm2 (`self.Mech_Arm2`))
  (cast `/Game/Blueprints/BPMechParts/BPArms/BP_Arm` (`ChildActorComponent.ChildActor` (`self.Mech_Arm2`)))
  (switch `/Game/Blueprints/Enums/ArmType` (`self.Arm2Type`)
    (:`NewEnumerator0`
      (`ChildActorComponent.SetChildActorClass` _mech_arm2 "/Game/Blueprints/BPMechParts/BPArms/BP_GatlingArm.BP_GatlingArm_C"))
    (:`NewEnumerator1`
      (`ChildActorComponent.SetChildActorClass` _mech_arm2 "/Game/Blueprints/BPMechParts/BPArms/BP_PlasmaArm.BP_PlasmaArm_C"))
    (:`NewEnumerator3`
      (`ChildActorComponent.SetChildActorClass` _mech_arm2 "/Game/Blueprints/BPMechParts/BPArms/BP_RocketArm.BP_RocketArm_C"))
    (:`NewEnumerator4`
      (`ChildActorComponent.SetChildActorClass` _mech_arm2 "/Game/Blueprints/BPMechParts/BPArms/BP_LaserArm.BP_LaserArm_C"))
    (:`NewEnumerator5`
      (`ChildActorComponent.SetChildActorClass` _mech_arm2 "/Game/Blueprints/BPMechParts/BPArms/BP_SwordArm.BP_SwordArm_C"))
    (:`NewEnumerator7`
      (`ChildActorComponent.SetChildActorClass` _mech_arm2 "/Game/Blueprints/BPMechParts/BPArms/BP_CorrosionArm.BP_CorrosionArm_C")))
  (bind _asbp_arm (cast `/Game/Blueprints/BPMechParts/BPArms/BP_Arm` (`ChildActorComponent.ChildActor` _mech_arm2)))
  (set `/Game/Blueprints/BPMechParts/BPArms/BP_Arm.Direction` true _asbp_arm)
  (`/Game/Blueprints/BPMechParts/BPArms/BP_Arm.Init` _asbp_arm))

(fn `SetChassis`
  (bind _mech_chassis (`self.Mech_Chassis`))
  (switch `/Game/Blueprints/Enums/ChassisType` (`self.ChassisType`)
    (:`NewEnumerator0`
      (`SkinnedMeshComponent.SetSkinnedAssetAndUpdate` _mech_chassis null true))
    (:`NewEnumerator1`
      (`SkinnedMeshComponent.SetSkinnedAssetAndUpdate` _mech_chassis "/Game/Meshes/MechParts/Mech_Chassis/Mech_Chassis_Strong.Mech_Chassis_Strong" true))
    (:`NewEnumerator2`
      (`SkinnedMeshComponent.SetSkinnedAssetAndUpdate` _mech_chassis null true))))

(fn `SetIsSpinning`
  (set `self.IsSpinning` false))

(fn `SetLegs`
  (bind _mech_chassis (`self.Mech_Chassis`))
  (bind _mech_legs (`self.Mech_Legs`))
  (switch `/Game/Blueprints/Enums/LegType` (`self.LegType`)
    (:`NewEnumerator0`
      (`ChildActorComponent.SetChildActorClass` _mech_legs "/Game/Blueprints/BPMechParts/BPLegs/BP_BipedLeg.BP_BipedLeg_C")
      (cast `/Game/Blueprints/BPMechParts/BPLegs/BP_Leg` (`ChildActorComponent.ChildActor` _mech_legs))
      (`SceneComponent.K2_SetRelativeLocation` _mech_chassis (0.0 0.0 175.0) false false))
    (:`NewEnumerator1`
      (`ChildActorComponent.SetChildActorClass` _mech_legs "/Game/Blueprints/BPMechParts/BPLegs/BP_QuadLeg.BP_QuadLeg_C")
      (cast `/Game/Blueprints/BPMechParts/BPLegs/BP_Leg` (`ChildActorComponent.ChildActor` _mech_legs))
      (`SceneComponent.K2_SetRelativeLocation` _mech_chassis (0.0 0.0 90.0) false false))
    (:`NewEnumerator2`
      (`ChildActorComponent.SetChildActorClass` _mech_legs "/Game/Blueprints/BPMechParts/BPLegs/BP_TreadLeg.BP_TreadLeg_C")
      (cast `/Game/Blueprints/BPMechParts/BPLegs/BP_Leg` (`ChildActorComponent.ChildActor` _mech_legs))
      (`SceneComponent.K2_SetRelativeLocation` _mech_chassis (0.0 0.0 110.0) false false)))
  (`self.SetSpeedFromLegs`))

(fn `SetMovementSpeed`
  (set `CharacterMovementComponent.MaxWalkSpeed` (* (/ (`self.Speed`) 5.0) 600.0) (`self.CharacterMovement`)))

(fn `SetSpeedFromLegs`
  (bind _returnvalue (* (`self.Speed`) 2.0))
  (bind _asbp_leg (cast `/Game/Blueprints/BPMechParts/BPLegs/BP_Leg` (`ChildActorComponent.ChildActor` (`self.Mech_Legs`))))
  (set `self.Speed` (`/Game/Blueprints/BPMechParts/BPLegs/BP_Leg.Speed` _asbp_leg))
  (switch `/Game/Blueprints/Enums/LegType` (`self.LegType`)
    (:`NewEnumerator0`
      (bind _mechpart (`/Game/Blueprints/BPMechParts/BP_MechPart.MechPart` _asbp_leg))
      (`SkeletalMeshComponent.SetPlayRate` _mechpart (/ _returnvalue 3.2)))
    (:`NewEnumerator1`
      (`SkeletalMeshComponent.SetPlayRate` _mechpart (/ _returnvalue 1.25)))))

(fn `SetTargetRot`
  (bind (_returnvalue_x _returnvalue_y) (`KismetMathLibrary.BreakVector` (`self.K2_GetActorLocation`)))
  (bind _returnvalue (`self.GetInputAxisValue`))
  (bind _returnvalue_2 (`self.GetInputAxisValue`))
  (bind _mech_chassis (`self.Mech_Chassis`))
  (bind _returnvalue_3 (< _returnvalue_2 0.0))
  (bind _returnvalue_4 (< _returnvalue 0.0))
  (bind _returnvalue_5 (== _returnvalue_2 0.0))
  (bind (_returnvalue_roll _returnvalue_pitch) (`KismetMathLibrary.BreakRotator` (`SceneComponent.K2_GetComponentRotation` _mech_chassis)))
  (bind _returnvalue_6 (== _returnvalue 0.0))
  (bind _returnvalue_7 (> _returnvalue_2 0.0))
  (bind _returnvalue_8 (> _returnvalue 0.0))
  (bind (_bblockinghit _binitialoverlap _time _distance _location) (`GameplayStatics.BreakHitResult` (`PlayerController.GetHitResultUnderCursorForObjects` (`GameplayStatics.GetPlayerController` 0) (`|MakeArray` "ObjectTypeQuery7" :!type "EObjectTypeQuery Enum") true)))
  (bind (_returnvalue_roll_2 _returnvalue_pitch_2 _returnvalue_yaw) (`KismetMathLibrary.BreakRotator` (`KismetMathLibrary.FindLookAtRotation` (`KismetMathLibrary.MakeVector` _returnvalue_x _returnvalue_y) (`KismetMathLibrary.MakeVector` (.x _location) (.y _location)))))
  (`|ExecutionSequence`
    (:`then_0`
      (if (and _returnvalue_6 _returnvalue_5)
        (set `self.IsWalking` false)
        (bind _asbp_leg (cast `/Game/Blueprints/BPMechParts/BPLegs/BP_Leg` (`ChildActorComponent.ChildActor` (`self.Mech_Legs`))))
        (`SkeletalMeshComponent.SetPlayRate` (`/Game/Blueprints/BPMechParts/BP_MechPart.MechPart` _asbp_leg) 0.0)
        (elif (and _returnvalue_8 _returnvalue_5)
          (set `self.TargetLegRot` 0.0)
          (if (not (`self.IsWalking`)) :!label _label
            (set `self.IsWalking` true)
            (`self.SetSpeedFromLegs`))
          (elif (and _returnvalue_8 _returnvalue_7)
            (set `self.TargetLegRot` 45.0)
            (goto _label)
            (elif (and _returnvalue_7 _returnvalue_6)
              (set `self.TargetLegRot` 90.0)
              (goto _label)
              (elif (and _returnvalue_7 _returnvalue_4)
                (set `self.TargetLegRot` 135.0)
                (goto _label)
                (elif (and _returnvalue_4 _returnvalue_5)
                  (set `self.TargetLegRot` 180.0)
                  (goto _label)
                  (elif (and _returnvalue_4 _returnvalue_3)
                    (set `self.TargetLegRot` -135.0)
                    (goto _label)
                    (elif (and _returnvalue_3 _returnvalue_6)
                      (set `self.TargetLegRot` -90.0)
                      (goto _label)
                      (elif (and _returnvalue_3 _returnvalue_8)
                        (set `self.TargetLegRot` -45.0)
                        (goto _label)))))))))))
    (:`then_1`
      (`SceneComponent.K2_SetWorldRotation` _mech_chassis (`KismetMathLibrary.MakeRotator` _returnvalue_roll _returnvalue_pitch (- _returnvalue_yaw 90.0)) false false))))

(fn `SetupRobot`
  (`self.SetLegs`)
  (`self.SetChassis`)
  (`self.SetArm1`)
  (`self.SetArm2`)
  (`self.SetMovementSpeed`))

(fn `SetupUI`
  (bind _returnvalue (`|CreateWidget` "/Game/UI/mouseWidget.mouseWidget_C" (`GameplayStatics.GetPlayerController` 0)))
  (`UserWidget.AddToViewport` _returnvalue 0))

(fn `SpinBreak`
  (set `self.V_SpinBreak` false))

(fn `UserConstructionScript`)