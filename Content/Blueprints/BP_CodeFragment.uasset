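; BP_CodeFragment is a collectible cube pickup that adds its Value to the player's FragmentNum.
; On spawn it gets a random launch velocity, stops simulating physics shortly after, and becomes collectable after Delay.
; Entering Radius enables a Tick lerp toward the player; touching Hit or a one-second timeout collects it, playing a random-pitch sound and destroying it.
; The construction script randomizes cube scale, smaller for a Value of 1.
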(event `self.ReceiveBeginPlay`
  (`PrimitiveComponent.SetPhysicsLinearVelocity` (`self.Cube`) (`KismetMathLibrary.MakeVector` (`KismetMathLibrary.RandomFloatInRange` -1000.0 1000.0) (`KismetMathLibrary.RandomFloatInRange` -1000.0 1000.0) (`KismetMathLibrary.RandomFloatInRange` 0.0 500.0)) true "None")
  (`KismetSystemLibrary.K2_SetTimerDelegate` (delegate `DisablePhysics`) (`KismetMathLibrary.RandomFloatInRange` 1.0 1.5))
  (`KismetSystemLibrary.K2_SetTimerDelegate` (delegate `EndDelay`) (`self.Delay`)))

(event `DisablePhysics`
  (`PrimitiveComponent.SetSimulatePhysics` (`self.Cube`) false))

(event `EndDelay`
  (set `self.CanBePickedUp` true))

(event `self.ReceiveTick`
  (params (DeltaSeconds :type "Float (single-precision)"))
  (bind (_returnvalue_x _returnvalue_y _returnvalue_z) (`KismetMathLibrary.BreakVector` (`self.K2_GetActorLocation` (`GameplayStatics.GetPlayerPawn` 0))))
  (`self.K2_SetActorLocation` (`KismetMathLibrary.VLerp` (`self.K2_GetActorLocation`) (`KismetMathLibrary.MakeVector` _returnvalue_x _returnvalue_y (+ _returnvalue_z 90.0)) 0.35)))

(event `self.Radius.OnComponentBeginOverlap`
  (params (OverlappedComponent :type "PrimitiveComponent Object Reference") (OtherActor :type "Actor Object Reference") (OtherComp :type "PrimitiveComponent Object Reference") (OtherBodyIndex :type Integer) (bFromSweep :type Boolean) (SweepResult :type "HitResult Structure (by ref)"))
  (if (`self.CanBePickedUp`)
    (cast `/Game/Blueprints/PlayerCharacter_Final` OtherActor)
    (`/Engine/EditorBlueprintResources/StandardMacros.DoOnce` false
      (:`Completed`
        (`self.SetActorTickEnabled` true)
        (`KismetSystemLibrary.K2_SetTimerDelegate` (delegate `DestroySelf`) 1.0)))))

(event `DestroySelf`
  (bind _asplayer_character_final (cast `/Game/Blueprints/PlayerCharacter_Final` (`GameplayStatics.GetPlayerPawn` 0) :!label _label))
  (set `/Game/Blueprints/PlayerCharacter_Final.FragmentNum` (+ (`/Game/Blueprints/PlayerCharacter_Final.FragmentNum` _asplayer_character_final) (`self.Value`)) _asplayer_character_final)
  (`GameplayStatics.PlaySoundAtLocation` "/Game/Audio/WAV_PointSound.WAV_PointSound" (0.0 0.0 0.0) (struct) (`KismetMathLibrary.RandomFloatInRange` 0.2 0.5) (`KismetMathLibrary.RandomFloatInRange` 1.0 4.0) 0.0 null null null)
  (`self.K2_DestroyActor`))

(event `self.Hit.OnComponentBeginOverlap`
  (params (OverlappedComponent :type "PrimitiveComponent Object Reference") (OtherActor :type "Actor Object Reference") (OtherComp :type "PrimitiveComponent Object Reference") (OtherBodyIndex :type Integer) (bFromSweep :type Boolean) (SweepResult :type "HitResult Structure (by ref)"))
  (if (`self.CanBePickedUp`)
    (cast `/Game/Blueprints/PlayerCharacter_Final` OtherActor)
    (`/Engine/EditorBlueprintResources/StandardMacros.DoOnce` false
      (:`Completed`
        (goto _label)))))

(fn `UserConstructionScript`
  (bind _returnvalue (`KismetMathLibrary.RandomFloatInRange` 0.25 0.4))
  (bind _returnvalue_2 (`KismetMathLibrary.RandomFloatInRange` 0.1 0.25))
  (bind _cube (`self.Cube`))
  (if (== (`self.Value`) 1)
    (`SceneComponent.SetWorldScale3D` _cube (`KismetMathLibrary.MakeVector` _returnvalue_2 _returnvalue_2 _returnvalue_2))
    (else
      (`SceneComponent.SetWorldScale3D` _cube (`KismetMathLibrary.MakeVector` _returnvalue _returnvalue _returnvalue)))))