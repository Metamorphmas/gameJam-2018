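; FadeTop is an actor that fades out its static mesh while the player character is inside its Box trigger, and fades it back on exit.
; On begin play it creates a dynamic instance of M_FadeMaterial.
; Entering swaps that instance onto the mesh and a timeline drives its Opacity.
; Leaving plays a second timeline, then restores M_BuildingMaster; the construction script applies the configurable mesh.
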(event `self.ReceiveBeginPlay`
  (bind _returnvalue (`KismetMaterialLibrary.CreateDynamicMaterialInstance` "/Game/Materials/M_FadeMaterial.M_FadeMaterial"))
  (set `self.FadeMat` _returnvalue))

(event `self.Box.OnComponentBeginOverlap`
  (params (OverlappedComponent :type "PrimitiveComponent Object Reference") (OtherActor :type "Actor Object Reference") (OtherComp :type "PrimitiveComponent Object Reference") (OtherBodyIndex :type Integer) (bFromSweep :type Boolean) (SweepResult :type "HitResult Structure (by ref)"))
  (bind _fademat (`self.FadeMat`))
  (cast `/Game/Blueprints/PlayerCharacter_Final` OtherActor)
  (`PrimitiveComponent.SetMaterial` (`self.StaticMesh`) 0 _fademat)
  (bind (_direction _opacity) (`Timeline|FadeOut` :!via `PlayFromStart`)
    (:`Update`
      (`MaterialInstanceDynamic.SetScalarParameterValue` _fademat "Opacity" _opacity))))

(event `self.Box.OnComponentEndOverlap`
  (params (OverlappedComponent :type "PrimitiveComponent Object Reference") (OtherActor :type "Actor Object Reference") (OtherComp :type "PrimitiveComponent Object Reference") (OtherBodyIndex :type Integer))
  (cast `/Game/Blueprints/PlayerCharacter_Final` OtherActor)
  (bind (_direction _opacity) (`Timeline|FadeIn` :!via `PlayFromStart`)
    (:`Update`
      (`MaterialInstanceDynamic.SetScalarParameterValue` (`self.FadeMat`) "Opacity" _opacity))
    (:`Finished`
      (`PrimitiveComponent.SetMaterial` (`self.StaticMesh`) 0 "/Game/Materials/M_BuildingMaster.M_BuildingMaster"))))

(fn `UserConstructionScript`
  (`StaticMeshComponent.SetStaticMesh` (`self.StaticMesh`) (`self.Mesh`)))