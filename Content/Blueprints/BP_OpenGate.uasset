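; BP_OpenGate is a double gate that starts open and shuts once when the player enters its trigger box.
; An Open timeline drives mirrored yaw on the left and right gates, playing on BeginPlay and reversing from its end to close.
; If Powered, the first overlap by PlayerCharacter_Final latches Closed, plays audio and enables the blocking collision that BeginPlay disabled.
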(event `self.ReceiveBeginPlay`
  (`self.OpenGates`)
  (`PrimitiveComponent.SetCollisionEnabled` (`self.Coll`) "NoCollision"))

(event `OpenGates`
  (bind (_direction _angle) (`Timeline|Open` :!label _label)
    (:`Update`
      (`SceneComponent.K2_SetRelativeRotation` (`self.Gate_Right`) (`KismetMathLibrary.MakeRotator` 0.0 0.0 _angle) false false)
      (`SceneComponent.K2_SetRelativeRotation` (`self.Gate_Left`) (`KismetMathLibrary.MakeRotator` 0.0 0.0 (* _angle -1.0)) false false))))

(event `CloseGates`
  (goto _label :!via `ReverseFromEnd`))

(event `self.Box.OnComponentBeginOverlap`
  (params (OverlappedComponent :type "PrimitiveComponent Object Reference") (OtherActor :type "Actor Object Reference") (OtherComp :type "PrimitiveComponent Object Reference") (OtherBodyIndex :type Integer) (bFromSweep :type Boolean) (SweepResult :type "HitResult Structure (by ref)"))
  (cast `/Game/Blueprints/PlayerCharacter_Final` OtherActor)
  (if (`self.Powered`)
    (if (not (`self.Closed`))
      (set `self.Closed` true)
      (`self.CloseGates`)
      (`AudioComponent.Play` (`self.Audio`) 0.0)
      (`PrimitiveComponent.SetCollisionEnabled` (`self.Coll`) "QueryAndPhysics"))))

(fn `UserConstructionScript`)