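; Destructible mesh actor with configurable mesh, material and health that explodes when its health runs out.
; Damage is reduced by armor, then doubled for the weakness type or halved for the resistance type.
; A widget health bar receives a reference to the actor and is unhidden once on the first non-lethal hit.
; Destruction spawns a fragment spawner, explosion particles and sound, then removes the actor.
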(event `self.ReceiveBeginPlay`
  (`self.Init`))

(event `self.TakeDamage`
  (params (Damage :type "Float (single-precision)") (DamageType :type "/Game/Blueprints/Enums/DamageType Enum" :default "NewEnumerator5"))
  (bind _health (`self.Health`))
  (bind _returnvalue (* Damage (- 1.0 (`self.Armor`))))
  (if (== DamageType (`self.Weakness`))
    (set `self.Health` (- _health (* _returnvalue 2.0)))
    (elif (== DamageType (`self.Resistance`))
      (set `self.Health` (- _health (* _returnvalue 0.5)))
      (else
        (bind _output_get (set `self.Health` (- _health _returnvalue))))))
  (`self.CheckHealth`)
  (set `self.HealthPercent` (/ (`self.Health`) (`self.MaxHealth`))))

(event `self.CheckHealth`
  (if (<= (`self.Health`) 0.0)
    (`self.CallWhenDestroyed`)
    (else
      (`/Engine/EditorBlueprintResources/StandardMacros.DoOnce` false
        (:`Completed`
          (`SceneComponent.SetHiddenInGame` (`self.HealthBar`) false false))))))

(fn `CallWhenDestroyed`
  (bind _expsize (`self.ExpSize`))
  (bind _returnvalue (`SceneComponent.K2_GetComponentLocation` (`self.DefaultSceneRoot`)))
  (`|SpawnActorFromClass` "/Game/Blueprints/BP_FragmentSpawner.BP_FragmentSpawner_C" (`self.GetTransform`) "Undefined" "OverrideRootScale" null (`self.FragmentSpawnNum`) null)
  (`GameplayStatics.SpawnEmitterAtLocation` "/Game/ParticleEffects/P_Explosion.P_Explosion" _returnvalue (struct) (`KismetMathLibrary.MakeVector` _expsize _expsize _expsize))
  (`GameplayStatics.PlaySoundAtLocation` "/Game/Audio/WAV_Explosion1_Reverb.WAV_Explosion1_Reverb" _returnvalue (struct) (`self.Volume`) (`self.Pitch`) 0.0 null null null)
  (`self.K2_DestroyActor`))

(fn `Init`
  (bind _asdestructable_mesh_health_bar (cast `/Game/UI/DestructableMeshHealthBar` (`WidgetComponent.GetUserWidgetObject` (`self.HealthBar`))))
  (set `/Game/UI/DestructableMeshHealthBar.MeshWithHealth` self _asdestructable_mesh_health_bar)
  (set `self.Health` (`self.MaxHealth`))
  (`SceneComponent.K2_SetWorldRotation` (`self.HealthBar`) (struct :`Yaw` 180.0) false false))

(fn `UserConstructionScript`
  (bind _staticmesh (`self.StaticMesh`))
  (bind _healthbar (`self.HealthBar`))
  (bind (_returnvalue_x _returnvalue_y) (`KismetMathLibrary.BreakVector` (`SceneComponent.K2_GetComponentLocation` (`self.StaticMesh`))))
  (`StaticMeshComponent.SetStaticMesh` _staticmesh (`self.Mesh`))
  (`PrimitiveComponent.SetMaterial` _staticmesh 0 (`self.Mat`))
  (set `self.Health` (`self.MaxHealth`))
  (`SceneComponent.K2_SetWorldRotation` _healthbar (struct :`Yaw` 180.0) false false)
  (`SceneComponent.K2_SetWorldLocation` _healthbar (`KismetMathLibrary.MakeVector` _returnvalue_x _returnvalue_y (+ (`self.HealthBarHeight`) 220.0)) false false)
  (`SceneComponent.K2_SetWorldRotation` (`self.HealthBar`) (struct :`Yaw` -180.0) false false))