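; Trader bot that offers mech parts to the player, priced in Code Fragments.
; Overlapping its box shows a tip, plays audio and registers the bot as the player's Trader.
; MakeTrade spawns the offered part as a pickup nearby, then rerolls a weighted random arm or legs while stock remains, otherwise closes trading.
; SetWidget displays the current offer's stats, and audio pitch signals successful or unaffordable trades.
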(event `self.ReceiveBeginPlay`
  (`self.SetWidget`)
  (`SkeletalMeshComponent.SetPlayRate` (`self.Character_BugBot`) 0.75))

(event `MakeTrade`
  (bind _returnvalue (`KismetMathLibrary.RandomIntegerInRange` 0 12))
  (bind (_returnvalue_location _returnvalue_rotation) (`KismetMathLibrary.BreakTransform` (`self.GetTransform`)))
  (bind _audio (`self.Audio`))
  (bind (_returnvalue_x _returnvalue_y _returnvalue_z) (`KismetMathLibrary.BreakVector` (+ (* (`self.GetActorRightVector`) 500.0) _returnvalue_location)))
  (`|SpawnActorFromClass` "/Game/Blueprints/BP_MechPartPickup.BP_MechPartPickup_C" (`KismetMathLibrary.MakeTransform` (`KismetMathLibrary.MakeVector` (+ _returnvalue_x (`KismetMathLibrary.RandomFloatInRange` -500.0 500.0)) (+ _returnvalue_y (`KismetMathLibrary.RandomFloatInRange` -500.0 500.0)) (+ _returnvalue_z 500.0)) _returnvalue_rotation (0.5 0.5 0.5)) "Undefined" "OverrideRootScale" null (`self.PartType`) (`self.ArmType`) (`self.LegType`) (`self.ChassisType`) (`self.Health`) (`self.Armor`) false null)
  (if (and (`self.GenerateItems`) (> (`self.ItemNum`) 0))
    (`/Engine/EditorBlueprintResources/StandardMacros.DecrementInt` (`self.ItemNum`)
      (:`  `
        (`|ExecutionSequence`
          (:`then_0`
            (set `self.Health` (/ (`KismetMathLibrary.Conv_IntToDouble` (`KismetMathLibrary.RandomIntegerInRange` 60 100)) 100.0))
            (if (== (`KismetMathLibrary.RandomIntegerInRange` 0 4) 0)
              (set `self.PartType` "NewEnumerator1")
              (switch `int` (`KismetMathLibrary.RandomIntegerInRange` 0 2)
                (:`0`
                  (set `self.LegType` "NewEnumerator0")
                  (set `self.Armor` 0.0))
                (:`1`
                  (set `self.LegType` "NewEnumerator1")
                  (set `self.Armor` 0.5))
                (:`2`
                  (set `self.LegType` "NewEnumerator2")
                  (set `self.Armor` 0.75)))
              (set `self.Price` 75)
              (else
                (set `self.PartType` "NewEnumerator0")
                (if (< _returnvalue 2)
                  (set `self.ArmType` "NewEnumerator1")
                  (set `self.Price` 50)
                  (elif (< _returnvalue 4)
                    (set `self.ArmType` "NewEnumerator5")
                    (set `self.Price` 75)
                    (elif (< _returnvalue 6)
                      (set `self.ArmType` "NewEnumerator4")
                      (set `self.Price` 75)
                      (elif (< _returnvalue 8)
                        (set `self.ArmType` "NewEnumerator3")
                        (set `self.Price` 65)
                        (elif (< _returnvalue 9)
                          (set `self.ArmType` "NewEnumerator0")
                          (set `self.Price` 100)
                          (elif (< _returnvalue 10)
                            (set `self.ArmType` "NewEnumerator7")
                            (set `self.Price` 200)
                            (elif (< _returnvalue 11)
                              (set `self.ArmType` "NewEnumerator8")
                              (set `self.Price` 250)
                              (else
                                (set `self.ArmType` "NewEnumerator9")
                                (set `self.Price` 300))))))))))))
          (:`then_1`
            (`self.SetWidget`)
            (`AudioComponent.SetPitchMultiplier` _audio 1.5)
            (`AudioComponent.Play` _audio 0.0)))))
    (else
      (`SceneComponent.SetHiddenInGame` (`self.TipPlane`) true true)
      (set `self.CanTrade` false))))

(event `self.Box.OnComponentBeginOverlap`
  (params (OverlappedComponent :type "PrimitiveComponent Object Reference") (OtherActor :type "Actor Object Reference") (OtherComp :type "PrimitiveComponent Object Reference") (OtherBodyIndex :type Integer) (bFromSweep :type Boolean) (SweepResult :type "HitResult Structure (by ref)"))
  (bind _asplayer_character_final (cast `/Game/Blueprints/PlayerCharacter_Final` OtherActor))
  (`SceneComponent.SetHiddenInGame` (`self.TipPlane`) false true)
  (`AudioComponent.Play` (`self.Audio`) 0.0)
  (set `/Game/Blueprints/PlayerCharacter_Final.Trader` self _asplayer_character_final))

(event `self.Box.OnComponentEndOverlap`
  (params (OverlappedComponent :type "PrimitiveComponent Object Reference") (OtherActor :type "Actor Object Reference") (OtherComp :type "PrimitiveComponent Object Reference") (OtherBodyIndex :type Integer))
  (bind _asplayer_character_final (cast `/Game/Blueprints/PlayerCharacter_Final` OtherActor))
  (`SceneComponent.SetHiddenInGame` (`self.TipPlane`) true true)
  (set `/Game/Blueprints/PlayerCharacter_Final.Trader` null _asplayer_character_final))

(event `NotEnoughFragments`
  (bind _audio (`self.Audio`))
  (`AudioComponent.SetPitchMultiplier` _audio 0.5)
  (`AudioComponent.Play` _audio 0.0))

(fn `SetWidget`
  (bind _health (`self.Health`))
  (bind _returnvalue (* (- _health 0.5) 2.0))
  (bind _aspart_trade (cast `/Game/UI/PartTrade` (`WidgetComponent.GetUserWidgetObject` (`self.Widget`))))
  (`TextBlock.SetText` (`/Game/UI/PartTrade.Price` _aspart_trade) (`KismetTextLibrary.Conv_StringToText` (`KismetStringLibrary.Concat_StrStr` (`KismetStringLibrary.Conv_IntToString` (`self.Price`)) " Code Fragments")))
  (bind _integritypercent (`/Game/UI/PartTrade.IntegrityPercent` _aspart_trade))
  (`TextBlock.SetText` _integritypercent (`KismetTextLibrary.Conv_StringToText` (`KismetStringLibrary.Concat_StrStr` (`KismetStringLibrary.Conv_DoubleToString` (* _health 100.0)) "%")))
  (`TextBlock.SetColorAndOpacity` _integritypercent (make `SlateColor` (`KismetMathLibrary.MakeColor` 1.0 _returnvalue _returnvalue)))
  (`TextBlock.SetText` (`/Game/UI/PartTrade.ArmorValue` _aspart_trade) (`KismetTextLibrary.Conv_DoubleToText` (`self.Armor`) "HalfToEven"))
  (switch `/Game/Blueprints/Enums/PartTypes` (`self.PartType`)
    (:`NewEnumerator0`
      (`TextBlock.SetText` (`/Game/UI/PartTrade.Speed` _aspart_trade) "Type:")
      (switch `/Game/Blueprints/Enums/ArmType` (`self.ArmType`)
        (:`NewEnumerator0`
          (bind _partname (`/Game/UI/PartTrade.PartName` _aspart_trade))
          (`TextBlock.SetText` _partname "Gatling Gun")
          (bind _speedval (`/Game/UI/PartTrade.SpeedVal` _aspart_trade))
          (`TextBlock.SetText` _speedval "Kinetic")
          (`TextBlock.SetColorAndOpacity` _speedval (make `SlateColor` (struct :`R` 1.0 :`G` 0.703717 :`B` 0.328125 :`A` 1.0))))
        (:`NewEnumerator1`
          (`TextBlock.SetText` _partname "Plasma Cannon")
          (`TextBlock.SetText` _speedval "Plasma")
          (`TextBlock.SetColorAndOpacity` _speedval (make `SlateColor` (struct :`R` 0.303628 :`B` 1.0 :`A` 1.0))))
        (:`NewEnumerator3`
          (`TextBlock.SetText` _partname "Rocket Launcher")
          (`TextBlock.SetText` _speedval "Explosive")
          (`TextBlock.SetColorAndOpacity` _speedval (make `SlateColor` (struct :`R` 1.0 :`G` 0.121763 :`A` 1.0))))
        (:`NewEnumerator4`
          (`TextBlock.SetText` _partname "Beam Laser")
          (`TextBlock.SetText` _speedval "Laser")
          (`TextBlock.SetColorAndOpacity` _speedval (make `SlateColor` (struct :`G` 0.742144 :`B` 1.0 :`A` 1.0))))
        (:`NewEnumerator5`
          (`TextBlock.SetText` _partname "Hydraulic Sword")
          (`TextBlock.SetText` _speedval "Kinetic")
          (`TextBlock.SetColorAndOpacity` _speedval (make `SlateColor` (struct :`R` 1.0 :`G` 0.703717 :`B` 0.328125 :`A` 1.0))))
        (:`NewEnumerator7`
          (`TextBlock.SetText` _partname "Corrosion Cannon")
          (`TextBlock.SetText` _speedval "Plasma")
          (`TextBlock.SetColorAndOpacity` _speedval (make `SlateColor` (struct :`R` 0.303628 :`B` 1.0 :`A` 1.0))))
        (:`NewEnumerator8`
          (`TextBlock.SetText` _partname "Grenade Launcher")
          (`TextBlock.SetText` _speedval "Explosive")
          (`TextBlock.SetColorAndOpacity` _speedval (make `SlateColor` (struct :`R` 1.0 :`G` 0.121763 :`A` 1.0))))
        (:`NewEnumerator9`
          (`TextBlock.SetText` _partname "Laser Javelin")
          (`TextBlock.SetText` _speedval "Laser")
          (`TextBlock.SetColorAndOpacity` _speedval (make `SlateColor` (struct :`G` 0.742144 :`B` 1.0 :`A` 1.0))))
        (:`NewEnumerator10`
          (`TextBlock.SetText` _partname "Broken Appendage")
          (`TextBlock.SetText` _speedval "None")
          (`TextBlock.SetColorAndOpacity` _speedval (make `SlateColor` (struct :`R` 1.0 :`G` 1.0 :`B` 1.0 :`A` 1.0))))))
    (:`NewEnumerator1`
      (switch `/Game/Blueprints/Enums/LegType` (`self.LegType`)
        (:`NewEnumerator0`
          (bind _partname_2 (`/Game/UI/PartTrade.PartName` _aspart_trade))
          (`TextBlock.SetText` _partname_2 "Bipedal Legs")
          (bind _speedval_2 (`/Game/UI/PartTrade.SpeedVal` _aspart_trade))
          (`TextBlock.SetText` _speedval_2 "9"))
        (:`NewEnumerator1`
          (`TextBlock.SetText` _partname_2 "Quadrupedal Legs")
          (`TextBlock.SetText` _speedval_2 "3"))
        (:`NewEnumerator2`
          (`TextBlock.SetText` _partname_2 "AT Treads")
          (`TextBlock.SetText` _speedval_2 "13")))
      (`TextBlock.SetText` (`/Game/UI/PartTrade.Speed` _aspart_trade) "Speed:"))))

(fn `UserConstructionScript`
  (`SceneComponent.K2_SetWorldRotation` (`self.TipPlane`) (struct :`Roll` 90.0) false false))