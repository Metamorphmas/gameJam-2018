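; BP_Leg is a mech leg part, with an empty LegAbility function and health-based breakage that slows the player.
; When CheckHealth finds Health at zero, a DoOnce marks the leg broken, updates player 0's armor, calls MakeBroken and cuts Speed to 70%.
; It then has the parent actor, cast to PlayerCharacter_Final, recalculate its leg-derived and movement speed.
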(event `self.CheckHealth`
  (if (== (`self.Health`) 0.0)
    (`/Engine/EditorBlueprintResources/StandardMacros.DoOnce` false
      (:`Completed`
        (set `self.Broken` true)
        (bind _asplayer_character_final (cast `/Game/Blueprints/PlayerCharacter_Final` (`GameplayStatics.GetPlayerCharacter` 0)))
        (`/Game/Blueprints/PlayerCharacter_Final.SetArmorVal` _asplayer_character_final)
        (`self.MakeBroken`)
        (set `self.Speed` (* (`self.Speed`) 0.7))
        (bind _asplayer_character_final_2 (cast `/Game/Blueprints/PlayerCharacter_Final` (`self.GetParentActor`)))
        (`/Game/Blueprints/PlayerCharacter_Final.SetSpeedFromLegs` _asplayer_character_final_2)
        (`/Game/Blueprints/PlayerCharacter_Final.SetMovementSpeed` _asplayer_character_final_2)))))

(fn `LegAbility`)

(fn `UserConstructionScript`)