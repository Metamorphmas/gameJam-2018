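; BP_RocketArm is a mech arm weapon that charges rockets while attack is held and fires them as a volley on release.
; AttackOnce starts a looping timer on LoadRocket, which adds one rocket per second up to four.
; AttackOnceRelease stops loading and calls QueRockets, which re-arms a short timer until the load is empty.
; FireRocket spawns BP_Rocket at four muzzle points in rotation, with a yaw offset.
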(event `self.Attack_Constant`
  (params (ButtonVal :type "Float (single-precision)")))

(event `self.Attack_Once`
  (`KismetSystemLibrary.K2_SetTimer` self "LoadRocket" 1.0 true))

(event `self.Attack_Once_Release`
  (`KismetSystemLibrary.PrintString` "Firing")
  (`KismetSystemLibrary.K2_ClearTimer` self "LoadRocket")
  (`self.QueRockets`))

(event `FireRocket`
  (bind _returnvalue (`SceneComponent.K2_GetComponentToWorld` (`self.FireLoc4`)))
  (bind _returnvalue_2 (`SceneComponent.K2_GetComponentToWorld` (`self.FireLoc1`)))
  (bind _returnvalue_3 (`SceneComponent.K2_GetComponentToWorld` (`self.FireLoc2`)))
  (bind _returnvalue_4 (`SceneComponent.K2_GetComponentToWorld` (`self.FireLoc3`)))
  (switch `int` (`self.CurrentRocket`)
    (:`Default`
      (`|SpawnActorFromClass` "/Game/Blueprints/BP_Rocket.BP_Rocket_C" (`KismetMathLibrary.MakeTransform` (.location _returnvalue_2) (`KismetMathLibrary.MakeRotator` (.roll (.rotation _returnvalue_2)) (.pitch (.rotation _returnvalue_2)) (+ (.yaw (.rotation _returnvalue_2)) 90.0)) (0.8 0.8 0.8)) "Undefined" "OverrideRootScale" null null 20.0 false null :!label _label)
      (`/Engine/EditorBlueprintResources/StandardMacros.IncrementInt` (`self.CurrentRocket`)))
    (:`0`
      (goto _label))
    (:`1`
      (`|SpawnActorFromClass` "/Game/Blueprints/BP_Rocket.BP_Rocket_C" (`KismetMathLibrary.MakeTransform` (.location _returnvalue_3) (`KismetMathLibrary.MakeRotator` (.roll (.rotation _returnvalue_3)) (.pitch (.rotation _returnvalue_3)) (+ (.yaw (.rotation _returnvalue_3)) 90.0)) (0.8 0.8 0.8)) "Undefined" "OverrideRootScale" null null 20.0 false null)
      (`/Engine/EditorBlueprintResources/StandardMacros.IncrementInt` (`self.CurrentRocket`)))
    (:`2`
      (`|SpawnActorFromClass` "/Game/Blueprints/BP_Rocket.BP_Rocket_C" (`KismetMathLibrary.MakeTransform` (.location _returnvalue_4) (`KismetMathLibrary.MakeRotator` (.roll (.rotation _returnvalue_4)) (.pitch (.rotation _returnvalue_4)) (+ (.yaw (.rotation _returnvalue_4)) 90.0)) (0.8 0.8 0.8)) "Undefined" "OverrideRootScale" null null 20.0 false null)
      (`/Engine/EditorBlueprintResources/StandardMacros.IncrementInt` (`self.CurrentRocket`)))
    (:`3`
      (`|SpawnActorFromClass` "/Game/Blueprints/BP_Rocket.BP_Rocket_C" (`KismetMathLibrary.MakeTransform` (.location _returnvalue) (`KismetMathLibrary.MakeRotator` (.roll (.rotation _returnvalue)) (.pitch (.rotation _returnvalue)) (+ (.yaw (.rotation _returnvalue)) 90.0)) (0.8 0.8 0.8)) "Undefined" "OverrideRootScale" null null 20.0 false null)
      (set `self.CurrentRocket` 0))))

(fn `LoadRocket`
  (bind _output_get (set `self.NumLoaded` (`KismetMathLibrary.Clamp` (+ (`self.NumLoaded`) 1) 0 4)))
  (`KismetSystemLibrary.PrintString` (`KismetStringLibrary.Conv_IntToString` _output_get)))

(fn `QueRockets`
  (bind _numloaded (`self.NumLoaded`))
  (if (> _numloaded 0)
    (`self.FireRocket`)
    (bind _output_get (set `self.NumLoaded` (`KismetMathLibrary.Clamp` (- _numloaded 1) 0 4)))
    (if (> _output_get 0)
      (`KismetSystemLibrary.K2_SetTimer` self "QueRockets" 0.2))))

(fn `UserConstructionScript`)