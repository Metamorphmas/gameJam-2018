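; BP_Arm is a mech arm part that swivels to aim at the mouse cursor, with empty attack functions, likely for child arms to override.
; Init starts a fast looping timer for RotateToCursor and negates AngleAdj when Direction is false.
; RotateToCursor traces under the cursor and changes only the root's yaw, applying a quarter-turn offset plus an AngleAdj correction that varies linearly with target distance.
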(event `self.ReceiveBeginPlay`)

(fn `Attack_Constant`
  (params (ButtonVal :type "Float (double-precision)")))

(fn `Attack_Once`)

(fn `Attack_Once_Release`)

(fn `Init`
  (`KismetSystemLibrary.K2_SetTimer` self "RotateToCursor" 0.02 true)
  (if (not (`self.Direction`))
    (set `self.AngleAdj` (* (`self.AngleAdj`) -1.0))))

(fn `RotateToCursor`
  (bind _returnvalue (`self.K2_GetActorLocation`))
  (bind _defaultsceneroot (`self.DefaultSceneRoot`))
  (bind (_returnvalue_roll _returnvalue_pitch) (`KismetMathLibrary.BreakRotator` (`SceneComponent.K2_GetComponentRotation` _defaultsceneroot)))
  (bind (_bblockinghit _binitialoverlap _time _distance _location) (`GameplayStatics.BreakHitResult` (`PlayerController.GetHitResultUnderCursorForObjects` (`GameplayStatics.GetPlayerController` 0) (`|MakeArray` "ObjectTypeQuery7" :!type "EObjectTypeQuery Enum") true)))
  (bind (_returnvalue_roll_2 _returnvalue_pitch_2 _returnvalue_yaw) (`KismetMathLibrary.BreakRotator` (`KismetMathLibrary.FindLookAtRotation` _returnvalue (`KismetMathLibrary.MakeVector` (.x _location) (.y _location) (+ (.z _location) 100.0)))))
  (`SceneComponent.K2_SetWorldRotation` _defaultsceneroot (`KismetMathLibrary.MakeRotator` _returnvalue_roll _returnvalue_pitch (- _returnvalue_yaw (+ 90.0 (* (`self.AngleAdj`) (- 1.5 (/ (`KismetMathLibrary.VSize` (- _returnvalue _location)) 1500.0)))))) false false))

(fn `UserConstructionScript`)