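; Mech arm weapon that charges while attack is held and fires a laser javelin.
; A looping timer raises the charge, scaling an attached effect and driving a dynamic material.
; It fires automatically at full charge or on release when nearly full; earlier release fades glow and sound without firing.
; Timelines animate the glow afterward, and breaking the arm activates sparks and updates the player's armor value.
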(event `self.ReceiveBeginPlay`
  (bind _returnvalue (`KismetMaterialLibrary.CreateDynamicMaterialInstance` "/Game/Materials/MI_JavelinArm.MI_JavelinArm"))
  (bind _output_get (set `self.Mat` _returnvalue))
  (`PrimitiveComponent.SetMaterial` (`self.MechPart`) 0 _output_get))

(event `self.Attack_Once`
  (bind _returnvalue (`|SpawnActorFromClass` "/Game/Blueprints/Projectiles/BP_JavelinEffect.BP_JavelinEffect_C" (`KismetMathLibrary.MakeTransform` (`SceneComponent.K2_GetComponentLocation` (`self.FireLocation`))) "Undefined" "OverrideRootScale" null null))
  (`self.K2_AttachToComponent` _returnvalue (`self.FireLocation`) "None" "KeepWorld" "KeepWorld" "KeepWorld" true)
  (bind _returnvalue_2 (`KismetSystemLibrary.K2_SetTimerDelegate` (delegate `IncreaseDamage`) 0.02 true))
  (`AudioComponent.FadeIn` (`self.WAV_JavelinCharge`) 1.0 1.0 0.0))

(event `IncreaseDamage`
  (bind _firelocation (`self.FireLocation`))
  (bind (_returnvalue_roll _returnvalue_pitch _returnvalue_yaw) (`KismetMathLibrary.BreakRotator` (`SceneComponent.K2_GetComponentRotation` _firelocation)))
  (bind _output_get (set `self.Damage` (`KismetMathLibrary.FClamp` (+ (`self.Damage`) 0.004))))
  (bind _returnvalue (* _output_get 1.5))
  (`self.SetActorScale3D` (stale `self.Attack_Once` _returnvalue) (`KismetMathLibrary.MakeVector` _returnvalue _returnvalue _returnvalue))
  (`MaterialInstanceDynamic.SetScalarParameterValue` (`self.Mat`) "ChargeAmount" (+ (* _output_get 0.32) 0.35))
  (if (== _output_get 1.0)
    (if (> (`self.Damage`) 0.9) :!label _label
      (`|SpawnActorFromClass` "/Game/Blueprints/Projectiles/BP_LaserJavelin.BP_LaserJavelin_C" (`KismetMathLibrary.MakeTransform` (`SceneComponent.K2_GetComponentLocation` _firelocation) (`KismetMathLibrary.MakeRotator` _returnvalue_roll _returnvalue_pitch (+ _returnvalue_yaw 90.0)) (0.6 0.6 0.6)) "Undefined" "OverrideRootScale" null null 15.0 false 3.5 self null)
      (`self.FireGlow`)
      (`AudioComponent.Play` (`self.WAV_JavelinFire`) 0.0)
      (else
        (`self.FadeGlow`)
        (`AudioComponent.FadeOut` (`self.WAV_JavelinCharge`) 0.15 0.0)))
    (bind _particlesystem (`/Game/Blueprints/Projectiles/BP_JavelinEffect.ParticleSystem` (stale `self.Attack_Once` _returnvalue)))
    (if (`KismetSystemLibrary.IsValid` _particlesystem)
      (`ActorComponent.SetActive` _particlesystem false false))
    (`KismetSystemLibrary.K2_ClearAndInvalidateTimerHandle` (stale `self.Attack_Once` _returnvalue_2))
    (set `self.Damage` 0.0)))

(event `self.Attack_Once_Release`
  (goto _label))

(event `FadeGlow`
  (bind _mat (`self.Mat`))
  (bind (_direction _glowamt) (`Timeline|FadeOut` :!via `PlayFromStart`)
    (:`Update`
      (`MaterialInstanceDynamic.SetScalarParameterValue` _mat "Glow" _glowamt))
    (:`Finished`
      (`MaterialInstanceDynamic.SetScalarParameterValue` _mat "ChargeAmount" 0.0)
      (`MaterialInstanceDynamic.SetScalarParameterValue` _mat "Glow" 1.0))))

(event `FireGlow`
  (bind _mat (`self.Mat`))
  (bind (_direction _glowamt) (`Timeline|Drain` :!via `PlayFromStart`)
    (:`Update`
      (`MaterialInstanceDynamic.SetScalarParameterValue` _mat "Glow" _glowamt)
      (`MaterialInstanceDynamic.SetScalarParameterValue` _mat "ChargeAmount" (+ (* _glowamt 0.5) 0.3)))
    (:`Finished`
      (`MaterialInstanceDynamic.SetScalarParameterValue` _mat "ChargeAmount" 0.0)
      (`MaterialInstanceDynamic.SetScalarParameterValue` _mat "Glow" 1.0))))

(event `self.MakeBroken`
  (`ActorComponent.SetActive` (`self.P_Sparks`) true false)
  (bind _asplayer_character_final (cast `/Game/Blueprints/PlayerCharacter_Final` (`GameplayStatics.GetPlayerPawn` 0)))
  (`/Game/Blueprints/PlayerCharacter_Final.SetArmorVal` _asplayer_character_final))

(fn `UserConstructionScript`)