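; BP_BrokenArm is a mech arm part that starts out broken, setting its Health to zero on BeginPlay and running CheckHealth.
; Its overlap, Tick and AttackOnce events are left empty.
; UpdateSwordType casts the parent actor to PlayerCharacter_Final and uses its LegType to choose between the biped and alternate sword-arm skeletal mesh and matching animation.
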(event `self.ReceiveBeginPlay`
  (set `self.Health` 0.0)
  (`self.CheckHealth`))

(event `self.Attack_Once`)

(fn `UpdateSwordType`
  (bind _mechpart (`self.MechPart`))
  (bind _asplayer_character_final (cast `/Game/Blueprints/PlayerCharacter_Final` (`self.GetParentActor`)))
  (if (`|EnumEquality` (`/Game/Blueprints/PlayerCharacter_Final.LegType` _asplayer_character_final) "NewEnumerator0")
    (`SkinnedMeshComponent.SetSkinnedAssetAndUpdate` _mechpart "/Game/Meshes/MechParts/Mesh_Arms/Mech_SwordArm_Biped.Mech_SwordArm_Biped" true)
    (set `self.Anim` "/Game/Animations/Arms/Mech_SwordArm_Biped_Anim.Mech_SwordArm_Biped_Anim")
    (else
      (`SkinnedMeshComponent.SetSkinnedAssetAndUpdate` _mechpart "/Game/Meshes/MechParts/Mesh_Arms/Mech_SwordArm2.Mech_SwordArm2" true)
      (set `self.Anim` "/Game/Animations/Arms/Mech_SwordArm2_Anim.Mech_SwordArm2_Anim"))))

(fn `UserConstructionScript`)