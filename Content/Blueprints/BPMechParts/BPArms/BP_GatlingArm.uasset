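; Gatling gun arm for a mech that spins up while attack input is held and winds down on release, with Rot driving the part's play rate.
; Near full spin, a looping timer calls Fire, which line-traces for the impact effect, flickers the light and damages CanTakeDamage actors.
; DoOnce gates toggle audio and effects once per state change.
; MakeBroken stops firing, shows fire and calls SetArmorVal on the player.
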(event `self.ReceiveTick`
  (params (DeltaSeconds :type "Float (single-precision)"))
  (`SkeletalMeshComponent.SetPlayRate` (`self.MechPart`) (`self.Rot`)))

(event `self.Attack_Constant`
  (params (ButtonVal :type "Float (single-precision)"))
  (bind _pointlight (`self.PointLight`))
  (bind _audio (`self.Audio`))
  (if (> ButtonVal 0.0)
    (`|ExecutionSequence`
      (:`then_0`
        (goto _label_3 :!via `Reset`))
      (:`then_1`
        (bind _output_get (set `self.Rot` (`KismetMathLibrary.FClamp` (+ (`self.Rot`) (`self.SpinUpSpeed`)) 0.0 10.0)))
        (if (> _output_get 9.0)
          (`/Engine/EditorBlueprintResources/StandardMacros.DoOnce` false :!label _label
            (:`Completed`
              (`ActorComponent.SetActive` (`self.P_MuzzleFlash`) true false)
              (`ActorComponent.SetActive` (`self.P_Impact`) true false)
              (`SceneComponent.SetHiddenInGame` (`self.PointLight`) false false)
              (`KismetSystemLibrary.K2_SetTimer` self "Fire" 0.08 true)
              (`AudioComponent.Play` _audio 0.0)))))
      (:`then_2`
        (`/Engine/EditorBlueprintResources/StandardMacros.DoOnce` false :!label _label_2
          (:`Completed`
            (`AudioComponent.Play` (`self.Audio1`) 0.0)))))
    (else
      (set `self.Rot` (`KismetMathLibrary.FClamp` (+ (`self.Rot`) -0.12) 0.0 10.0))
      (`/Engine/EditorBlueprintResources/StandardMacros.DoOnce` false :!label _label_3
        (:`Completed`
          (`ActorComponent.SetActive` (`self.P_MuzzleFlash`) false false)
          (`ActorComponent.SetActive` (`self.P_Impact`) false false)
          (`KismetSystemLibrary.K2_ClearTimer` self "Fire")
          (`LightComponent.SetIntensity` _pointlight 0.0)
          (`SceneComponent.SetHiddenInGame` _pointlight true false)
          (`AudioComponent.Play` (`self.Audio2`) 0.0)
          (`AudioComponent.FadeOut` _audio 0.2 0.0)
          (`|ExecutionSequence`
            (:`then_0`
              (goto _label :!via `Reset`))
            (:`then_1`
              (goto _label_2 :!via `Reset`))))))))

(event `self.MakeBroken`
  (`ActorComponent.SetActive` (`self.P_FireBroken`) true false)
  (`ActorComponent.SetActive` (`self.P_MuzzleFlash`) false false)
  (`ActorComponent.SetActive` (`self.P_Impact`) false false)
  (`KismetSystemLibrary.K2_ClearTimer` self "Fire")
  (`SceneComponent.SetHiddenInGame` (`self.PointLight`) true false)
  (set `self.Rot` 0.0)
  (bind _asplayer_character_final (cast `/Game/Blueprints/PlayerCharacter_Final` (`GameplayStatics.GetPlayerPawn` 0)))
  (`/Game/Blueprints/PlayerCharacter_Final.SetArmorVal` _asplayer_character_final))

(fn `Fire`
  (bind _firelocation (`self.FireLocation`))
  (bind _returnvalue (`SceneComponent.K2_GetComponentLocation` _firelocation))
  (`LightComponent.SetIntensity` (`self.PointLight`) (`KismetMathLibrary.RandomFloatInRange` 1000.0 3000.0))
  (bind _outhit (`KismetSystemLibrary.LineTraceSingle` _returnvalue (+ _returnvalue (* (`SceneComponent.GetRightVector` _firelocation) (`self.Range`))) "TraceTypeQuery1"))
  (bind (_bblockinghit _binitialoverlap _time _distance _location _impactpoint _normal _impactnormal _physmat _hitactor) (`GameplayStatics.BreakHitResult` _outhit))
  (`SceneComponent.K2_SetWorldLocation` (`self.P_Impact`) _location false false)
  (if (`KismetSystemLibrary.DoesImplementInterface` _hitactor "/Game/Blueprints/CanTakeDamage.CanTakeDamage_C")
    (message `/Game/Blueprints/CanTakeDamage.TakeDamage` _hitactor (`self.Damage`) "NewEnumerator0")))

(fn `UserConstructionScript`)