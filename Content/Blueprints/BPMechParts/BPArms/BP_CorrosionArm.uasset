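; BP_CorrosionArm is a mech arm weapon that charges while attacking and fires a corrosive orb on release.
; AttackOnce spawns a corrosion effect at FireLocation and starts a looping timer that raises clamped Damage, scales the effect with it and prints it.
; AttackOnceRelease spawns the orb with Damage-based damage and duration and reattaches the effect to it, or destroys the effect below the minimum charge, then resets.
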(event `self.Attack_Once`
  (bind _returnvalue (`|SpawnActorFromClass` "/Game/Blueprints/Projectiles/BP_CorrosionEffect.BP_CorrosionEffect_C" (`KismetMathLibrary.MakeTransform` (`SceneComponent.K2_GetComponentLocation` (`self.FireLocation`))) "Undefined" "OverrideRootScale" null null))
  (`self.K2_AttachToComponent` _returnvalue (`self.FireLocation`) "None" "KeepWorld" "KeepWorld" "KeepWorld" true)
  (bind _returnvalue_2 (`KismetSystemLibrary.K2_SetTimerDelegate` (delegate `IncreaseDamage`) 0.02 true)))

(event `IncreaseDamage`
  (bind _output_get (set `self.Damage` (`KismetMathLibrary.FClamp` (+ (`self.Damage`) 0.002) 0.02 0.2)))
  (bind _returnvalue (* _output_get 5.0))
  (`self.SetActorScale3D` (stale `self.Attack_Once` _returnvalue) (`KismetMathLibrary.MakeVector` _returnvalue _returnvalue _returnvalue))
  (`KismetSystemLibrary.PrintString` (`KismetStringLibrary.Conv_DoubleToString` _output_get)))

(event `self.Attack_Once_Release`
  (bind _damage (`self.Damage`))
  (bind _firelocation (`self.FireLocation`))
  (bind (_returnvalue_roll _returnvalue_pitch _returnvalue_yaw) (`KismetMathLibrary.BreakRotator` (`SceneComponent.K2_GetComponentRotation` _firelocation)))
  (if (>= (`self.Damage`) 0.02)
    (bind _returnvalue (`|SpawnActorFromClass` "/Game/Blueprints/Projectiles/BP_CorrosiveOrb.BP_CorrosiveOrb_C" (`KismetMathLibrary.MakeTransform` (`SceneComponent.K2_GetComponentLocation` _firelocation) (`KismetMathLibrary.MakeRotator` _returnvalue_roll _returnvalue_pitch (+ _returnvalue_yaw 90.0)) (0.6 0.6 0.6)) "Undefined" "OverrideRootScale" null null 15.0 false _damage (* _damage 25.0) null))
    (`self.K2_AttachToComponent` (stale `self.Attack_Once` _returnvalue) (`/Game/Blueprints/Projectiles/BP_CorrosiveOrb.Sphere` _returnvalue) "None" "KeepWorld" "KeepWorld" "KeepWorld" true)
    (else
      (`self.K2_DestroyActor` (stale `self.Attack_Once` _returnvalue))))
  (`KismetSystemLibrary.K2_ClearAndInvalidateTimerHandle` (stale `self.Attack_Once` _returnvalue_2))
  (set `self.Damage` 0.02))

(fn `UserConstructionScript`)