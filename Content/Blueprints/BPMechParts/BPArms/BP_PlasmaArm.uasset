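; Plasma arm mech part that fires plasma orbs and shows a broken state.
; It runs a health check on begin play.
; Each single attack spawns a scaled-down BP_PlasmaOrb at the fire location, passing the arm's damage and turning the yaw a quarter turn from that component's rotation.
; When broken, it activates a plasma-broken effect and has the player character set its armor value.
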(event `self.ReceiveBeginPlay`
  (`self.CheckHealth`))

(event `self.Attack_Once`
  (bind _firelocation (`self.FireLocation`))
  (bind (_returnvalue_roll _returnvalue_pitch _returnvalue_yaw) (`KismetMathLibrary.BreakRotator` (`SceneComponent.K2_GetComponentRotation` _firelocation)))
  (`|SpawnActorFromClass` "/Game/Blueprints/Projectiles/BP_PlasmaOrb.BP_PlasmaOrb_C" (`KismetMathLibrary.MakeTransform` (`SceneComponent.K2_GetComponentLocation` _firelocation) (`KismetMathLibrary.MakeRotator` _returnvalue_roll _returnvalue_pitch (+ _returnvalue_yaw 90.0)) (0.6 0.6 0.6)) "Undefined" "OverrideRootScale" null null 15.0 false (`self.Damage`) null))

(event `/Game/Blueprints/BPMechParts/BP_MechPart.MakeBroken`
  (`ActorComponent.SetActive` (`self.P_PlasmaBroken`) true false)
  (bind _asplayer_character_final (cast `/Game/Blueprints/PlayerCharacter_Final` (`GameplayStatics.GetPlayerPawn` 0)))
  (`/Game/Blueprints/PlayerCharacter_Final.SetArmorVal` _asplayer_character_final))

(fn `UserConstructionScript`)