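; Mech rocket arm weapon that charges up to four rockets while the attack is held and fires them in a burst on release.
; A looping timer runs LoadRocket each second, raising the count and the dynamic material's ChargeAmount.
; On release, QueRockets re-arms a short timer to call FireRocket until empty, draining the charge per shot.
; FireRocket spawns BP_Rocket with the arm's Damage, cycling through four muzzle points across bursts.
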(event `self.ReceiveBeginPlay`
  (bind _returnvalue (`KismetMaterialLibrary.CreateDynamicMaterialInstance` "/Game/Materials/MI_RocketArm.MI_RocketArm"))
  (bind _output_get (set `self.Mat` _returnvalue))
  (`PrimitiveComponent.SetMaterial` (`self.MechPart`) 0 _output_get)
  (`MaterialInstanceDynamic.SetScalarParameterValue` _output_get "ChargeAmount" 0.0))

(event `self.Attack_Constant`
  (params (ButtonVal :type "Float (single-precision)")))

(event `self.Attack_Once`
  (`KismetSystemLibrary.K2_SetTimer` self "LoadRocket" 1.0 true))

(event `self.Attack_Once_Release`
  (`KismetSystemLibrary.PrintString` "Firing")
  (`KismetSystemLibrary.K2_ClearTimer` self "LoadRocket")
  (`self.QueRockets`))

(event `FireRocket`
  (bind _damage (`self.Damage`))
  (bind _returnvalue (`SceneComponent.K2_GetComponentToWorld` (`self.FireLoc4`)))
  (bind _returnvalue_2 (`SceneComponent.K2_GetComponentToWorld` (`self.FireLoc1`)))
  (bind _returnvalue_3 (`SceneComponent.K2_GetComponentToWorld` (`self.FireLoc2`)))
  (bind _returnvalue_4 (`SceneComponent.K2_GetComponentToWorld` (`self.FireLoc3`)))
  (switch `int` (`self.CurrentRocket`)
    (:`Default`
      (`|SpawnActorFromClass` "/Game/Blueprints/Projectiles/BP_Rocket.BP_Rocket_C" (`KismetMathLibrary.MakeTransform` (.location _returnvalue_2) (`KismetMathLibrary.MakeRotator` (.roll (.rotation _returnvalue_2)) (.pitch (.rotation _returnvalue_2)) (+ (.yaw (.rotation _returnvalue_2)) 90.0)) (0.8 0.8 0.8)) "Undefined" "OverrideRootScale" null null 15.0 false _damage null :!label _label)
      (`/Engine/EditorBlueprintResources/StandardMacros.IncrementInt` (`self.CurrentRocket`)))
    (:`0`
      (goto _label))
    (:`1`
      (`|SpawnActorFromClass` "/Game/Blueprints/Projectiles/BP_Rocket.BP_Rocket_C" (`KismetMathLibrary.MakeTransform` (.location _returnvalue_3) (`KismetMathLibrary.MakeRotator` (.roll (.rotation _returnvalue_3)) (.pitch (.rotation _returnvalue_3)) (+ (.yaw (.rotation _returnvalue_3)) 90.0)) (0.8 0.8 0.8)) "Undefined" "OverrideRootScale" null null 15.0 false _damage null)
      (`/Engine/EditorBlueprintResources/StandardMacros.IncrementInt` (`self.CurrentRocket`)))
    (:`2`
      (`|SpawnActorFromClass` "/Game/Blueprints/Projectiles/BP_Rocket.BP_Rocket_C" (`KismetMathLibrary.MakeTransform` (.location _returnvalue_4) (`KismetMathLibrary.MakeRotator` (.roll (.rotation _returnvalue_4)) (.pitch (.rotation _returnvalue_4)) (+ (.yaw (.rotation _returnvalue_4)) 90.0)) (0.8 0.8 0.8)) "Undefined" "OverrideRootScale" null null 15.0 false _damage null)
      (`/Engine/EditorBlueprintResources/StandardMacros.IncrementInt` (`self.CurrentRocket`)))
    (:`3`
      (`|SpawnActorFromClass` "/Game/Blueprints/Projectiles/BP_Rocket.BP_Rocket_C" (`KismetMathLibrary.MakeTransform` (.location _returnvalue) (`KismetMathLibrary.MakeRotator` (.roll (.rotation _returnvalue)) (.pitch (.rotation _returnvalue)) (+ (.yaw (.rotation _returnvalue)) 90.0)) (0.8 0.8 0.8)) "Undefined" "OverrideRootScale" null null 15.0 false _damage null)
      (set `self.CurrentRocket` 0))))

(fn `LoadRocket`
  (bind _mat (`self.Mat`))
  (bind _returnvalue (`MaterialInstanceDynamic.K2_GetScalarParameterValue` _mat "ChargeAmount"))
  (`MaterialInstanceDynamic.SetScalarParameterValue` _mat "ChargeAmount" (`KismetMathLibrary.FClamp` (+ _returnvalue 0.25) 0.0 1.0))
  (bind _output_get (set `self.NumLoaded` (`KismetMathLibrary.Clamp` (+ (`self.NumLoaded`) 1) 0 4)))
  (`KismetSystemLibrary.PrintString` (`KismetStringLibrary.Conv_IntToString` _output_get)))

(fn `QueRockets`
  (bind _numloaded (`self.NumLoaded`))
  (bind _mat (`self.Mat`))
  (if (> _numloaded 0)
    (bind _returnvalue (`MaterialInstanceDynamic.K2_GetScalarParameterValue` _mat "ChargeAmount"))
    (`MaterialInstanceDynamic.SetScalarParameterValue` _mat "ChargeAmount" (`KismetMathLibrary.FClamp` (+ _returnvalue -0.25)))
    (`self.FireRocket`)
    (bind _output_get (set `self.NumLoaded` (`KismetMathLibrary.Clamp` (- _numloaded 1) 0 4)))
    (if (> _output_get 0)
      (`KismetSystemLibrary.K2_SetTimer` self "QueRockets" 0.2))))

(fn `UserConstructionScript`)