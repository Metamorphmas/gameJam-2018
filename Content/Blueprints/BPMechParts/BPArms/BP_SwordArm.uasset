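; Sword arm part for the player's mech, providing a melee spin attack through its parent character.
; Init picks the mesh and animation to match the leg type, then checks health.
; Attacks timed within a short spin window chain into faster spins with rising swish pitch.
; While spinning, blade overlaps damage other actors via the CanTakeDamage interface and flash sparks; breaking starts fire and updates player armor.
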(event `self.Init`
  (`self.UpdateSwordType`)
  (`self.CheckHealth`))

(event `self.Attack_Once`
  (bind _spincont (`self.SpinCont`))
  (bind _wav_swish (`self.WAV_Swish`))
  (bind _mechpart (`self.MechPart`))
  (bind _returnvalue (- _spincont 0.5))
  (bind _asplayer_character_final (cast `/Game/Blueprints/PlayerCharacter_Final` (`self.GetParentActor`)))
  (bind _timeleft (`/Game/Blueprints/PlayerCharacter_Final.QueryIsSpinning` _asplayer_character_final))
  (if (and (> _timeleft 0.01) (< _timeleft 0.18))
    (set `self.SpinCont` (+ (`self.SpinCont`) 0.6))
    (`/Game/Blueprints/PlayerCharacter_Final.SpinAttack` _asplayer_character_final (`self.Direction`) _spincont :!label _label)
    (`SkeletalMeshComponent.PlayAnimation` _mechpart (`self.Anim`) false)
    (`SkeletalMeshComponent.SetPlayRate` _mechpart 3.5)
    (`AudioComponent.SetPitchMultiplier` _wav_swish (`KismetMathLibrary.RandomFloatInRange` _returnvalue (+ _returnvalue 0.2)))
    (`AudioComponent.Play` _wav_swish 0.0)
    (elif (not (`/Game/Blueprints/PlayerCharacter_Final.IsSpinning` _asplayer_character_final))
      (set `self.SpinCont` 1.0)
      (goto _label))))

(event `self.SwordColl.OnComponentBeginOverlap`
  (params (OverlappedComponent :type "PrimitiveComponent Object Reference") (OtherActor :type "Actor Object Reference") (OtherComp :type "PrimitiveComponent Object Reference") (OtherBodyIndex :type Integer) (bFromSweep :type Boolean) (SweepResult :type "HitResult Structure (by ref)"))
  (bind _returnvalue (`self.GetParentActor`))
  (bind _asplayer_character_final (cast `/Game/Blueprints/PlayerCharacter_Final` _returnvalue))
  (if (`/Game/Blueprints/PlayerCharacter_Final.IsSpinning` _asplayer_character_final)
    (if (!= (`self.GetParentActor` OtherActor) _returnvalue)
      (if (`KismetSystemLibrary.DoesImplementInterface` OtherActor "/Game/Blueprints/CanTakeDamage.CanTakeDamage_C")
        (message `/Game/Blueprints/CanTakeDamage.TakeDamage` OtherActor (`self.Damage`) "NewEnumerator0"))
      (`ActorComponent.SetActive` (`self.ParticleSystem`) true false)
      (`KismetSystemLibrary.K2_SetTimerDelegate` (delegate `StopSparks`) (`KismetMathLibrary.RandomFloatInRange` 0.01 0.1)))))

(event `StopSparks`
  (`ActorComponent.SetActive` (`self.ParticleSystem`) false false))

(event `self.MakeBroken`
  (`ActorComponent.SetActive` (`self.P_FireBroken`) true false)
  (bind _asplayer_character_final (cast `/Game/Blueprints/PlayerCharacter_Final` (`GameplayStatics.GetPlayerPawn` 0)))
  (`/Game/Blueprints/PlayerCharacter_Final.SetArmorVal` _asplayer_character_final))

(fn `UpdateSwordType`
  (bind _mechpart (`self.MechPart`))
  (bind _asplayer_character_final (cast `/Game/Blueprints/PlayerCharacter_Final` (`self.GetParentActor`)))
  (if (`|EnumEquality` (`/Game/Blueprints/PlayerCharacter_Final.LegType` _asplayer_character_final) "NewEnumerator0")
    (`SkinnedMeshComponent.SetSkinnedAssetAndUpdate` _mechpart "/Game/Meshes/MechParts/Mesh_Arms/Mech_SwordArm_Biped.Mech_SwordArm_Biped" true)
    (set `self.Anim` "/Game/Animations/Arms/Mech_SwordArm_Biped_Anim.Mech_SwordArm_Biped_Anim")
    (else
      (`SkinnedMeshComponent.SetSkinnedAssetAndUpdate` _mechpart "/Game/Meshes/MechParts/Mesh_Arms/Mech_SwordArm2.Mech_SwordArm2" true)
      (set `self.Anim` "/Game/Animations/Arms/Mech_SwordArm2_Anim.Mech_SwordArm2_Anim"))))

(fn `UserConstructionScript`)