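; Mech gatling arm weapon that spins up its barrels while the attack input is held and fires projectiles once near full speed.
; AttackConstant steps a clamped spin value up or down on each call, spawning a projectile at FireLocation with a yaw offset above the threshold.
; Tick feeds that spin value into the BarrelRot timeline's play rate, which drives the Rotator's pitch.
; The trailing Delay gates nothing, so fire rate follows call frequency.
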(event `self.ReceiveBeginPlay`
  (`TimelineComponent.SetPlayRate` (`self.BarrelRot`) 0.0)
  (bind (_direction _rotval) (`Timeline|BarrelRot`)
    (:`Update`
      (`SceneComponent.K2_SetRelativeRotation` (`self.Rotator`) (`KismetMathLibrary.MakeRotator` 0.0 _rotval 0.0) false false))))

(event `self.ReceiveTick`
  (params (DeltaSeconds :type "Float (single-precision)"))
  (`TimelineComponent.SetPlayRate` (`self.BarrelRot`) (`self.Rot`)))

(event `self.Attack_Constant`
  (params (ButtonVal :type "Float (single-precision)"))
  (bind _firelocation (`self.FireLocation`))
  (bind (_returnvalue_roll _returnvalue_pitch _returnvalue_yaw) (`KismetMathLibrary.BreakRotator` (`SceneComponent.K2_GetComponentRotation` _firelocation)))
  (if (> ButtonVal 0.0)
    (bind _output_get (set `self.Rot` (`KismetMathLibrary.FClamp` (+ (`self.Rot`) 0.2) 0.0 5.0)))
    (if (> _output_get 4.0)
      (`|SpawnActorFromClass` "/Game/Blueprints/Projectile.Projectile_C" (`KismetMathLibrary.MakeTransform` (`SceneComponent.K2_GetComponentLocation` _firelocation) (`KismetMathLibrary.MakeRotator` _returnvalue_roll _returnvalue_pitch (+ _returnvalue_yaw 90.0))) "Undefined" "OverrideRootScale" null null))
    (`KismetSystemLibrary.Delay` 0.02)
    (else
      (set `self.Rot` (`KismetMathLibrary.FClamp` (+ (`self.Rot`) -0.2) 0.0 5.0)))))

(fn `UserConstructionScript`)