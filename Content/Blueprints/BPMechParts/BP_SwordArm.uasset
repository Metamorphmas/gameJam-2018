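; Sword arm mech part that triggers a spin attack on its parent PlayerCharacter_Final.
; Init picks the biped mesh and attack animation when the owner's leg type matches the first enum entry.
; AttackOnce chains spins: an attack within a narrow QueryIsSpinning window raises spin speed, while one made when not spinning resets it.
; Each accepted attack calls SpinAttack and plays the arm animation sped up.
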(event `self.Init`
  (`self.UpdateSwordType`))

(event `self.Attack_Once`
  (bind _mechpart (`self.MechPart`))
  (bind _asplayer_character_final (cast `/Game/Blueprints/PlayerCharacter_Final` (`self.GetParentActor`)))
  (bind _timeleft (`/Game/Blueprints/PlayerCharacter_Final.QueryIsSpinning` _asplayer_character_final))
  (if (and (> _timeleft 0.01) (< _timeleft 0.18))
    (set `self.SpinCont` (+ (`self.SpinCont`) 0.6))
    (`/Game/Blueprints/PlayerCharacter_Final.SpinAttack` _asplayer_character_final (`self.Direction`) (`self.SpinCont`) :!label _label)
    (`SkeletalMeshComponent.PlayAnimation` _mechpart (`self.Anim`) false)
    (`SkeletalMeshComponent.SetPlayRate` _mechpart 3.5)
    (elif (not (`/Game/Blueprints/PlayerCharacter_Final.IsSpinning` _asplayer_character_final))
      (set `self.SpinCont` 1.0)
      (goto _label))))

(fn `UnblockSpin`)

(fn `UpdateSwordType`
  (bind _asplayer_character_final (cast `/Game/Blueprints/PlayerCharacter_Final` (`self.GetParentActor`)))
  (if (`|EnumEquality` (`/Game/Blueprints/PlayerCharacter_Final.LegType` _asplayer_character_final) "NewEnumerator0")
    (`SkinnedMeshComponent.SetSkinnedAssetAndUpdate` (`self.MechPart`) "/Game/Meshes/MechParts/Mesh_Arms/Mech_SwordArm_Biped.Mech_SwordArm_Biped" true)
    (set `self.Anim` "/Game/Animations/Arms/Mech_SwordArm_Biped_Anim.Mech_SwordArm_Biped_Anim")))

(fn `UserConstructionScript`)