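; BP_MechPart is a mech part Blueprint with health, armor and a broken state.
; TakeDamage reduces incoming damage by the Armor fraction, clamps Health, then runs CheckHealth, which prints Health while it is nonzero.
; At zero Health, a DoOnce sets Broken, tells the player character to update its armor value and calls MakeBroken, which is empty here.
; ResetBrokenCheck re-arms the DoOnce and repeats the health check.
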(event `/Game/Blueprints/CanTakeDamage.TakeDamage`
  (params (Damage :type "Float (single-precision)") (DamageType :type "/Game/Blueprints/Enums/DamageType Enum" :default "NewEnumerator5"))
  (set `self.Health` (`KismetMathLibrary.FClamp` (- (`self.Health`) (* Damage (- 1.0 (`self.Armor`)))) 0.0 100.0))
  (`/Game/Blueprints/CanTakeDamage.CheckHealth`))

(event `/Game/Blueprints/CanTakeDamage.CheckHealth`
  (bind _health (`self.Health`))
  (if (== _health 0.0) :!label _label
    (`/Engine/EditorBlueprintResources/StandardMacros.DoOnce` false :!label _label_2
      (:`Completed`
        (set `self.Broken` true)
        (bind _asplayer_character_final (cast `/Game/Blueprints/PlayerCharacter_Final` (`GameplayStatics.GetPlayerCharacter` 0)))
        (`/Game/Blueprints/PlayerCharacter_Final.SetArmorVal` _asplayer_character_final)
        (`self.MakeBroken`)))
    (else
      (`KismetSystemLibrary.PrintString` (`KismetStringLibrary.Conv_DoubleToString` _health)))))

(event `ResetBrokenCheck`
  (`|ExecutionSequence`
    (:`then_0`
      (goto _label_2 :!via `Reset`))
    (:`then_1`
      (goto _label))))

(fn `MakeBroken`)

(fn `UserConstructionScript`)