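; Mech part pickup for an arm or leg part that the player can pick up.
; The construction script picks the skeletal mesh from PartType and its subtype, and SetWidget fills an info widget with name, health, armor and damage type or speed.
; After a brief spawn delay, PickupRadius overlaps register it as the player's PickupPart and toggle the widget.
; Tick holds the widget at a fixed rotation above the box.
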(event `self.ReceiveBeginPlay`
  (bind _overlappingactors (`PrimitiveComponent.GetOverlappingActors` (`self.PickupRadius`) "/Game/Blueprints/PlayerCharacter_Final.PlayerCharacter_Final_C"))
  (`self.SetWidget`)
  (if (`self.FlipDirection`)
    _
    (else
      _))
  (`KismetSystemLibrary.Delay` 0.04)
  (set `self.CanPickUp` true)
  (if (> (`KismetArrayLibrary.Array_Length` _overlappingactors) 0)
    (bind _asplayer_character_final (cast `/Game/Blueprints/PlayerCharacter_Final` (`|GetArrayItem` _overlappingactors)))
    (set `/Game/Blueprints/PlayerCharacter_Final.PickupPart` self _asplayer_character_final)
    (`SceneComponent.SetHiddenInGame` (`self.Widget`) false false)))

(event `self.ReceiveTick`
  (params (DeltaSeconds :type "Float (single-precision)"))
  (bind _widget (`self.Widget`))
  (bind (_returnvalue_x _returnvalue_y _returnvalue_z) (`KismetMathLibrary.BreakVector` (`SceneComponent.K2_GetComponentLocation` (`self.Box`))))
  (`SceneComponent.K2_SetWorldRotation` _widget (struct :`Pitch` 45.0 :`Yaw` 180.0) false false)
  (`SceneComponent.K2_SetWorldLocation` _widget (`KismetMathLibrary.MakeVector` _returnvalue_x _returnvalue_y (+ _returnvalue_z 300.0)) false false))

(event `self.PickupRadius.OnComponentBeginOverlap`
  (params (OverlappedComponent :type "PrimitiveComponent Object Reference") (OtherActor :type "Actor Object Reference") (OtherComp :type "PrimitiveComponent Object Reference") (OtherBodyIndex :type Integer) (bFromSweep :type Boolean) (SweepResult :type "HitResult Structure (by ref)"))
  (if (`self.CanPickUp`)
    (bind _asplayer_character_final (cast `/Game/Blueprints/PlayerCharacter_Final` OtherActor))
    (set `/Game/Blueprints/PlayerCharacter_Final.PickupPart` self _asplayer_character_final)
    (`SceneComponent.SetHiddenInGame` (`self.Widget`) false false)))

(event `self.PickupRadius.OnComponentEndOverlap`
  (params (OverlappedComponent :type "PrimitiveComponent Object Reference") (OtherActor :type "Actor Object Reference") (OtherComp :type "PrimitiveComponent Object Reference") (OtherBodyIndex :type Integer))
  (if (`self.CanPickUp`)
    (bind _asplayer_character_final (cast `/Game/Blueprints/PlayerCharacter_Final` OtherActor))
    (if (== (`/Game/Blueprints/PlayerCharacter_Final.PickupPart` _asplayer_character_final) self)
      (set `/Game/Blueprints/PlayerCharacter_Final.PickupPart` null _asplayer_character_final))
    (`SceneComponent.SetHiddenInGame` (`self.Widget`) true false)))

(fn `SetWidget`
  (bind _health (`self.Health`))
  (bind _returnvalue (* (- _health 0.5) 2.0))
  (bind _aspart_pickup (cast `/Game/UI/PartPickup` (`WidgetComponent.GetUserWidgetObject` (`self.Widget`))))
  (bind _integritypercent (`/Game/UI/PartPickup.IntegrityPercent` _aspart_pickup))
  (`TextBlock.SetText` _integritypercent (`KismetTextLibrary.Conv_StringToText` (`KismetStringLibrary.Concat_StrStr` (`KismetStringLibrary.Conv_DoubleToString` (* _health 100.0)) "%")))
  (`TextBlock.SetColorAndOpacity` _integritypercent (make `SlateColor` (`KismetMathLibrary.MakeColor` 1.0 _returnvalue _returnvalue)))
  (`TextBlock.SetText` (`/Game/UI/PartPickup.ArmorValue` _aspart_pickup) (`KismetTextLibrary.Conv_DoubleToText` (`self.Armor`) "HalfToEven"))
  (switch `/Game/Blueprints/Enums/PartTypes` (`self.PartType`)
    (:`NewEnumerator0`
      (`TextBlock.SetText` (`/Game/UI/PartPickup.Speed` _aspart_pickup) "Type:")
      (switch `/Game/Blueprints/Enums/ArmType` (`self.ArmType`)
        (:`NewEnumerator0`
          (bind _partname (`/Game/UI/PartPickup.PartName` _aspart_pickup))
          (`TextBlock.SetText` _partname "Gatling Gun")
          (bind _speedval (`/Game/UI/PartPickup.SpeedVal` _aspart_pickup))
          (`TextBlock.SetText` _speedval "Kinetic")
          (`TextBlock.SetColorAndOpacity` _speedval (make `SlateColor` (struct :`R` 1.0 :`G` 0.703717 :`B` 0.328125 :`A` 1.0))))
        (:`NewEnumerator1`
          (`TextBlock.SetText` _partname "Plasma Cannon")
          (`TextBlock.SetText` _speedval "Plasma")
          (`TextBlock.SetColorAndOpacity` _speedval (make `SlateColor` (struct :`R` 0.303628 :`B` 1.0 :`A` 1.0))))
        (:`NewEnumerator3`
          (`TextBlock.SetText` _partname "Rocket Launcher")
          (`TextBlock.SetText` _speedval "Explosive")
          (`TextBlock.SetColorAndOpacity` _speedval (make `SlateColor` (struct :`R` 1.0 :`G` 0.121763 :`A` 1.0))))
        (:`NewEnumerator4`
          (`TextBlock.SetText` _partname "Beam Laser")
          (`TextBlock.SetText` _speedval "Laser")
          (`TextBlock.SetColorAndOpacity` _speedval (make `SlateColor` (struct :`G` 0.742144 :`B` 1.0 :`A` 1.0))))
        (:`NewEnumerator5`
          (`TextBlock.SetText` _partname "Hydraulic Sword")
          (`TextBlock.SetText` _speedval "Kinetic")
          (`TextBlock.SetColorAndOpacity` _speedval (make `SlateColor` (struct :`R` 1.0 :`G` 0.703717 :`B` 0.328125 :`A` 1.0))))
        (:`NewEnumerator7`
          (`TextBlock.SetText` _partname "Corrosion Cannon")
          (`TextBlock.SetText` _speedval "Plasma")
          (`TextBlock.SetColorAndOpacity` _speedval (make `SlateColor` (struct :`R` 0.303628 :`B` 1.0 :`A` 1.0))))
        (:`NewEnumerator8`
          (`TextBlock.SetText` _partname "Grenade Launcher")
          (`TextBlock.SetText` _speedval "Explosive")
          (`TextBlock.SetColorAndOpacity` _speedval (make `SlateColor` (struct :`R` 1.0 :`G` 0.121763 :`A` 1.0))))
        (:`NewEnumerator9`
          (`TextBlock.SetText` _partname "Laser Javelin")
          (`TextBlock.SetText` _speedval "Laser")
          (`TextBlock.SetColorAndOpacity` _speedval (make `SlateColor` (struct :`G` 0.742144 :`B` 1.0 :`A` 1.0))))
        (:`NewEnumerator10`
          (`TextBlock.SetText` _partname "Broken Appendage")
          (`TextBlock.SetText` _speedval "None")
          (`TextBlock.SetColorAndOpacity` _speedval (make `SlateColor` (struct :`R` 1.0 :`G` 1.0 :`B` 1.0 :`A` 1.0))))))
    (:`NewEnumerator1`
      (switch `/Game/Blueprints/Enums/LegType` (`self.LegType`)
        (:`NewEnumerator0`
          (bind _partname_2 (`/Game/UI/PartPickup.PartName` _aspart_pickup))
          (`TextBlock.SetText` _partname_2 "Bipedal Legs")
          (bind _speedval_2 (`/Game/UI/PartPickup.SpeedVal` _aspart_pickup))
          (`TextBlock.SetText` _speedval_2 "9"))
        (:`NewEnumerator1`
          (`TextBlock.SetText` _partname_2 "Quadrupedal Legs")
          (`TextBlock.SetText` _speedval_2 "3"))
        (:`NewEnumerator2`
          (`TextBlock.SetText` _partname_2 "AT Treads")
          (`TextBlock.SetText` _speedval_2 "13")))
      (`TextBlock.SetText` (`/Game/UI/PartPickup.Speed` _aspart_pickup) "Speed:"))))

(fn `UserConstructionScript`
  (bind _mechpart (`self.MechPart`))
  (bind _mechpart_2 (`self.MechPart`))
  (switch `/Game/Blueprints/Enums/PartTypes` (`self.PartType`)
    (:`NewEnumerator0`
      (switch `/Game/Blueprints/Enums/ArmType` (`self.ArmType`)
        (:`NewEnumerator0`
          (`SkinnedMeshComponent.SetSkinnedAssetAndUpdate` _mechpart "/Game/Meshes/MechParts/Mesh_Arms/Mech_GatlingArm2.Mech_GatlingArm2" true))
        (:`NewEnumerator1`
          (`SkinnedMeshComponent.SetSkinnedAssetAndUpdate` _mechpart "/Game/Meshes/MechParts/Mesh_Arms/Mech_PlasmaCannon1.Mech_PlasmaCannon1" true))
        (:`NewEnumerator3`
          (`SkinnedMeshComponent.SetSkinnedAssetAndUpdate` _mechpart "/Game/Meshes/MechParts/Mesh_Arms/Mech_RocketArm.Mech_RocketArm" true))
        (:`NewEnumerator4`
          (`SkinnedMeshComponent.SetSkinnedAssetAndUpdate` _mechpart "/Game/Meshes/MechParts/Mesh_Arms/Mech_LaserArm3.Mech_LaserArm3" true))
        (:`NewEnumerator5`
          (`SkinnedMeshComponent.SetSkinnedAssetAndUpdate` _mechpart "/Game/Meshes/MechParts/Mesh_Arms/Mech_SwordArm2.Mech_SwordArm2" true))
        (:`NewEnumerator7`
          (`SkinnedMeshComponent.SetSkinnedAssetAndUpdate` _mechpart "/Game/Meshes/MechParts/Mesh_Arms/Mech_CorrosionCannon.Mech_CorrosionCannon" true))
        (:`NewEnumerator8`
          (`SkinnedMeshComponent.SetSkinnedAssetAndUpdate` _mechpart "/Game/Meshes/MechParts/Mesh_Arms/Mech_GrenadeLauncher2.Mech_GrenadeLauncher2" true))
        (:`NewEnumerator9`
          (`SkinnedMeshComponent.SetSkinnedAssetAndUpdate` _mechpart "/Game/Meshes/MechParts/Mesh_Arms/Mech_JavelinArm.Mech_JavelinArm" true))
        (:`NewEnumerator10`
          (`SkinnedMeshComponent.SetSkinnedAssetAndUpdate` _mechpart "/Game/Meshes/MechParts/Mesh_Arms/Mech_Broken_Arm.Mech_Broken_Arm" true))))
    (:`NewEnumerator1`
      (switch `/Game/Blueprints/Enums/LegType` (`self.LegType`)
        (:`NewEnumerator0`
          (`SkinnedMeshComponent.SetSkinnedAssetAndUpdate` _mechpart_2 "/Game/Meshes/MechParts/Mesh_BipedLegs/Mech_Legs_Biped1_RIGTEST2.Mech_Legs_Biped1_RIGTEST2" true))
        (:`NewEnumerator1`
          (`SkinnedMeshComponent.SetSkinnedAssetAndUpdate` _mechpart_2 "/Game/Meshes/MechParts/Mesh_QuadLegs/Mech_QuadLegs1.Mech_QuadLegs1" true))
        (:`NewEnumerator2`
          (`SkinnedMeshComponent.SetSkinnedAssetAndUpdate` _mechpart_2 "/Game/Meshes/MechParts/Mesh_TreadLegs/Mech_TreadLegs1.Mech_TreadLegs1" true))))))