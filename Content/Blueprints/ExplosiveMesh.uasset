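; A configurable explosive prop that takes armor-reduced damage, with mesh, material and blast radius set in its construction script.
; Weakness damage is doubled, while Resistance damage leaves health untouched and can spill one oil actor nearby.
; At zero health it waits a short random delay, damages overlapping actors through the CanTakeDamage interface, spawns explosion and fragments, ignites its oil, then destroys itself.
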(event `/Game/Blueprints/CanTakeDamage.TakeDamage`
  (params (Damage :type "Float (single-precision)") (DamageType :type "/Game/Blueprints/Enums/DamageType Enum" :default "NewEnumerator5"))
  (bind _returnvalue (`KismetMathLibrary.RandomFloatInRange` -25.0 25.0))
  (bind _health (`self.Health`))
  (bind (_returnvalue_x _returnvalue_y _returnvalue_z) (`KismetMathLibrary.BreakVector` (`SceneComponent.K2_GetComponentLocation` (`self.DefaultSceneRoot`))))
  (bind _returnvalue_2 (* Damage (- 1.0 (`self.Armor`))))
  (if (== DamageType (`self.Weakness`))
    (set `self.Health` (- _health (* _returnvalue_2 2.0)))
    (`/Game/Blueprints/CanTakeDamage.CheckHealth` :!label _label)
    (elif (== DamageType (`self.Resistance`))
      (`/Engine/EditorBlueprintResources/StandardMacros.DoOnce` false
        (:`Completed`
          (if (`self.Oil`)
            (bind _returnvalue_3 (`|SpawnActorFromClass` "/Game/Blueprints/BP_Oil.BP_Oil_C" (`KismetMathLibrary.MakeTransform` (`KismetMathLibrary.MakeVector` (+ _returnvalue_x _returnvalue) (+ _returnvalue_y _returnvalue) _returnvalue_z)) "Undefined" "OverrideRootScale" null self null))
            (set `self.OilBP` _returnvalue_3))))
      (else
        (set `self.Health` (- _health _returnvalue_2))
        (goto _label)))))

(event `/Game/Blueprints/CanTakeDamage.CheckHealth`
  (bind _oilbp (`self.OilBP`))
  (bind _expsize (`self.ExpSize`))
  (if (<= (`self.Health`) 0.0)
    (`/Engine/EditorBlueprintResources/StandardMacros.DoOnce` false
      (:`Completed`
        (`KismetSystemLibrary.Delay` (`KismetMathLibrary.RandomFloatInRange` 0.05 0.2))
        (for _array_element (`PrimitiveComponent.GetOverlappingActors` (`self.Radius`) null)
          (if (`KismetSystemLibrary.DoesImplementInterface` _array_element "/Game/Blueprints/CanTakeDamage.CanTakeDamage_C")
            (message `/Game/Blueprints/CanTakeDamage.TakeDamage` _array_element (`self.Damage`) "NewEnumerator4")))
        (`GameplayStatics.SpawnEmitterAtLocation` "/Game/ParticleEffects/P_Explosion.P_Explosion" (`SceneComponent.K2_GetComponentLocation` (`self.Radius`)) (struct) (`KismetMathLibrary.MakeVector` _expsize _expsize _expsize))
        (`SceneComponent.SetHiddenInGame` (`self.StaticMesh`) true false)
        (`|SpawnActorFromClass` "/Game/Blueprints/BP_FragmentSpawner.BP_FragmentSpawner_C" (`self.GetTransform`) "Undefined" "OverrideRootScale" null (`self.FragmentSpawnNum`) null)
        (if (`KismetSystemLibrary.IsValid` _oilbp)
          (`/Game/Blueprints/BP_Oil.Burn` _oilbp true))
        (`KismetSystemLibrary.K2_SetTimer` self "DestroySelf" 0.1)))))

(fn `DestroySelf`
  (`self.K2_DestroyActor`))

(fn `UserConstructionScript`
  (bind _staticmesh (`self.StaticMesh`))
  (`StaticMeshComponent.SetStaticMesh` _staticmesh (`self.Mesh`))
  (`PrimitiveComponent.SetMaterial` _staticmesh 0 (`self.Mat`))
  (`SphereComponent.SetSphereRadius` (`self.Radius`) (`self.DmgRadius`) true))