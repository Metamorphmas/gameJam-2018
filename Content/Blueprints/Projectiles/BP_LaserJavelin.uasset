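; Laser javelin projectile that flies forward, damages what it overlaps and expires after a few seconds.
; A looping timer moves it by unswept location offsets with capped acceleration, while Guided only toggles homing on ProjectileMovement.
; Box overlaps ignore the instantiator and its child actors, sending interface damage and spawning a laser explosion on damageable actors.
; Impacts do not destroy it, and Hit and Primed have no effect here.
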(event `Prime`
  (set `self.Primed` true))

(event `self.ReceiveBeginPlay`
  (set `ProjectileMovementComponent.bIsHomingProjectile` (`self.Guided`) (`self.ProjectileMovement`))
  (`KismetSystemLibrary.K2_SetTimerDelegate` (delegate `Prime`) 0.01 true)
  (`KismetSystemLibrary.K2_SetTimerDelegate` (delegate `Update`) 0.02 true)
  (`KismetSystemLibrary.K2_SetTimerDelegate` (delegate `DestroySelf`) 5.0))

(event `DestroySelf`
  (`self.K2_DestroyActor`))

(event `Update`
  (if (not (`self.Hit`))
    (`self.K2_SetActorLocation` (+ (`self.K2_GetActorLocation`) (* (`self.GetActorForwardVector`) (`self.Speed`))))
    (set `self.Speed` (`KismetMathLibrary.FClamp` (+ (`self.Speed`) 1.0) 0.0 50.0))))

(event `self.Box.OnComponentBeginOverlap`
  (params (OverlappedComponent :type "PrimitiveComponent Object Reference") (OtherActor :type "Actor Object Reference") (OtherComp :type "PrimitiveComponent Object Reference") (OtherBodyIndex :type Integer) (bFromSweep :type Boolean) (SweepResult :type "HitResult Structure (by ref)"))
  (bind _instantiator (`self.Instantiator`))
  (if (and (!= (`self.GetParentActor` OtherActor) _instantiator) (!= OtherActor _instantiator))
    (if (`KismetSystemLibrary.DoesImplementInterface` OtherActor "/Game/Blueprints/CanTakeDamage.CanTakeDamage_C")
      (message `/Game/Blueprints/CanTakeDamage.TakeDamage` OtherActor (`self.Damage`) "NewEnumerator1")
      (`GameplayStatics.SpawnEmitterAtLocation` "/Game/ParticleEffects/P_LaserExplosion.P_LaserExplosion" (`self.K2_GetActorLocation`)))))

(fn `UserConstructionScript`)