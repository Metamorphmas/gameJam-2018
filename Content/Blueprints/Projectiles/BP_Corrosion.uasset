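; BP_Corrosion is a projectile-related actor that applies corrosion damage over time to a Target.
; On BeginPlay it starts a looping half-second timer that sends TakeDamageMessage with Damage to the Target, plus a one-shot Duration timer.
; When the duration expires or the Target becomes invalid, it stops the damage timer, deactivates the Corrosion component and destroys itself after a short delay.
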(event `self.ReceiveBeginPlay`
  (`KismetSystemLibrary.K2_SetTimerDelegate` (delegate `DurationExpired`) (`self.Duration`))
  (bind _returnvalue (`KismetSystemLibrary.K2_SetTimerDelegate` (delegate `DealDamage`) 0.5 true)))

(event `DealDamage`
  (bind _target (`self.Target`))
  (if (`KismetSystemLibrary.IsValid` _target)
    (message `/Game/Blueprints/CanTakeDamage.TakeDamage` _target (`self.Damage`))
    (else
      (`KismetSystemLibrary.K2_ClearAndInvalidateTimerHandle` (stale `self.ReceiveBeginPlay` _returnvalue) :!label _label)
      (`ActorComponent.SetActive` (`self.Corrosion`) false false)
      (`KismetSystemLibrary.Delay` 0.5)
      (`self.K2_DestroyActor`))))

(event `DurationExpired`
  (goto _label))

(fn `UserConstructionScript`)