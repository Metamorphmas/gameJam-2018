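; Rocket projectile that flies along its forward vector and explodes on contact, damaging overlapped actors that implement CanTakeDamage.
; A looping timer moves it with swept location updates and accelerates it to a capped speed.
; Overlaps ignore other rockets and the instigator, while blocking hits explode without damage.
; Impact disables collision, plays pitch-randomized audio, spawns the explosion, hides the mesh and delays destruction; the Primed flag gates nothing.
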(event `Prime`
  (set `self.Primed` true))

(event `self.ReceiveBeginPlay`
  (`KismetSystemLibrary.K2_SetTimerDelegate` (delegate `Prime`) 0.1 true)
  (`KismetSystemLibrary.K2_SetTimerDelegate` (delegate `Update`) 0.02 true))

(event `Update`
  (`self.K2_SetActorLocation` (+ (`self.K2_GetActorLocation`) (* (`self.GetActorForwardVector`) (`self.Speed`))) true)
  (set `self.Speed` (`KismetMathLibrary.FClamp` (+ (`self.Speed`) 1.0) 0.0 50.0)))

(event `self.Hit.OnComponentBeginOverlap`
  (params (OverlappedComponent :type "PrimitiveComponent Object Reference") (OtherActor :type "Actor Object Reference") (OtherComp :type "PrimitiveComponent Object Reference") (OtherBodyIndex :type Integer) (bFromSweep :type Boolean) (SweepResult :type "HitResult Structure (by ref)"))
  (bind _audio (`self.Audio`))
  (bind _instantiator (`self.Instantiator`))
  (cast `/Game/Blueprints/Projectiles/BP_Rocket` OtherActor
    (:`CastFailed`
      (if (`self.Primed`)
        _
        (else
          _))
      (if (and (!= (`self.GetParentActor` OtherActor) _instantiator) (!= _instantiator OtherActor))
        (`/Engine/EditorBlueprintResources/StandardMacros.DoOnce` false
          (:`Completed`
            (`PrimitiveComponent.SetCollisionEnabled` (`self.Hit`) "NoCollision")
            (`AudioComponent.SetPitchMultiplier` _audio (`KismetMathLibrary.RandomFloatInRange` 0.6 0.9))
            (`AudioComponent.Play` _audio 0.0)
            (if (`KismetSystemLibrary.DoesImplementInterface` OtherActor "/Game/Blueprints/CanTakeDamage.CanTakeDamage_C")
              (message `/Game/Blueprints/CanTakeDamage.TakeDamage` OtherActor (`self.Damage`) "NewEnumerator4"))
            (`GameplayStatics.SpawnEmitterAtLocation` "/Game/ParticleEffects/P_Explosion.P_Explosion" (`SceneComponent.K2_GetComponentLocation` (`self.RocketMesh`)) :!label _label)
            (`SceneComponent.SetHiddenInGame` (`self.RocketMesh`) true false)
            (`ActorComponent.SetActive` (`self.ParticleSystem`) false false)
            (`KismetSystemLibrary.K2_SetTimerDelegate` (delegate `DestroySelf`) 5.0)))))))

(event `self.Hit.OnComponentHit`
  (params (HitComponent :type "PrimitiveComponent Object Reference") (OtherActor :type "Actor Object Reference") (OtherComp :type "PrimitiveComponent Object Reference") (NormalImpulse :type "Vector Structure") (Hit :type "HitResult Structure (by ref)"))
  (bind _audio (`self.Audio`))
  (`/Engine/EditorBlueprintResources/StandardMacros.DoOnce` false
    (:`Completed`
      (`PrimitiveComponent.SetCollisionEnabled` (`self.Hit`) "NoCollision")
      (`AudioComponent.SetPitchMultiplier` _audio (`KismetMathLibrary.RandomFloatInRange` 0.6 0.9))
      (`AudioComponent.Play` _audio 0.0)
      (goto _label))))

(event `DestroySelf`
  (`self.K2_DestroyActor`))

(fn `UserConstructionScript`)