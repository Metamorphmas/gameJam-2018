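; BP_Grenade is a timed grenade projectile that explodes and damages actors within its radius.
; Power sets both the projectile's initial speed and an upward velocity applied to the capsule on BeginPlay, which also starts the fuse timer.
; Detonate sends damage through the CanTakeDamage interface to overlapping actors, then spawns an explosion and plays randomly pitched audio.
; It hides Sphere1 and destroys the actor after a short delay.
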(event `self.ReceiveBeginPlay`
  (bind _capsule (`self.Capsule`))
  (bind _returnvalue (`PrimitiveComponent.GetPhysicsLinearVelocity` _capsule "None"))
  (`PrimitiveComponent.SetPhysicsLinearVelocity` _capsule (`KismetMathLibrary.MakeVector` (.x _returnvalue) (.y _returnvalue) (/ (`self.Power`) 2.0)) false "None")
  (`KismetSystemLibrary.K2_SetTimer` self "Detonate" (`self.Duration`)))

(fn `DestroySelf`
  (`self.K2_DestroyActor`))

(fn `Detonate`
  (bind _audio (`self.Audio`))
  (for _array_element (`PrimitiveComponent.GetOverlappingActors` (`self.Radius`) null)
    (if (`KismetSystemLibrary.DoesImplementInterface` _array_element "/Game/Blueprints/CanTakeDamage.CanTakeDamage_C")
      (message `/Game/Blueprints/CanTakeDamage.TakeDamage` _array_element (`self.Damage`) "NewEnumerator4")))
  (`GameplayStatics.SpawnEmitterAtLocation` "/Game/ParticleEffects/P_Explosion.P_Explosion" (`SceneComponent.K2_GetComponentLocation` (`self.Capsule`)) (struct) (3.0 3.0 3.0))
  (`AudioComponent.SetPitchMultiplier` _audio (`KismetMathLibrary.RandomFloatInRange` 0.8 1.4))
  (`AudioComponent.Play` _audio 0.0)
  (`SceneComponent.SetHiddenInGame` (`self.Sphere1`) true false)
  (`KismetSystemLibrary.K2_SetTimer` self "DestroySelf" 1.0))

(fn `UserConstructionScript`
  (set `ProjectileMovementComponent.InitialSpeed` (* (`self.Power`) 0.5) (`self.ProjectileMovement`)))