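; Corrosive orb projectile that arms shortly after spawning and applies corrosion on impact.
; A looping timer moves it forward with capped acceleration and no sweep, while Guided sets the ProjectileMovement homing flag.
; Its first armed hit spawns BP_Corrosion on CanTakeDamage targets, or an explosion emitter otherwise, scaled by the attached BP_CorrosionEffect.
; It then disables collision and particles, stops moving, and destroys itself and the effect after a delay.
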(event `Prime`
  (set `self.Primed` true))

(event `self.ReceiveBeginPlay`
  (set `ProjectileMovementComponent.bIsHomingProjectile` (`self.Guided`) (`self.ProjectileMovement`))
  (`KismetSystemLibrary.K2_SetTimerDelegate` (delegate `Prime`) 0.2 true)
  (`KismetSystemLibrary.K2_SetTimerDelegate` (delegate `Update`) 0.02 true))

(event `Update`
  (if (not (`self.Hit`))
    (`self.K2_SetActorLocation` (+ (`self.K2_GetActorLocation`) (* (`self.GetActorForwardVector`) (`self.Speed`))))
    (set `self.Speed` (`KismetMathLibrary.FClamp` (+ (`self.Speed`) 1.0) 0.0 50.0))))

(event `self.Sphere.OnComponentHit`
  (params (HitComponent :type "PrimitiveComponent Object Reference") (OtherActor :type "Actor Object Reference") (OtherComp :type "PrimitiveComponent Object Reference") (NormalImpulse :type "Vector Structure") (Hit :type "HitResult Structure (by ref)"))
  (bind _sphere (`self.Sphere`))
  (bind _returnvalue (`SceneComponent.K2_GetComponentLocation` _sphere))
  (bind _output (`|GetArrayItem` (`self.GetAttachedActors`)))
  (bind _returnvalue_2 (`self.GetActorScale3D` _output))
  (`/Engine/EditorBlueprintResources/StandardMacros.DoOnce` false
    (:`Completed`
      (if (`self.Primed`)
        (bind _asbp_corrosion_effect (cast `/Game/Blueprints/Projectiles/BP_CorrosionEffect` _output))
        (if (`KismetSystemLibrary.DoesImplementInterface` OtherActor "/Game/Blueprints/CanTakeDamage.CanTakeDamage_C")
          (`|SpawnActorFromClass` "/Game/Blueprints/Projectiles/BP_Corrosion.BP_Corrosion_C" (`KismetMathLibrary.MakeTransform` _returnvalue (struct) _returnvalue_2) "Undefined" "OverrideRootScale" null (`self.Damage`) (`self.Duration`) OtherActor null)
          (else
            (`GameplayStatics.SpawnEmitterAtLocation` "/Game/ParticleEffects/P_CorrosionExplosion.P_CorrosionExplosion" _returnvalue (struct) _returnvalue_2)))
        (`PrimitiveComponent.SetCollisionEnabled` _sphere "NoCollision")
        (`ActorComponent.SetActive` (`/Game/Blueprints/Projectiles/BP_CorrosionEffect.ParticleSystem` _asbp_corrosion_effect) false false)
        (set `self.Hit` true)
        (`KismetSystemLibrary.K2_SetTimerDelegate` (delegate `DestroySelf`) 5.0)))))

(event `DestroySelf`
  (`self.K2_DestroyActor` (`|GetArrayItem` (`self.GetAttachedActors`)))
  (`self.K2_DestroyActor`))

(fn `UserConstructionScript`)