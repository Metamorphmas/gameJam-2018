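; Player mech character assembled from modular legs, chassis and two arm weapons, with top-down style mouse aiming.
; On BeginPlay it sets meshes from type enums, derives walk speed from Speed and adds the mouse widget.
; Each tick, legs lerp toward one of eight world yaws chosen from movement input, while the chassis independently faces the cursor hit point.
; Walker leg animations scale with Speed and pause without input; some part types have no mesh assigned.
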(event `self.ReceiveBeginPlay`
  (`self.SetupRobot`)
  (`self.SetupUI`))

(event `Update`
  (bind (_returnvalue_roll _returnvalue_pitch _returnvalue_yaw) (`KismetMathLibrary.BreakRotator` (`SceneComponent.K2_GetComponentRotation` (`self.Mech_Legs`))))
  (`self.SetTargetRot`)
  (`SceneComponent.K2_SetWorldRotation` (`self.Mech_Legs`) (`KismetMathLibrary.MakeRotator` 0.0 0.0 (`KismetMathLibrary.Lerp` _returnvalue_yaw (`self.TargetLegRot`) 0.15)) false false))

(event `self.ReceiveTick`
  (params (DeltaSeconds :type "Float (single-precision)"))
  (`self.Update`))

(event `InputAxis|MoveForward`
  (params (AxisValue :type "Float (single-precision)"))
  (`self.AddMovementInput` (`self.GetActorForwardVector`) (* AxisValue (`self.Speed`))))

(event `InputAxis|MoveRight`
  (params (AxisValue :type "Float (single-precision)"))
  (`self.AddMovementInput` (`self.GetActorRightVector`) (* (`self.Speed`) AxisValue)))

(fn `SetAnimPlayRate`
  (bind _mech_legs (`self.Mech_Legs`))
  (bind _returnvalue (* (`self.Speed`) 2.0))
  (switch `/Game/Blueprints/Enums/LegType` (`self.LegType`)
    (:`NewEnumerator0`
      (`SkeletalMeshComponent.SetPlayRate` _mech_legs (/ _returnvalue 3.2)))
    (:`NewEnumerator1`
      (`SkeletalMeshComponent.SetPlayRate` _mech_legs (/ _returnvalue 2.0)))))

(fn `SetArm1`
  (bind _mech_arm1 (`self.Mech_Arm1`))
  (switch `/Game/Blueprints/Enums/ArmType` (`self.Arm1Type`)
    (:`NewEnumerator0`
      (`SkinnedMeshComponent.SetSkinnedAssetAndUpdate` _mech_arm1 "/Game/Meshes/MechParts/Mesh_Arms/Mech_GatlingArm1.Mech_GatlingArm1" true))
    (:`NewEnumerator1`
      (`SkinnedMeshComponent.SetSkinnedAssetAndUpdate` _mech_arm1 "/Game/Meshes/MechParts/Mesh_Arms/Mech_PlasmaCannon1.Mech_PlasmaCannon1" true))
    (:`NewEnumerator3`
      (`SkinnedMeshComponent.SetSkinnedAssetAndUpdate` _mech_arm1 "/Game/Meshes/MechParts/Mesh_Arms/Mech_RocketArm.Mech_RocketArm" true))
    (:`NewEnumerator4`
      (`SkinnedMeshComponent.SetSkinnedAssetAndUpdate` _mech_arm1 null true))
    (:`NewEnumerator5`
      (`SkinnedMeshComponent.SetSkinnedAssetAndUpdate` _mech_arm1 "/Game/Meshes/MechParts/Mesh_Arms/Mech_SwordArm.Mech_SwordArm" true))))

(fn `SetArm2`
  (bind _mech_arm2 (`self.Mech_Arm2`))
  (switch `/Game/Blueprints/Enums/ArmType` (`self.Arm2Type`)
    (:`NewEnumerator0`
      (`SkinnedMeshComponent.SetSkinnedAssetAndUpdate` _mech_arm2 "/Game/Meshes/MechParts/Mesh_Arms/Mech_GatlingArm1.Mech_GatlingArm1" true))
    (:`NewEnumerator1`
      (`SkinnedMeshComponent.SetSkinnedAssetAndUpdate` _mech_arm2 null true))
    (:`NewEnumerator3`
      (`SkinnedMeshComponent.SetSkinnedAssetAndUpdate` _mech_arm2 "/Game/Meshes/MechParts/Mesh_Arms/Mech_RocketArm.Mech_RocketArm" true))
    (:`NewEnumerator4`
      (`SkinnedMeshComponent.SetSkinnedAssetAndUpdate` _mech_arm2 null true))
    (:`NewEnumerator5`
      (`SkinnedMeshComponent.SetSkinnedAssetAndUpdate` _mech_arm2 "/Game/Meshes/MechParts/Mesh_Arms/Mech_SwordArm.Mech_SwordArm" true))))

(fn `SetChassis`
  (bind _mech_chassis (`self.Mech_Chassis`))
  (switch `/Game/Blueprints/Enums/ChassisType` (`self.ChassisType`)
    (:`NewEnumerator0`
      (`SkinnedMeshComponent.SetSkinnedAssetAndUpdate` _mech_chassis null true))
    (:`NewEnumerator1`
      (`SkinnedMeshComponent.SetSkinnedAssetAndUpdate` _mech_chassis "/Game/Meshes/MechParts/Mech_Chassis/Mech_Chassis1.Mech_Chassis1" true))
    (:`NewEnumerator2`
      (`SkinnedMeshComponent.SetSkinnedAssetAndUpdate` _mech_chassis null true))))

(fn `SetLegs`
  (bind _mech_legs (`self.Mech_Legs`))
  (bind _mech_chassis (`self.Mech_Chassis`))
  (bind _mech_legs_2 (`self.Mech_Legs`))
  (switch `/Game/Blueprints/Enums/LegType` (`self.LegType`)
    (:`NewEnumerator0`
      (`SkinnedMeshComponent.SetSkinnedAssetAndUpdate` _mech_legs_2 "/Game/Meshes/MechParts/Mesh_BipedLegs/Mech_Legs_Biped1_RIGTEST2.Mech_Legs_Biped1_RIGTEST2" true)
      (`SceneComponent.K2_SetRelativeLocation` _mech_chassis (0.0 0.0 185.0) false false)
      (`SkeletalMeshComponent.PlayAnimation` _mech_legs "/Game/Animations/BipedLegs/Mech_Legs_Biped1_RIGTEST2_Anim.Mech_Legs_Biped1_RIGTEST2_Anim" true)
      (`self.SetAnimPlayRate` :!label _label))
    (:`NewEnumerator1`
      (`SkinnedMeshComponent.SetSkinnedAssetAndUpdate` _mech_legs_2 "/Game/Meshes/MechParts/Mesh_QuadLegs/Mech_QuadLegs1.Mech_QuadLegs1" true)
      (`SceneComponent.K2_SetRelativeLocation` _mech_chassis (0.0 0.0 90.0) false false)
      (`SkeletalMeshComponent.PlayAnimation` _mech_legs "/Game/Animations/QuadLegs/Mech_QuadLegs1_Anim.Mech_QuadLegs1_Anim" true)
      (goto _label))
    (:`NewEnumerator2`
      (`SkinnedMeshComponent.SetSkinnedAssetAndUpdate` _mech_legs_2 "/Game/Meshes/MechParts/Mesh_TreadLegs/Mech_TreadLegs1.Mech_TreadLegs1" true)
      (`SceneComponent.K2_SetRelativeLocation` _mech_chassis (0.0 0.0 110.0) false false))))

(fn `SetMovementSpeed`
  (set `CharacterMovementComponent.MaxWalkSpeed` (* (/ (`self.Speed`) 5.0) 600.0) (`self.CharacterMovement`)))

(fn `SetTargetRot`
  (bind (_returnvalue_x _returnvalue_y) (`KismetMathLibrary.BreakVector` (`self.K2_GetActorLocation`)))
  (bind _returnvalue (`self.GetInputAxisValue`))
  (bind _returnvalue_2 (`self.GetInputAxisValue`))
  (bind _mech_chassis (`self.Mech_Chassis`))
  (bind _returnvalue_3 (< _returnvalue_2 0.0))
  (bind _returnvalue_4 (< _returnvalue 0.0))
  (bind _returnvalue_5 (== _returnvalue_2 0.0))
  (bind (_returnvalue_roll _returnvalue_pitch) (`KismetMathLibrary.BreakRotator` (`SceneComponent.K2_GetComponentRotation` _mech_chassis)))
  (bind _returnvalue_6 (== _returnvalue 0.0))
  (bind _returnvalue_7 (> _returnvalue_2 0.0))
  (bind _returnvalue_8 (> _returnvalue 0.0))
  (bind (_bblockinghit _binitialoverlap _time _distance _location) (`GameplayStatics.BreakHitResult` (`PlayerController.GetHitResultUnderCursorByChannel` (`GameplayStatics.GetPlayerController` 0) "TraceTypeQuery1" true)))
  (bind (_returnvalue_roll_2 _returnvalue_pitch_2 _returnvalue_yaw) (`KismetMathLibrary.BreakRotator` (`KismetMathLibrary.FindLookAtRotation` (`KismetMathLibrary.MakeVector` _returnvalue_x _returnvalue_y) (`KismetMathLibrary.MakeVector` (.x _location) (.y _location)))))
  (`|ExecutionSequence`
    (:`then_0`
      (if (and _returnvalue_6 _returnvalue_5)
        (set `self.IsWalking` false)
        (`SkeletalMeshComponent.SetPlayRate` (`self.Mech_Legs`) 0.0)
        (elif (and _returnvalue_8 _returnvalue_5)
          (set `self.TargetLegRot` 0.0)
          (set `self.IsWalking` true :!label _label)
          (`self.SetAnimPlayRate`)
          (elif (and _returnvalue_8 _returnvalue_7)
            (set `self.TargetLegRot` 45.0)
            (goto _label)
            (elif (and _returnvalue_7 _returnvalue_6)
              (set `self.TargetLegRot` 90.0)
              (goto _label)
              (elif (and _returnvalue_7 _returnvalue_4)
                (set `self.TargetLegRot` 135.0)
                (goto _label)
                (elif (and _returnvalue_4 _returnvalue_5)
                  (set `self.TargetLegRot` 180.0)
                  (goto _label)
                  (elif (and _returnvalue_4 _returnvalue_3)
                    (set `self.TargetLegRot` -135.0)
                    (goto _label)
                    (elif (and _returnvalue_3 _returnvalue_6)
                      (set `self.TargetLegRot` -90.0)
                      (goto _label)
                      (elif (and _returnvalue_3 _returnvalue_8)
                        (set `self.TargetLegRot` -45.0)
                        (goto _label)))))))))))
    (:`then_1`
      (`SceneComponent.K2_SetWorldRotation` _mech_chassis (`KismetMathLibrary.MakeRotator` _returnvalue_roll _returnvalue_pitch (- _returnvalue_yaw 90.0)) false false))))

(fn `SetupRobot`
  (`self.SetLegs`)
  (`self.SetChassis`)
  (`self.SetArm1`)
  (`self.SetArm2`)
  (`self.SetMovementSpeed`))

(fn `SetupUI`
  (bind _returnvalue (`|CreateWidget` "/Game/UI/mouseWidget.mouseWidget_C" (`GameplayStatics.GetPlayerController` 0)))
  (`UserWidget.AddToViewport` _returnvalue 0))

(fn `UserConstructionScript`)