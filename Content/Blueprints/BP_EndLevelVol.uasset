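; BP_EndLevelVol is a trigger volume that ends the level when the player character overlaps its box.
; A Done flag makes it fire once, telling the first BP_FadeHandler found in the world to fade out.
; After a five-second delay it shows the LevelComplete widget on player 0's screen and calls Death(true) on the character.
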(event `self.Box.OnComponentBeginOverlap`
  (params (OverlappedComponent :type "PrimitiveComponent Object Reference") (OtherActor :type "Actor Object Reference") (OtherComp :type "PrimitiveComponent Object Reference") (OtherBodyIndex :type Integer) (bFromSweep :type Boolean) (SweepResult :type "HitResult Structure (by ref)"))
  (bind _asplayer_character_final (cast `/Game/Blueprints/PlayerCharacter_Final` OtherActor))
  (if (not (`self.Done`))
    (set `self.Done` true)
    (bind _outactors (`GameplayStatics.GetAllActorsOfClass` "/Game/Blueprints/BP_FadeHandler.BP_FadeHandler_C"))
    (`/Game/Blueprints/BP_FadeHandler.FadeOut` (`|GetArrayItem` _outactors))
    (`KismetSystemLibrary.Delay` 5.0)
    (bind _returnvalue (`|CreateWidget` "/Game/UI/LevelComplete.LevelComplete_C" (`GameplayStatics.GetPlayerController` 0)))
    (`UserWidget.AddToPlayerScreen` _returnvalue 0)
    (`/Game/Blueprints/PlayerCharacter_Final.Death` _asplayer_character_final true)))

(fn `UserConstructionScript`)