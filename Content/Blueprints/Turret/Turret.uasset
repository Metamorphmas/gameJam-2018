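; Turret actor that takes damage from projectile hits and explodes when its health runs out.
; On hit, it destroys any Projectile that struck it, subtracts a fixed amount of health, and calls a Death event at zero or prints a debug message otherwise.
; Death spawns a rocket explosion emitter at its location and destroys the turret.
; Tick prints current health every frame for debugging; no aiming or firing logic is present.
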(event `self.ReceiveHit`
  (params (MyComp :type "PrimitiveComponent Object Reference") (Other :type "Actor Object Reference") (OtherComp :type "PrimitiveComponent Object Reference") (bSelfMoved :type Boolean) (HitLocation :type "Vector Structure") (HitNormal :type "Vector Structure") (NormalImpulse :type "Vector Structure") (Hit :type "HitResult Structure (by ref)"))
  (bind _asprojectile (cast `/Game/Blueprints/Projectile` Other))
  (`self.K2_DestroyActor` _asprojectile)
  (set `self.Health` (- (`self.Health`) 5))
  (if (<= (`self.Health`) 0)
    (`self.Death`)
    (else
      (`KismetSystemLibrary.PrintString` "I've been shot"))))

(event `Death`
  (`GameplayStatics.SpawnEmitterAtLocation` "/Game/ParticleEffects/RocketExplosion.RocketExplosion" (`self.K2_GetActorLocation`))
  (`self.K2_DestroyActor`))

(event `self.ReceiveTick`
  (params (DeltaSeconds :type "Float (single-precision)"))
  (`KismetSystemLibrary.PrintString` (`KismetStringLibrary.Conv_IntToString` (`self.Health`))))

(fn `UserConstructionScript`)