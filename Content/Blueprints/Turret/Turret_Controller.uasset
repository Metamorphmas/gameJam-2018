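; AI controller for a turret that starts its behavior tree on BeginPlay and supplies it with a target through perception.
; When perception updates and the Blackboard holds no valid Enemy, it searches the currently perceived actors for the player character and stores it as Enemy.
; An existing valid Enemy is kept, as this controller never clears the key.
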(event `self.ReceiveBeginPlay`
  (`self.RunBehaviorTree` "/Game/Blueprints/Turret/Turret_BehaviorTree.Turret_BehaviorTree"))

(event `self.AIPerception.OnPerceptionUpdated`
  (params (UpdatedActors :type "Array of Actor Object Reference (by ref)"))
  (bind _returnvalue (`AIBlueprintHelperLibrary.GetBlackboard` null))
  (`/Engine/EditorBlueprintResources/StandardMacros.IsValid` (`BlackboardComponent.GetValueAsObject` _returnvalue "Enemy")
    (:`Is Not Valid`
      (for _array_element (`AIPerceptionComponent.GetCurrentlyPerceivedActors` (`self.AIPerception`) null)
        (bind _asplayer_character_final (cast `/Game/Blueprints/PlayerCharacter_Final` _array_element))
        (`BlackboardComponent.SetValueAsObject` _returnvalue "Enemy" _asplayer_character_final)
        (break)))))

(fn `UserConstructionScript`)