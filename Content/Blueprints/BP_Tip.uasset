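; BP_Tip is a placeable in-world hint sign that shows a five-line text tip when the player comes near.
; On BeginPlay it pushes its Line1 to Line5 variables into the Tip widget component.
; A trigger sphere reveals the widget and backing plane with a chirp sound when PlayerCharacter_Final enters, and hides both on exit.
; The construction script applies Radius to the sphere and uses Width to scale the plane and offset the widget.
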(event `self.ReceiveBeginPlay`
  (bind _astip (cast `/Game/UI/Tip` (`WidgetComponent.GetUserWidgetObject` (`self.Tip`))))
  (`/Game/UI/Tip.SetTipText` _astip (`self.Line1`) (`self.Line2`) (`self.Line3`) (`self.Line4`) (`self.Line5`)))

(event `self.Sphere.OnComponentBeginOverlap`
  (params (OverlappedComponent :type "PrimitiveComponent Object Reference") (OtherActor :type "Actor Object Reference") (OtherComp :type "PrimitiveComponent Object Reference") (OtherBodyIndex :type Integer) (bFromSweep :type Boolean) (SweepResult :type "HitResult Structure (by ref)"))
  (cast `/Game/Blueprints/PlayerCharacter_Final` OtherActor)
  (`SceneComponent.SetHiddenInGame` (`self.Tip`) false true)
  (`SceneComponent.SetHiddenInGame` (`self.TipPlane`) false true)
  (`AudioComponent.Play` (`self.WAV_Chirp1`) 0.0))

(event `self.Sphere.OnComponentEndOverlap`
  (params (OverlappedComponent :type "PrimitiveComponent Object Reference") (OtherActor :type "Actor Object Reference") (OtherComp :type "PrimitiveComponent Object Reference") (OtherBodyIndex :type Integer))
  (cast `/Game/Blueprints/PlayerCharacter_Final` OtherActor)
  (`SceneComponent.SetHiddenInGame` (`self.Tip`) true true)
  (`SceneComponent.SetHiddenInGame` (`self.TipPlane`) true true))

(fn `UserConstructionScript`
  (bind _tipplane (`self.TipPlane`))
  (bind (_relativescale3d_x _relativescale3d_y _relativescale3d_z) (`KismetMathLibrary.BreakVector` (`SceneComponent.RelativeScale3D` _tipplane)))
  (`SphereComponent.SetSphereRadius` (`self.Sphere`) (`self.Radius`) true)
  (`SceneComponent.SetRelativeScale3D` _tipplane (`KismetMathLibrary.MakeVector` _relativescale3d_x (`self.Width`) _relativescale3d_z))
  (`SceneComponent.K2_SetRelativeLocation` (`self.Tip`) (`KismetMathLibrary.MakeVector` 0.0 (* (- (`self.Width`) 5.2) 100.0)) false false))