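; BP_FragmentSpawner is an actor that scatters BP_CodeFragment pickups or pieces worth a total of FragmentNum, then destroys itself.
; A fast looping timer calls Spawn, which creates one fragment at a random offset around and above the spawner, passing along Delay.
; While more than ten remain, a coin flip picks a default fragment or a ten-value one, reducing FragmentNum by one or ten accordingly.
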(event `self.ReceiveBeginPlay`
  (`KismetSystemLibrary.K2_SetTimer` self "Spawn" 0.002 true))

(fn `Spawn`
  (bind _returnvalue (`self.GetTransform`))
  (bind _delay (`self.Delay`))
  (bind _returnvalue_2 (+ (.z (.location _returnvalue)) (`KismetMathLibrary.RandomFloatInRange` 0.0 100.0)))
  (bind _returnvalue_3 (+ (.y (.location _returnvalue)) (`KismetMathLibrary.RandomFloatInRange` -50.0 50.0)))
  (bind _returnvalue_4 (+ (.x (.location _returnvalue)) (`KismetMathLibrary.RandomFloatInRange` -50.0 50.0)))
  (if (> (`self.FragmentNum`) 0)
    (if (> (/ (`KismetMathLibrary.Conv_IntToDouble` (`self.FragmentNum`)) 10.0) 1.0)
      (switch `int` (`KismetMathLibrary.RandomIntegerInRange` 0 1)
        (:`Default`
          (`|SpawnActorFromClass` "/Game/Blueprints/BP_CodeFragment.BP_CodeFragment_C" (`KismetMathLibrary.MakeTransform` (`KismetMathLibrary.MakeVector` _returnvalue_4 _returnvalue_3 _returnvalue_2) (.rotation _returnvalue) (.scale _returnvalue)) "Undefined" "OverrideRootScale" null 1 _delay null :!label _label)
          (`/Engine/EditorBlueprintResources/StandardMacros.DecrementInt` (`self.FragmentNum`)))
        (:`0`
          (goto _label))
        (:`1`
          (`|SpawnActorFromClass` "/Game/Blueprints/BP_CodeFragment.BP_CodeFragment_C" (`KismetMathLibrary.MakeTransform` (`KismetMathLibrary.MakeVector` _returnvalue_4 _returnvalue_3 _returnvalue_2) (.rotation _returnvalue) (.scale _returnvalue)) "Undefined" "OverrideRootScale" null 10 _delay null)
          (set `self.FragmentNum` (- (`self.FragmentNum`) 10))))
      (else
        (goto _label)))
    (else
      (`self.K2_DestroyActor`))))

(fn `UserConstructionScript`)